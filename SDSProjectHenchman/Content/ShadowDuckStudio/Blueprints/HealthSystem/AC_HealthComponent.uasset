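; Actor component that tracks health for the actor it is attached to.
; Current health starts at the maximum on BeginPlay, and the Damage event subtracts from it without clamping.
; At zero or below, Damage calls DeathMessage without an explicit target, while a separate Death event sends DeathMessage to the owning actor.
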(event EventBeginPlay
  (Variables|Default|SetCurrentHealth (Variables|Default|GetMaxHealth)))

(event EventTick
  (params (DeltaSeconds :type Float%20%28single-precision%29)))

(event EventDamage
  (params (Damage :type Float%20%28double-precision%29))
  (bind _output_get (Variables|Default|SetCurrentHealth (- (Variables|Default|GetCurrentHealth) Damage)))
  (if (<= _output_get 0.0)
    (Class|BIHealthInterface|Death(Message) self)))

(event EventDeath
  (Class|BIHealthInterface|Death(Message) (Components|GetOwner)))