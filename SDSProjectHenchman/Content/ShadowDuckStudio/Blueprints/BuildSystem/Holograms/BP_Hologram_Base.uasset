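; Base hologram actor for the build system, which tracks whether its placement area overlaps other actors.
; Overlap begin and end events on the Cube1 component maintain a unique list of overlapping actors, excluding itself.
; CollisionCheck reports true while that list is not empty, and GetMeshes returns both the Cube and Cube1 components.
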(event OnComponentBeginOverlap(Cube1)
  (params (OverlappedComponent :type Primitive%20Component%20Object%20Reference) (OtherActor :type Actor%20Object%20Reference) (OtherComp :type Primitive%20Component%20Object%20Reference) (OtherBodyIndex :type Integer) (bFromSweep :type Boolean) (SweepResult :type Hit%20Result%20Structure%20%28by%20ref%29))
  (if (not (== OtherActor self))
    (Utilities|Array|AddUnique (Variables|Default|GetOverlappingActors) OtherActor)))

(event OnComponentEndOverlap(Cube1)
  (params (OverlappedComponent :type Primitive%20Component%20Object%20Reference) (OtherActor :type Actor%20Object%20Reference) (OtherComp :type Primitive%20Component%20Object%20Reference) (OtherBodyIndex :type Integer))
  (if (not (== self OtherActor))
    (Utilities|Array|RemoveItem (Variables|Default|GetOverlappingActors) OtherActor)))

(event EventBeginPlay)

(event Collision|EventActorBeginOverlap
  (params (OtherActor :type Actor%20Object%20Reference)))

(event EventTick
  (params (DeltaSeconds :type Float%20%28single-precision%29)))

(fn ConstructionScript)

(fn CollisionCheck
  (return (Utilities|Array|IsNotEmpty (Variables|Default|GetOverlappingActors))))

(fn GetMeshes
  (return (Utilities|Array|MakeArray (Variables|Default|GetCube) (Variables|Default|GetCube1))))