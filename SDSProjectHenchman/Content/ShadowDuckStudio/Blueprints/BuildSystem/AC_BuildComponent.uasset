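; Actor component that runs hologram-based building placement from a hotbar of buildables.
; While building, a looping timer traces from the camera, aligns the hologram to the surface normal with player rotation, and swaps valid/invalid materials.
; Validity requires a hit, no collision, enough resources and allowed angles.
; Confirming spawns the selected actor and charges the resource component; hotbar cycling restarts the preview and updates the widget.
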(event Custom|HotbarRight
  (Class|BIBuildInterface|EndBuild(Message) self)
  (Variables|Default|SetSelectedHotbar (select (> (+ (Variables|Default|GetSelectedHotbar) 1) (- (Utilities|Array|Length (Variables|Default|GetBuildList)) 1)) 0 (+ (Variables|Default|GetSelectedHotbar) 1)))
  (CallFunction|UpdateHotbarUI)
  (Class|BIBuildInterface|BeginBuild(Message) self))

(event Custom|HotbarLeft
  (Class|BIBuildInterface|EndBuild(Message) self)
  (Variables|Default|SetSelectedHotbar (select (< (- (Variables|Default|GetSelectedHotbar) 1) 0) (- (Utilities|Array|Length (Variables|Default|GetBuildList)) 1) (- (Variables|Default|GetSelectedHotbar) 1)))
  (CallFunction|UpdateHotbarUI)
  (Class|BIBuildInterface|BeginBuild(Message) self))

(event Custom|RotateLeft
  (Variables|Default|SetRotation (+ (Variables|Default|GetRotation) (Variables|Default|GetRotChange))))

(event Custom|RotateRight
  (Variables|Default|SetRotation (- (Variables|Default|GetRotation) (Variables|Default|GetRotChange))))

(event EventBeginPlay
  (Variables|Default|SetResourceComponent (Actor|GetComponentbyClass (Components|GetOwner) "/Game/ShadowDuckStudio/Blueprints/ResourcesSystem/AC_ResourceComponent.AC_ResourceComponent_C"))
  (CallFunction|UpdateHotbarUI))

(event EventBeginBuild
  (bind _returnvalue (Game|SpawnActorfromClass "/Game/ShadowDuckStudio/Blueprints/BuildSystem/Holograms/BP_Hologram_Base.BP_Hologram_Base_C" (Math|Transform|MakeTransform "0, 0, 0") "Undefined" "MultiplyWithRoot" 0 (Utilities|Struct|BreakF_BuildInfo (CallFunction|GetHotbarValue)) 0))
  (Variables|Default|SetHandledActor _returnvalue)
  (Utilities|Time|SetTimerbyFunctionName 0 "BuildTick" (Variables|Default|GetBuildTickTime) true)
  (Variables|Default|SetIsBuilding? true)
  (CallFunction|UpdateHotbarUI))

(event EventEndBuild
  (Utilities|Time|ClearTimerbyFunctionName 0 "BuildTick")
  (bind _handledactor (Variables|Default|GetHandledActor)
    (:then
      (Actor|DestroyActor _handledactor)
      (Variables|Default|SetIsBuilding? false))
    (:else)))

(event EventBuildHandled
  (if (Variables|Default|GetCanBuild?)
    (Game|SpawnActorfromClass (.Built (Utilities|Struct|BreakF_BuildInfo (CallFunction|GetHotbarValue))) (Transformation|GetActorTransform (Variables|Default|GetHandledActor)) "AlwaysSpawn" "MultiplyWithRoot" 0 0)
    (Class|BIResourceInterface|TakeResource(Message) (Variables|Default|GetResourceComponent) (.Cost (Utilities|Struct|BreakF_BuildInfo (CallFunction|GetHotbarValue))))
    (Class|BIBuildInterface|EndBuild(Message) self)))

(fn BuildTick
  (bind _returnvalue (Game|GetPlayerController 0))
  (bind _handledactor (Variables|Default|GetHandledActor))
  (bind _playercameramanager (Variables|/Script/Engine.PlayerController|GetPlayerCameraManager _returnvalue))
  (bind _returnvalue_2 (Transformation|GetActorLocation _playercameramanager))
  ;[1 1 1] Get Where Player Is Looking
  (bind _outhit (Collision|LineTraceByChannel _returnvalue_2 (+ _returnvalue_2 (* (Transformation|GetActorForwardVector _playercameramanager) (Variables|Default|GetBuildRange))) "TraceTypeQuery1" false (Utilities|Array|MakeArray (Game|Player|GetPlayerPawn 0) (Variables|Default|GetHandledActor)) "None"))
  (if (Variables|Default|GetHologramsCanFloat?)
    ;[1 1 1] Set Building Rotation And Location
    (Transformation|SetActorLocationAndRotation _handledactor (Math|Vector|SelectVector (.Location (Collision|BreakHitResult _outhit)) (.TraceEnd (Collision|BreakHitResult _outhit)) (.bBlockingHit (Collision|BreakHitResult _outhit))) (CallFunction|RotateRotatoronAxis (Math|Rotator|MakeRotfromZ (.Normal (Collision|BreakHitResult _outhit))) (Variables|Default|GetRotation) "NewEnumerator2") :!label _label)
    ;[1 1 1] Check If Can Build
    (bind _colliding_ (Class|BIBuildInterface|CollisionCheck(Message) _handledactor))
    (bind _enoughresource_ (Class|BIResourceInterface|CheckEnoughResources?(Message) (Variables|Default|GetResourceComponent) (.Cost (Utilities|Struct|BreakF_BuildInfo (CallFunction|GetHotbarValue)))))
    (bind _output_get (Variables|Default|SetCanBuild? (Math|Boolean|ANDBoolean (not _colliding_) _enoughresource_ (CallFunction|CheckRotation _handledactor) (.bBlockingHit (Collision|BreakHitResult _outhit)))))
    ;[1 1 1] Set Materials On Actor
    (bind _meshes (Class|BIBuildInterface|GetMeshes(Message) (Variables|Default|GetHandledActor)))
    (for _array_element _meshes
      (for _index (range 0 (Rendering|Material|GetNumMaterials _array_element))
        (Rendering|Material|SetMaterial _array_element _index (select _output_get (Variables|Default|GetValidMaterial) (Variables|Default|GetInvalidMaterial)))))
    (elif (.bBlockingHit (Collision|BreakHitResult _outhit))
      (goto _label))))

(fn GetHotbarValue
  (return (Utilities|Array|Get(acopy) (Variables|Default|GetBuildList) (Variables|Default|GetSelectedHotbar))))

(fn CheckRotation
  (params (ActorToCheck :type Actor%20Object%20Reference))
  (bind _returnvalue (Transformation|GetActorRotation ActorToCheck))
  (bind _output (CallFunction|GetHotbarValue))
  (bind _angleconstraints (Utilities|Struct|BreakF_BuildInfo _output))
  (bind (_roll _pitch) (Math|Rotator|BreakRotator _returnvalue))
  (bind (_minx _maxx _miny _maxy) (Utilities|Struct|BreakF_BuildConstraints _angleconstraints))
  (return (and (and (<= _roll _maxx) (>= _roll _minx)) (and (<= _pitch _maxy) (>= _pitch _miny)))))

(fn UpdateHotbarUI
  (bind _buildlist (Variables|Default|GetBuildList))
  (bind _selectedhotbar (Variables|Default|GetSelectedHotbar))
  (bind _hotbarref (Variables|Default|GetHotbarRef)
    (:then
      (Default|UpdateHotbar _hotbarref _selectedhotbar _buildlist))
    (:else
      (bind _returnvalue (UserInterface|CreateWidget "/Game/Thomas/Widgets/BuildableHotBar_WBP.BuildableHotBar_WBP_C"))
      (bind _output_get (Variables|Default|SetHotbarRef _returnvalue))
      (Default|UpdateHotbar _output_get _selectedhotbar _buildlist)
      (Utilities|IsValid _hotbarref
        (:Is%20Valid
          (Default|UpdateHotbar _output_get _selectedhotbar _buildlist))
        (:Is%20Not%20Valid
          (Development|PrintString "ZZZZZZZZZZZZZZZZZZZZZZZZZZZZ"))))))

(fn CollisionCheck)

(fn GetMeshes
  (return 0))