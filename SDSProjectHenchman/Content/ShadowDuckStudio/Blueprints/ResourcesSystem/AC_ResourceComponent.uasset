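; AC_ResourceComponent stores a resource pool, currently handling only Resource1, with functions to query it and check costs.
; BeginPlay caches the BP_HMCharacter and shares the add path, which lazily finds that character's AC_BuildComponent.
; Adding and taking resources both refresh the build component's hotbar UI.
; TakeResource only requires a positive balance, so amounts can go negative unless callers use CheckEnoughResources.
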(event EventBeginPlay
  (bind _resources (Variables|Default|GetResources))
  (bind _returnvalue (Actor|GetActorOfClass "/Game/ShadowDuckStudio/Blueprints/Player/BP_HMCharacter.BP_HMCharacter_C"))
  (bind _output_get (Variables|Default|SetPlayerRef _returnvalue))
  (bind _buildcomponent (Variables|Default|GetBuildComponent)
    (:then
      (Variables|Default|SetBuildComponent _buildcomponent))
    (:else
      (Variables|Default|SetBuildComponent (Actor|GetComponentbyClass _output_get "/Game/ShadowDuckStudio/Blueprints/BuildSystem/AC_BuildComponent.AC_BuildComponent_C"))))
  (Utilities|Struct|SetmembersinF_Resources _resources (+ (Utilities|Struct|BreakF_Resources _resources) (Utilities|Struct|BreakF_Resources (stale EventAddResource ResourcesAdded))))
  (Default|UpdateHotbarUI (Variables|Default|GetBuildComponent)))

(event EventTick
  (params (DeltaSeconds :type Float%20%28single-precision%29)))

(event EventAddResource
  (params (ResourcesAdded :type F%20Resources%20Structure))
  (bind _resources (Variables|Default|GetResources))
  (bind _buildcomponent (Variables|Default|GetBuildComponent)
    (:then
      (Variables|Default|SetBuildComponent _buildcomponent))
    (:else
      (Variables|Default|SetBuildComponent (Actor|GetComponentbyClass (stale EventBeginPlay _output_get) "/Game/ShadowDuckStudio/Blueprints/BuildSystem/AC_BuildComponent.AC_BuildComponent_C"))))
  (Utilities|Struct|SetmembersinF_Resources _resources (+ (Utilities|Struct|BreakF_Resources _resources) (Utilities|Struct|BreakF_Resources ResourcesAdded)))
  (Default|UpdateHotbarUI (Variables|Default|GetBuildComponent)))

(event EventTakeResource
  (params (ResourcesTaken :type F%20Resources%20Structure))
  (bind _resources (Variables|Default|GetResources))
  (bind _resource1 (Utilities|Struct|BreakF_Resources _resources))
  (if (not (<= _resource1 0))
    (Utilities|Struct|SetmembersinF_Resources _resources (- _resource1 (Utilities|Struct|BreakF_Resources ResourcesTaken)))
    (Default|UpdateHotbarUI (Variables|Default|GetBuildComponent))))

(fn CheckEnoughResources?
  (params (AmountToCheck :type F%20Resources%20Structure))
  (return (and (<= (Utilities|Struct|BreakF_Resources AmountToCheck) (Utilities|Struct|BreakF_Resources (Variables|Default|GetResources))) true)))

(fn GetResourceAmount
  (return (Variables|Default|GetResources)))