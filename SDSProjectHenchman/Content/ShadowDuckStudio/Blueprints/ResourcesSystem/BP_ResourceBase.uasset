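; Base Blueprint for a harvestable resource node that gives the player resources on interaction and regrows after a delay.
; BeginPlay rolls the yield once between its min and max, and BeginInteract passes it to the player pawn's AC_ResourceComponent via AddResourceMessage.
; Harvesting clears CanHarvest and hides the mesh without collision until a random-length timer calls RegenResource to restore both.
; BeginInteract never checks CanHarvest itself, and GetOverlayMeshes is an empty stub.
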(event EventBeginPlay
  (Variables|Default|SetResources (Utilities|Struct|MakeF_Resources (Math|Random|RandomIntegerinRange (Variables|Default|GetMinResource) (Variables|Default|GetMaxResource)))))

(event EventBeginInteract
  (params (Source :type Actor%20Object%20Reference))
  (bind _returnvalue (Game|Player|GetPlayerPawn 0))
  (bind _returnvalue_2 (Actor|GetComponentbyClass _returnvalue "/Game/ShadowDuckStudio/Blueprints/ResourcesSystem/AC_ResourceComponent.AC_ResourceComponent_C"))
  (bind _resourcecon (Variables|Default|GetResourceCon)
    (:then
      (Variables|Default|SetResourceCon _resourcecon)
      (Variables|Default|SetCanHarvest? false :!label _label)
      (Class|BIResourceInterface|AddResource(Message) _returnvalue_2 (Variables|Default|GetResources))
      (CallFunction|DisableMesh)
      (Utilities|Time|SetTimerbyFunctionName 0 "RegenResource" (Math|Random|RandomFloatinRange (Variables|Default|GetMinRegenTime) (Variables|Default|GetMaxRegenTime))))
    (:else
      (bind _output_get (Variables|Default|SetResourceCon _returnvalue_2))
      (Utilities|IsValid _output_get
        (:Is%20Valid
          (goto _label))
        (:Is%20Not%20Valid
          (Development|PrintString "ResourceNOTWORKING"))))))

(fn ConstructionScript)

(fn DisableMesh
  (bind _staticmesh (Variables|Default|GetStaticMesh))
  (Development|SetHiddeninGame _staticmesh true false)
  (Collision|SetCollisionEnabled _staticmesh "NoCollision"))

(fn RegenResource
  (Variables|Default|SetCanHarvest? true)
  (CallFunction|EnableMesh))

(fn EnableMesh
  (bind _staticmesh (Variables|Default|GetStaticMesh))
  (Development|SetHiddeninGame _staticmesh false false)
  (Collision|SetCollisionEnabled _staticmesh "QueryAndPhysics"))

(fn GetOverlayMeshes
  (return 0))