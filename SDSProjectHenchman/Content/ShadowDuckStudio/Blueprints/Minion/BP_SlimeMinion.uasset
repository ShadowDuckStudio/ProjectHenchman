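; BP_SlimeMinion is a short-lived slime minion that seeks out enemies and leaves a lava puddle when it dies.
; A looping timer searches for the nearest BP_Enemy_Base, stops once a target is found, and starts AI movement toward it.
; Failed moves restart the search.
; Reaching the target damages its AC_HealthComponent and triggers Death, as does lifespan expiry, spawning BP_LavaPuddle and destroying the minion.
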(event Custom|Explode
  (Game|SpawnActorfromClass "/Game/ShadowDuckStudio/Blueprints/Minion/BP_LavaPuddle.BP_LavaPuddle_C" (Transformation|GetActorTransform) "AdjustIfPossibleButAlwaysSpawn" "MultiplyWithRoot" 0 0)
  (Actor|DestroyActor))

(event Custom|BeginMovement
  (bind _target (Variables|Default|GetTarget))
  (bind _movementresult (AI|AIMoveTo self "0, 0, 0" _target 5.0 true)
    (:then
      (switch Utilities|FlowControl|Switch|SwitchonEPathFollowingResult _movementresult
        (:Blocked
          _)
        (:OffPath
          _)
        (:Aborted
          _)
        (:Invalid
          _))
      (Utilities|Time|SetTimerbyFunctionName 0 "FindTarget" (Variables|Default|GetTargetingTickTime) true :!label _label))
    (:OnSuccess
      (CallFunction|Death)
      (Default|Damage (Actor|GetComponentbyClass _target "/Game/ShadowDuckStudio/Blueprints/HealthSystem/AC_HealthComponent.AC_HealthComponent_C") (Variables|Default|GetDamage)))
    (:OnFail
      (goto _label))))

(event EventBeginPlay
  (Utilities|Time|SetTimerbyFunctionName 0 "Death" (Variables|Actor|GetInitialLifeSpan))
  (Utilities|Time|SetTimerbyFunctionName 0 "FindTarget" (Variables|Default|GetTargetingTickTime) true))

(fn ConstructionScript)

(fn Death
  (CallFunction|Explode))

(fn FindTarget
  (bind _outactors (Actor|GetAllActorsOfClass "/Game/ShadowDuckStudio/Blueprints/Enemies/BP_Enemy_Base.BP_Enemy_Base_C"))
  (bind _output_get (Variables|Default|SetTarget (.ReturnValue (Actor|FindNearestActor (Transformation|GetActorLocation) _outactors))))
  (Utilities|IsValid _output_get
    (:Is%20Valid
      (Utilities|Time|ClearTimerbyFunctionName 0 "FindTarget")
      (CallFunction|BeginMovement))))