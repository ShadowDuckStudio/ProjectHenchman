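; BP_LavaPuddle is a lava hazard that deals periodic damage to actors standing inside its sphere.
; Sphere overlap events maintain a unique list of actors inside, with each entry (re)starting a looping LavaTick timer and the last exit clearing it.
; On each tick it sends Damage through DamageMessage to every listed actor's AC_HealthComponent, with no filtering by actor type.
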(event OnComponentBeginOverlap(Sphere)
  (params (OverlappedComponent :type Primitive%20Component%20Object%20Reference) (OtherActor :type Actor%20Object%20Reference) (OtherComp :type Primitive%20Component%20Object%20Reference) (OtherBodyIndex :type Integer) (bFromSweep :type Boolean) (SweepResult :type Hit%20Result%20Structure%20%28by%20ref%29))
  (bind _overlappingactors (Variables|Default|GetOverlappingActors))
  (Utilities|Array|AddUnique _overlappingactors OtherActor)
  (if (not (Utilities|Array|IsEmpty _overlappingactors))
    (Utilities|Time|SetTimerbyFunctionName 0 "LavaTick" (Variables|Default|GetLavaTickTime) true)))

(event OnComponentEndOverlap(Sphere)
  (params (OverlappedComponent :type Primitive%20Component%20Object%20Reference) (OtherActor :type Actor%20Object%20Reference) (OtherComp :type Primitive%20Component%20Object%20Reference) (OtherBodyIndex :type Integer))
  (bind _overlappingactors (Variables|Default|GetOverlappingActors))
  (Utilities|Array|RemoveItem _overlappingactors OtherActor)
  (if (Utilities|Array|IsEmpty _overlappingactors)
    (Utilities|Time|ClearTimerbyFunctionName 0 "LavaTick")))

(event EventBeginPlay)

(event Collision|EventActorBeginOverlap
  (params (OtherActor :type Actor%20Object%20Reference)))

(event EventTick
  (params (DeltaSeconds :type Float%20%28single-precision%29)))

(fn ConstructionScript)

(fn LavaTick
  (for _array_element (Variables|Default|GetOverlappingActors)
    (Class|BIHealthInterface|Damage(Message) (Actor|GetComponentbyClass _array_element "/Game/ShadowDuckStudio/Blueprints/HealthSystem/AC_HealthComponent.AC_HealthComponent_C") (Variables|Default|GetDamage))))