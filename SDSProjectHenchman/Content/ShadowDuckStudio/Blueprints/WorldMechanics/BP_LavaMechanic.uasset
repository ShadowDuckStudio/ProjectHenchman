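; BP_LavaMechanic is a world-mechanic lava body whose surface level rises and falls, with its Cube registered as lava through ACDamageOverlap.
; AddLava and RemoveLava clamp LavaValue, then a Timeline lerps the actor between positions interpolated from MinLavaVector and MaxLavaVector, though AddLava always animates from empty.
; Activating the mechanic sends a fixed lava-removal message.
; LavaTick damages overlapping actors' health components but is not called within this graph.
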(event Custom|MoveLavaLevel
  (Components|Timeline|SetPlayRate (Variables|Default|GetTimeline) (/ 1.0 (Variables|Default|GetLavaChangeSpeed)))
  (bind _newtrack_0 (Timeline|Timeline PlayFromStart)
    (:Update
      (Transformation|SetActorLocation (Math|Vector|Lerp(Vector) (Math|Vector|Lerp(Vector) (Variables|Default|GetMinLavaVector) (Variables|Default|GetMaxLavaVector) (/ (Variables|Default|GetOldLavaValue) (Variables|Default|GetMaxLavaValue))) (Math|Vector|Lerp(Vector) (Variables|Default|GetMinLavaVector) (Variables|Default|GetMaxLavaVector) (/ (Variables|Default|GetLavaValue) (Variables|Default|GetMaxLavaValue))) _newtrack_0) false false))))

(event EventBeginPlay
  (Variables|Default|SetLavaValue (Variables|Default|GetMaxLavaValue))
  (Default|MakeLava (Variables|Default|GetAC_DamageOverlap) (Utilities|Array|MakeArray (Variables|Default|GetCube))))

(event EventAddLava
  (params (LavaAmount :type Float%20%28double-precision%29))
  (bind _maxlavavalue (Variables|Default|GetMaxLavaValue))
  (Variables|Default|SetOldLavaValue 0.0)
  (Variables|Default|SetLavaValue (Math|Float|SelectFloat (+ LavaAmount (Variables|Default|GetLavaValue)) _maxlavavalue (< (+ LavaAmount (Variables|Default|GetLavaValue)) _maxlavavalue)))
  (CallFunction|MoveLavaLevel))

(event EventRemoveLava
  (params (LavaAmount :type Float%20%28double-precision%29))
  (Variables|Default|SetOldLavaValue (Variables|Default|GetLavaValue))
  (Variables|Default|SetLavaValue (Math|Float|SelectFloat (- (Variables|Default|GetLavaValue) LavaAmount) 0.0 (> (- (Variables|Default|GetLavaValue) LavaAmount) 0.0)))
  (CallFunction|MoveLavaLevel))

(event EventActivateWorldMechanic
  (Class|BIWorldMechanicInterface|RemoveLava(Message) self 5e+01))

(fn ConstructionScript)

(fn LavaTick
  (for _array_element (Variables|Default|GetOverlappingActors)
    (Class|BIHealthInterface|Damage(Message) (Actor|GetComponentbyClass _array_element "/Game/ShadowDuckStudio/Blueprints/HealthSystem/AC_HealthComponent.AC_HealthComponent_C") (Variables|Default|GetDamagePerTick))))

(fn CheckLavaValue
  (return (Variables|Default|GetLavaValue)))