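; Base Blueprint for moveable world mechanics that slide a Cube between waypoint actors when activated and stop when deactivated.
; BeginPlay selects the current and next waypoint, wrapping to the first after the last.
; A timeline lerps the transform from the stored Current fraction to Target along that segment, with play rate scaled by the gap and MoveSpeed.
; CheckLavaValue is a stub returning zero.
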(event Custom|BeginMove
  (bind (_starttransform _endtransform) (CallFunction|CalculateTransforms))
  (Variables|Default|SetOld%25 (Variables|Default|GetCurrent%25))
  (Components|Timeline|SetPlayRate (Variables|Default|GetTimeline) (CallFunction|SetPlayRate))
  (bind _newtrack_0 (Timeline|Timeline PlayFromStart)
    (:Update
      (Variables|Default|SetCurrent%25 (Math|Float|Lerp (Variables|Default|GetOld%25) (Variables|Default|GetTarget%25) _newtrack_0))
      (Transformation|SetWorldTransform (Variables|Default|GetCube) (Math|Transform|Lerp(Transform) _starttransform _endtransform _newtrack_0) false false))))

(event Custom|StopMove
  (bind (_starttransform _endtransform) (CallFunction|CalculateTransforms))
  (bind _newtrack_0 (Timeline|Timeline Stop)
    (:Update
      (Variables|Default|SetCurrent%25 (Math|Float|Lerp (Variables|Default|GetOld%25) (Variables|Default|GetTarget%25) _newtrack_0))
      (Transformation|SetWorldTransform (Variables|Default|GetCube) (Math|Transform|Lerp(Transform) _starttransform _endtransform _newtrack_0) false false))))

(event EventBeginPlay
  (CallFunction|SetCurrent&NextWaypoint))

(event Collision|EventActorBeginOverlap
  (params (OtherActor :type Actor%20Object%20Reference)))

(event EventTick
  (params (DeltaSeconds :type Float%20%28single-precision%29)))

(event EventActivateWorldMechanic
  (CallFunction|BeginMove))

(event EventDeactivateWorldMechanic
  (CallFunction|StopMove))

(fn ConstructionScript)

(fn CalculateTransforms
  (return (Math|Transform|Lerp(Transform) (Transformation|GetActorTransform (Variables|Default|GetCurrentWaypoint)) (Transformation|GetActorTransform (Variables|Default|GetNextWaypoint)) (Variables|Default|GetOld%25)) (Math|Transform|Lerp(Transform) (Transformation|GetActorTransform (Variables|Default|GetCurrentWaypoint)) (Transformation|GetActorTransform (Variables|Default|GetNextWaypoint)) (Variables|Default|GetTarget%25))))

(fn SetCurrent&NextWaypoint
  (bind _waypoints (Variables|Default|GetWaypoints))
  (bind _currentwaypointnum (Variables|Default|GetCurrentWaypointNum))
  (bind _returnvalue (+ _currentwaypointnum 1))
  (Variables|Default|SetCurrentWaypoint (Utilities|Array|Get(acopy) _waypoints _currentwaypointnum))
  (Variables|Default|SetNextWaypoint (Utilities|Array|Get(acopy) _waypoints (Math|Integer|SelectInt _returnvalue 0 (<= _returnvalue (- (Utilities|Array|Length _waypoints) 1))))))

(fn SetPlayRate
  (return (/ 1.0 (* (- (Variables|Default|GetTarget%25) (Variables|Default|GetOld%25)) (Variables|Default|GetMoveSpeed)))))

(fn CheckLavaValue
  (return 0.0))