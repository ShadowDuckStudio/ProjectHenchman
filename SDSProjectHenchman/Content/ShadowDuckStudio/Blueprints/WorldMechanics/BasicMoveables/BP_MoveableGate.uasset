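; Damageable, player-repairable gate whose world-mechanic movement target follows lost health, updated on damage or heal.
; Holding interact runs a looping timer that, after a set time, spends player resources for one heal.
; A minimap repair icon shows at low health, plus a hold-to-repair prompt when the player is inside the box.
; An enemy entering that box sends the villain behind the chair.
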(event OnComponentBeginOverlap(Box)
  (params (OverlappedComponent :type Primitive%20Component%20Object%20Reference) (OtherActor :type Actor%20Object%20Reference) (OtherComp :type Primitive%20Component%20Object%20Reference) (OtherBodyIndex :type Integer) (bFromSweep :type Boolean) (SweepResult :type Hit%20Result%20Structure%20%28by%20ref%29))
  ;[0.04417 1 0] On enemy overlap moves the villian behind the chair away from the gates
  (if (Actor|ActorHasTag OtherActor "Enemy")
    (bind _returnvalue (Actor|GetActorOfClass "/Game/ShadowDuckStudio/Blueprints/Villain/BP_Villain_Base.BP_Villain_Base_C"))
    (Default|VillianMovesBehindChair _returnvalue)
    (CallFunction|CheckRepairVisible)
    (elif (Actor|ActorHasTag OtherActor "Player")
      (Variables|Default|SetInVisibleRadius true)
      (CallFunction|CheckRepairVisible))))

(event OnComponentEndOverlap(Box)
  (params (OverlappedComponent :type Primitive%20Component%20Object%20Reference) (OtherActor :type Actor%20Object%20Reference) (OtherComp :type Primitive%20Component%20Object%20Reference) (OtherBodyIndex :type Integer))
  (if (Actor|ActorHasTag OtherActor "Player")
    (Variables|Default|SetInVisibleRadius false)
    (CallFunction|CheckRepairVisible)))

(event Custom|CheckRepairVisible
  (bind _holdtorepairwidget (Variables|Default|GetHoldtoRepairWidget))
  (bind _ac_healthcomponent (Variables|Default|GetAC_HealthComponent))
  (bind _repairiconminimap1 (Variables|Default|GetRepairIconMinimap1))
  (bind _currenthealth (Variables|/Game/ShadowDuckStudio/Blueprints/HealthSystem/AC_HealthComponent.AC_HealthComponent_C|GetCurrentHealth _ac_healthcomponent))
  (bind _returnvalue (<= _currenthealth 7e+01))
  (if _returnvalue
    (Rendering|SetVisibility _repairiconminimap1 true false)
    (else
      (Rendering|SetVisibility _repairiconminimap1 false false)))
  (if (and (Variables|Default|GetInVisibleRadius) _returnvalue)
    (Rendering|SetVisibility _holdtorepairwidget true false)
    (else
      (Rendering|SetVisibility _holdtorepairwidget false false))))

(event EventBeginPlay
  (|CallParentFunction))

(event Collision|EventActorBeginOverlap
  (params (OtherActor :type Actor%20Object%20Reference))
  (|CallParentFunction OtherActor) ; This node is disabled and will not be called.\nDrag off pins to build functionality.
)

(event EventTick
  (params (DeltaSeconds :type Float%20%28single-precision%29))
  (|CallParentFunction DeltaSeconds) ; This node is disabled and will not be called.\nDrag off pins to build functionality.
)

(event EventDamage
  (params (Damage :type Float%20%28double-precision%29))
  (Utilities|FlowControl|DelayUntilNextTick)
  (Variables|Default|SetTarget%25 (- 1.0 (CallFunction|GetHealth%)))
  (CallFunction|ActivateWorldMechanic)
  (CallFunction|CheckRepairVisible))

(event EventEndInteract
  (params (Source :type Actor%20Object%20Reference))
  (Utilities|Time|ClearTimerbyFunctionName 0 "ReloadTick"))

(event EventBeginInteract
  (params (Source :type Actor%20Object%20Reference))
  (Variables|Default|SetCurrentReloadTime 0.0)
  (Utilities|Time|SetTimerbyFunctionName 0 "ReloadTick" (Variables|Default|GetReloadTickTime) true))

(event EventHeal
  (params (Amount :type Float%20%28double-precision%29))
  (Utilities|FlowControl|DelayUntilNextTick)
  (Variables|Default|SetTarget%25 (- 1.0 (CallFunction|GetHealth%)))
  (CallFunction|ActivateWorldMechanic)
  (CallFunction|CheckRepairVisible))

(fn ConstructionScript
  (|CallParentFunction))

(fn GetHealth%
  (bind _ac_healthcomponent (Variables|Default|GetAC_HealthComponent))
  (return (/ (Variables|/Game/ShadowDuckStudio/Blueprints/HealthSystem/AC_HealthComponent.AC_HealthComponent_C|GetCurrentHealth _ac_healthcomponent) (Variables|/Game/ShadowDuckStudio/Blueprints/HealthSystem/AC_HealthComponent.AC_HealthComponent_C|GetMaxHealth _ac_healthcomponent))))

(fn ReloadTick
  (bind _ac_healthcomponent (Variables|Default|GetAC_HealthComponent))
  (bind _resources_taken_ (Variables|Default|GetResources%20Taken%20))
  (if (not (>= (Variables|/Game/ShadowDuckStudio/Blueprints/HealthSystem/AC_HealthComponent.AC_HealthComponent_C|GetCurrentHealth _ac_healthcomponent) (Variables|/Game/ShadowDuckStudio/Blueprints/HealthSystem/AC_HealthComponent.AC_HealthComponent_C|GetMaxHealth _ac_healthcomponent)))
    (if (< (Variables|Default|GetCurrentReloadTime) (Variables|Default|GetMaxReloadTime))
      (Variables|Default|SetCurrentReloadTime (+ (Variables|Default|GetCurrentReloadTime) (Variables|Default|GetReloadTickTime)))
      (else
        (Variables|Default|GetPlayerRef
          (:then
            _)
          (:else
            (bind _returnvalue (Actor|GetActorOfClass "/Game/ShadowDuckStudio/Blueprints/Player/BP_HMCharacter.BP_HMCharacter_C"))
            (Variables|Default|SetPlayerRef _returnvalue)))
        (if (< (.resource1 (Variables|/Game/ShadowDuckStudio/Blueprints/ResourcesSystem/AC_ResourceComponent.AC_ResourceComponent_C|GetResources (Variables|/Game/ShadowDuckStudio/Blueprints/Player/BP_HMCharacter.BP_HMCharacter_C|GetAC_ResourceComponent (Variables|Default|GetPlayerRef)))) _resources_taken_)
          (Development|PrintString "Returning true")
          (else
            (Default|TakeResource (Variables|/Game/ShadowDuckStudio/Blueprints/Player/BP_HMCharacter.BP_HMCharacter_C|GetAC_ResourceComponent (Variables|Default|GetPlayerRef)) (Utilities|Struct|MakeF_Resources _resources_taken_))
            (Class|BIHealthInterface|Heal(Message) (Variables|Default|GetAC_HealthComponent) (Variables|Default|GetReloadAmount))
            (Utilities|Time|ClearTimerbyFunctionName 0 "ReloadTick")
            (CallFunction|CheckRepairVisible)))))))

(fn GetOverlayMeshes
  (return 0))