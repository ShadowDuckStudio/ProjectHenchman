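; BP_MechanicCauser is an interactable, lever-style actor that switches linked world mechanics on and off.
; Interacting toggles its Active state and sends activate or deactivate messages to every actor in RelatedActors.
; When ActiveTime is positive, a looping TimerTick accumulates elapsed time and deactivates the lever automatically once it runs out.
; A sphere overlap shows its widget while an actor tagged Player is in range.
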(event OnComponentBeginOverlap(Sphere)
  (params (OverlappedComponent :type Primitive%20Component%20Object%20Reference) (OtherActor :type Actor%20Object%20Reference) (OtherComp :type Primitive%20Component%20Object%20Reference) (OtherBodyIndex :type Integer) (bFromSweep :type Boolean) (SweepResult :type Hit%20Result%20Structure%20%28by%20ref%29))
  (if (Actor|ActorHasTag OtherActor "Player")
    (Rendering|SetVisibility (Variables|Default|GetWidget) true false)))

(event OnComponentEndOverlap(Sphere)
  (params (OverlappedComponent :type Primitive%20Component%20Object%20Reference) (OtherActor :type Actor%20Object%20Reference) (OtherComp :type Primitive%20Component%20Object%20Reference) (OtherBodyIndex :type Integer))
  (if (Actor|ActorHasTag OtherActor "Player")
    (Rendering|SetVisibility (Variables|Default|GetWidget) false false)))

(event Custom|ActivateLever
  (Variables|Default|SetActive? true)
  (for _array_element (Variables|Default|GetRelatedActors)
    (Class|BIWorldMechanicInterface|ActivateWorldMechanic(Message) _array_element)
    (if (> (Variables|Default|GetActiveTime) 0.0)
      (Variables|Default|SetCurrentTime 0.0)
      (Utilities|Time|SetTimerbyFunctionName 0 "TimerTick" (Variables|Default|GetTickTime) true))))

(event Custom|DeactivateLever
  (Utilities|Time|ClearTimerbyFunctionName 0 "TimerTick")
  (Variables|Default|SetActive? false)
  (for _array_element (Variables|Default|GetRelatedActors)
    (Class|BIWorldMechanicInterface|DeactivateWorldMechanic(Message) _array_element)))

(event EventBeginPlay)

(event Collision|EventActorBeginOverlap
  (params (OtherActor :type Actor%20Object%20Reference)))

(event EventTick
  (params (DeltaSeconds :type Float%20%28single-precision%29)))

(event EventBeginInteract
  (params (Source :type Actor%20Object%20Reference))
  (if (not (Variables|Default|GetActive?))
    (CallFunction|ActivateLever)
    (else
      (CallFunction|DeactivateLever))))

(fn ConstructionScript)

(fn TimerTick
  (if (< (Variables|Default|GetCurrentTime) (Variables|Default|GetActiveTime))
    (Variables|Default|SetCurrentTime (+ (Variables|Default|GetCurrentTime) (Variables|Default|GetTickTime)))
    (else
      (CallFunction|DeactivateLever))))

(fn GetOverlayMeshes
  (return 0))