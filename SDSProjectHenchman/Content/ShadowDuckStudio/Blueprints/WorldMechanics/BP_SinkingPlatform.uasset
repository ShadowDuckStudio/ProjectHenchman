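; Sinking platform world mechanic that moves to a target transform when activated, then returns to where it started.
; ActivateWorldMechanic runs a timeline that lerps from the transform cached at BeginPlay to NewTransform, waits for Length, then a second timeline lerps back.
; Both timelines play at a rate of 1/MoveSpeed, so higher values mean slower movement.
; A CanActivate flag blocks retriggering until the return finishes.
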(event EventBeginPlay
  (Variables|Default|SetOriginalTransform (Transformation|GetActorTransform)))

(event Collision|EventActorBeginOverlap
  (params (OtherActor :type Actor%20Object%20Reference)))

(event EventTick
  (params (DeltaSeconds :type Float%20%28single-precision%29)))

(event EventActivateWorldMechanic
  (if (Variables|Default|GetCanActivate?)
    (Variables|Default|SetCanActivate? false)
    (Components|Timeline|SetPlayRate (Variables|Default|GetTimeline) (/ 1.0 (Variables|Default|GetMoveSpeed)))
    (bind _newtrack_0 (Timeline|Timeline PlayFromStart)
      (:Update
        (Transformation|SetActorTransform (Math|Transform|Lerp(Transform) (Variables|Default|GetOriginalTransform) (Variables|Default|GetNewTransform) _newtrack_0)))
      (:Finished
        (Utilities|FlowControl|Delay (Variables|Default|GetLength))
        (Components|Timeline|SetPlayRate (Variables|Default|GetTimeline_0) (/ 1.0 (Variables|Default|GetMoveSpeed)))
        (bind _newtrack_0_2 (Timeline|Timeline_0 PlayFromStart)
          (:Update
            (Transformation|SetActorTransform (Math|Transform|Lerp(Transform) (Variables|Default|GetNewTransform) (Variables|Default|GetOriginalTransform) _newtrack_0_2)))
          (:Finished
            (Variables|Default|SetCanActivate? true)))))))

(fn ConstructionScript)