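; Trigger volume that switches the player's equipment on entry and exit, presumably to the pickaxe inside and back to the hammer outside.
; Entering SwapCollision ends any active build through AC_BuildComponent, then sets the character's EquipEnum and calls EquipmentSwap on its equip component.
; Leaving sets the other enum value and swaps again; both swaps are skipped while a switch is already in progress.
; Older direct hammer/pickaxe swap and sheath chains remain unconnected.
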(event OnComponentBeginOverlap(SwapCollision)
  (params (OverlappedComponent :type Primitive%20Component%20Object%20Reference) (OtherActor :type Actor%20Object%20Reference) (OtherComp :type Primitive%20Component%20Object%20Reference) (OtherBodyIndex :type Integer) (bFromSweep :type Boolean) (SweepResult :type Hit%20Result%20Structure%20%28by%20ref%29))
  (bind _returnvalue (Game|Player|GetPlayerPawn 0))
  (bind _asbp_hmcharacter (Utilities|Casting|CastToBP_HMCharacter _returnvalue))
  (bind _ac_equipcomponent (Variables|/Game/ShadowDuckStudio/Blueprints/Player/BP_HMCharacter.BP_HMCharacter_C|GetAC_EquipComponent _asbp_hmcharacter))
  (if (Actor|ActorHasTag OtherActor "Player")
    (Default|EndBuild (Actor|GetComponentbyClass (Game|Player|GetPlayerPawn 0) "/Game/ShadowDuckStudio/Blueprints/BuildSystem/AC_BuildComponent.AC_BuildComponent_C"))
    (if (not (Variables|/Game/ShadowDuckStudio/Blueprints/Player/EquipSystem/AC_EquipComponent.AC_EquipComponent_C|GetIsSwitchingEquipment _ac_equipcomponent))
      (Variables|/Game/ShadowDuckStudio/Blueprints/Player/EquipSystem/AC_EquipComponent.AC_EquipComponent_C|SetEquipEnum _ac_equipcomponent "NewEnumerator1")
      (Default|EquipmentSwap _ac_equipcomponent))))

(event OnComponentEndOverlap(SwapCollision)
  (params (OverlappedComponent :type Primitive%20Component%20Object%20Reference) (OtherActor :type Actor%20Object%20Reference) (OtherComp :type Primitive%20Component%20Object%20Reference) (OtherBodyIndex :type Integer))
  (bind _returnvalue (Game|Player|GetPlayerPawn 0))
  (bind _asbp_hmcharacter (Utilities|Casting|CastToBP_HMCharacter _returnvalue))
  (bind _ac_equipcomponent (Variables|/Game/ShadowDuckStudio/Blueprints/Player/BP_HMCharacter.BP_HMCharacter_C|GetAC_EquipComponent _asbp_hmcharacter))
  (if (Actor|ActorHasTag OtherActor "Player")
    (if (not (Variables|/Game/ShadowDuckStudio/Blueprints/Player/EquipSystem/AC_EquipComponent.AC_EquipComponent_C|GetIsSwitchingEquipment _ac_equipcomponent))
      (Variables|/Game/ShadowDuckStudio/Blueprints/Player/EquipSystem/AC_EquipComponent.AC_EquipComponent_C|SetEquipEnum _ac_equipcomponent "NewEnumerator0")
      (Default|EquipmentSwap _ac_equipcomponent))))

(event EventBeginPlay
  (bind _returnvalue (Actor|GetActorOfClass "/Game/ShadowDuckStudio/Blueprints/Player/BP_HMCharacter.BP_HMCharacter_C"))
  (Variables|Default|SetCharRef _returnvalue))

(event Collision|EventActorBeginOverlap
  (params (OtherActor :type Actor%20Object%20Reference)))

(event EventTick
  (params (DeltaSeconds :type Float%20%28single-precision%29)))

(fn ConstructionScript)