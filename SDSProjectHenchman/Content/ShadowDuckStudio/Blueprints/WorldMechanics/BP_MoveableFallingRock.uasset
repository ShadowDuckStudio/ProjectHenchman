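; BP_MoveableFallingRock is a world mechanic rock that falls when activated and swaps the player's equipment near it.
; ActivateWorldMechanic starts the rockfall Niagara effect and calls BeginMove, then after timed delays marks the rock fallen, shows its minimap icon, and cleans up the effect.
; Box overlaps switch the player to the pickaxe on entry and from pickaxe to hammer on exit, unless equipment is already switching.
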(event OnComponentBeginOverlap(Box)
  (params (OverlappedComponent :type Primitive%20Component%20Object%20Reference) (OtherActor :type Actor%20Object%20Reference) (OtherComp :type Primitive%20Component%20Object%20Reference) (OtherBodyIndex :type Integer) (bFromSweep :type Boolean) (SweepResult :type Hit%20Result%20Structure%20%28by%20ref%29))
  (bind _returnvalue (Game|Player|GetPlayerPawn 0))
  (bind _asbp_hmcharacter (Utilities|Casting|CastToBP_HMCharacter _returnvalue))
  (bind _ac_equipcomponent (Variables|/Game/ShadowDuckStudio/Blueprints/Player/BP_HMCharacter.BP_HMCharacter_C|GetAC_EquipComponent _asbp_hmcharacter))
  (if (Actor|ActorHasTag OtherActor "Player")
    (if (not (Variables|/Game/ShadowDuckStudio/Blueprints/Player/EquipSystem/AC_EquipComponent.AC_EquipComponent_C|GetIsSwitchingEquipment _ac_equipcomponent))
      (if (Variables|/Game/ShadowDuckStudio/Blueprints/Player/EquipSystem/AC_EquipComponent.AC_EquipComponent_C|GetHasHammerEquipped? _ac_equipcomponent)
        (Default|PickaxeSwap _ac_equipcomponent)
        (else
          (Default|PickaxeSwap _ac_equipcomponent))))))

(event OnComponentEndOverlap(Box)
  (params (OverlappedComponent :type Primitive%20Component%20Object%20Reference) (OtherActor :type Actor%20Object%20Reference) (OtherComp :type Primitive%20Component%20Object%20Reference) (OtherBodyIndex :type Integer))
  (bind _returnvalue (Game|Player|GetPlayerPawn 0))
  (bind _asbp_hmcharacter (Utilities|Casting|CastToBP_HMCharacter _returnvalue))
  (bind _ac_equipcomponent (Variables|/Game/ShadowDuckStudio/Blueprints/Player/BP_HMCharacter.BP_HMCharacter_C|GetAC_EquipComponent _asbp_hmcharacter))
  (if (Actor|ActorHasTag OtherActor "Player")
    (if (not (Variables|/Game/ShadowDuckStudio/Blueprints/Player/EquipSystem/AC_EquipComponent.AC_EquipComponent_C|GetIsSwitchingEquipment (Variables|/Game/ShadowDuckStudio/Blueprints/Player/BP_HMCharacter.BP_HMCharacter_C|GetAC_EquipComponent _asbp_hmcharacter)))
      (if (Variables|/Game/ShadowDuckStudio/Blueprints/Player/EquipSystem/AC_EquipComponent.AC_EquipComponent_C|GetHasPickaxeEquipped? _ac_equipcomponent)
        (Default|HammerSwap _ac_equipcomponent)))))

(event Custom|MakeMinimapIconVisible
  (bind _fallenrockminimapicon (Variables|Default|GetFallenRockMinimapIcon))
  (if (Variables|Default|GetRockFallen)
    (Rendering|SetVisibility _fallenrockminimapicon true false)
    (else
      (Rendering|SetVisibility _fallenrockminimapicon false false))))

(event EventBeginPlay
  (|CallParentFunction)
  (bind _returnvalue (Actor|GetActorOfClass "/Game/ShadowDuckStudio/Blueprints/Player/BP_HMCharacter.BP_HMCharacter_C"))
  (Variables|Default|SetCharRef _returnvalue))

(event Collision|EventActorBeginOverlap
  (params (OtherActor :type Actor%20Object%20Reference))
  (|CallParentFunction OtherActor) ; This node is disabled and will not be called.\nDrag off pins to build functionality.
)

(event EventTick
  (params (DeltaSeconds :type Float%20%28single-precision%29))
  (|CallParentFunction DeltaSeconds) ; This node is disabled and will not be called.\nDrag off pins to build functionality.
)

(event EventActivateWorldMechanic
  (bind _fxs_rockfalling (Variables|Default|GetFXS_RockFalling))
  (Components|Activation|Activate _fxs_rockfalling true)
  (Utilities|FlowControl|Delay 0.3)
  (CallFunction|BeginMove)
  (Utilities|FlowControl|Delay 7.0)
  (Variables|Default|SetRockFallen true)
  (CallFunction|MakeMinimapIconVisible)
  (Niagara|SetNiagaraVariable(Bool) _fxs_rockfalling "Kill Particles" true)
  (Utilities|FlowControl|Delay 1e+01)
  (Components|DestroyComponent _fxs_rockfalling))

(fn ConstructionScript
  (|CallParentFunction))