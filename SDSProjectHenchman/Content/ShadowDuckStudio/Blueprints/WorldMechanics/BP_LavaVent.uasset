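; Lava vent world mechanic that toggles a lava flow, revealing it only when BP_LavaMechanic's lava value meets LavaCost.
; Activation runs a timeline driving MPC_LavaFlow, unhides StaticMesh's children and fades in audio; finishing re-enables query collision only on the loop's last element.
; Deactivation hides the children, disables their collision and fades audio out.
; ACDamageOverlap receives the lava meshes; LavaTick, uncalled here, damages overlapping actors' health components.
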(event Custom|No%20Collision
  (for _array_element (Components|GetChildrenComponents (Variables|Default|GetStaticMesh) false)
    (bind _asprimitive_component (Utilities|Casting|CastToPrimitiveComponent _array_element))
    (Collision|SetCollisionEnabled _asprimitive_component "NoCollision")))

(event EventBeginPlay
  (bind _returnvalue (Actor|GetActorOfClass "/Game/ShadowDuckStudio/Blueprints/WorldMechanics/BP_LavaMechanic.BP_LavaMechanic_C"))
  (Variables|Default|SetLavaManager _returnvalue)
  (Class|BIWorldMechanicInterface|DeactivateWorldMechanic(Message) self)
  (Default|MakeLava (Variables|Default|GetAC_DamageOverlap) (Utilities|Array|MakeArray (Variables|Default|GetSM_Lava_Bend) (Variables|Default|GetSM_Lava_Straight))))

(event Collision|EventActorBeginOverlap
  (params (OtherActor :type Actor%20Object%20Reference)))

(event EventTick
  (params (DeltaSeconds :type Float%20%28single-precision%29)))

(event EventActivateWorldMechanic
  (if (not (Variables|Default|GetActive?))
    (CallFunction|NoCollision)
    (Rendering|Material|SetScalarParameterValue "/Game/ShadowDuckStudio/VFX/Materials/MPC_LavaFlow.MPC_LavaFlow" "BlockAlpha" 0.0 :!class /Script/Engine.KismetMaterialLibrary)
    (bind _newtrack_0 (Timeline|Timeline PlayFromStart)
      (:Update
        (Rendering|Material|SetScalarParameterValue "/Game/ShadowDuckStudio/VFX/Materials/MPC_LavaFlow.MPC_LavaFlow" "AlphaFlow1" _newtrack_0 :!class /Script/Engine.KismetMaterialLibrary)
        (bind _lava (Class|BIWorldMechanicInterface|CheckLavaValue(Message) (Variables|Default|GetLavaManager)))
        (if (>= _lava (Variables|Default|GetLavaCost))
          (for _array_element (Components|GetChildrenComponents (Variables|Default|GetStaticMesh) false)
            (Development|SetHiddeninGame _array_element false true))
          (Audio|Components|Audio|FadeIn (Variables|Default|GetLavaComingFromPipe_Cue) 2.0 1.0 0.0 "Linear" :!class /Script/Engine.AudioComponent)))
      (:Finished
        (Variables|Default|SetActive? true)
        (bind _asprimitive_component (Utilities|Casting|CastToPrimitiveComponent _array_element))
        (Collision|SetCollisionEnabled _asprimitive_component "QueryOnly")))
    (else
      (CallFunction|DeactivateWorldMechanic))))

(event EventDeactivateWorldMechanic
  (for _array_element (Components|GetChildrenComponents (Variables|Default|GetStaticMesh) false)
    (Development|SetHiddeninGame _array_element true true)
    (bind _asprimitive_component (Utilities|Casting|CastToPrimitiveComponent _array_element))
    (Collision|SetCollisionEnabled _asprimitive_component "NoCollision"))
  (Audio|Components|Audio|FadeOut (Variables|Default|GetLavaComingFromPipe_Cue) 2.0 0.0 "Linear" :!class /Script/Engine.AudioComponent)
  (Variables|Default|SetActive? false))

(fn ConstructionScript)

(fn LavaTick
  (for _array_element (Variables|Default|GetOverlappingActors)
    (Class|BIHealthInterface|Damage(Message) (Actor|GetComponentbyClass _array_element "/Game/ShadowDuckStudio/Blueprints/HealthSystem/AC_HealthComponent.AC_HealthComponent_C") (Variables|Default|GetDamagePerTick))))

(fn CheckLavaValue
  (return 0.0))