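; Game mode that sets up local multiplayer at BeginPlay by creating players and giving each a BP_Input pawn.
; It gathers all PlayerStarts and matches each array index against their PlayerStartTag converted to an integer.
; Each match creates a local player, spawns a pawn possessed by that index's controller, and records both.
; Spawn transforms come from the array slot at that index, rather than the tag-matched start.
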(event EventBeginPlay
  (CallFunction|FindPlayerStartPoints)
  (CallFunction|SpawnsInputsonPlayerStarts))

(fn ConstructionScript)

(fn FindPlayerStartPoints
  (bind _outactors (Actor|GetAllActorsOfClass "/Script/Engine.PlayerStart"))
  (Variables|Default|SetPlayerStartArray _outactors))

(fn SpawnsInputsonPlayerStarts
  (for (_ _array_index) (Variables|Default|GetPlayerStartArray)
    (LocalVariables|SetIndex%20Number _array_index)
    (for _array_element (Variables|Default|GetPlayerStartArray)
      (if (== (CallFunction|PlayerTagtoInterger _array_element) (LocalVariables|GetIndex%20Number))
        (Class|GameplayStatics|CreatePlayer -1)
        (bind _returnvalue (Game|SpawnActorfromClass "/Game/ShadowDuckStudio/Blueprints/Player/Coop_BPs/BP_Input.BP_Input_C" (Transformation|GetActorTransform (Utilities|Array|Get(acopy) (Variables|Default|GetPlayerStartArray) (LocalVariables|GetIndex%20Number))) "Undefined" "MultiplyWithRoot" 0 (LocalVariables|GetIndex%20Number) 0))
        (Utilities|Array|AddUnique (Variables|Default|GetInput%20Array) _returnvalue)
        (Pawn|Possess (Game|GetPlayerController (LocalVariables|GetIndex%20Number)) _returnvalue)
        (Utilities|Array|AddUnique (Variables|Default|GetPlayerControllerArray) (Game|GetPlayerController (LocalVariables|GetIndex%20Number)))))))

(fn PlayerTagtoInterger
  (params (Player%20Start%20Element :type Player%20Start%20Object%20Reference))
  (return (Math|Conversions|ToInteger(Byte) (Utilities|String|ToString(Name) (Variables|/Script/Engine.PlayerStart|GetPlayerStartTag Player%20Start%20Element)))))