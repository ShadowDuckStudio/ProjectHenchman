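; Manager actor that respawns the player character at the respawn point nearest to where they died.
; On BeginPlay it caches all BP_RespawnPoint actors; SetRespawnLocation records the death point.
; Respawn waits a delay, spawns a new BP_HMCharacter at the closest point, and has the first player controller possess it.
; It then creates the HUD and build hotbar widgets and refreshes the equip and hotbar UI.
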(event EventBeginPlay
  (bind _outactors (Actor|GetAllActorsOfClass "/Game/ShadowDuckStudio/Blueprints/Player/RespawnSystem/BP_RespawnPoint.BP_RespawnPoint_C"))
  (Variables|Default|SetRespawnPoints _outactors))

(event Collision|EventActorBeginOverlap
  (params (OtherActor :type Actor%20Object%20Reference)))

(event EventTick
  (params (DeltaSeconds :type Float%20%28single-precision%29)))

(event EventRespawn
  (bind _returnvalue (Game|GetPlayerController 0))
  (Utilities|FlowControl|Delay (Variables|Default|GetRespawnTime))
  (bind _returnvalue_2 (Game|SpawnActorfromClass "/Game/ShadowDuckStudio/Blueprints/Player/BP_HMCharacter.BP_HMCharacter_C" (Transformation|GetActorTransform (.ReturnValue (Actor|FindNearestActor (Variables|Default|GetDeathPoint) (Variables|Default|GetRespawnPoints)))) "AlwaysSpawn" "MultiplyWithRoot" 0 0))
  (Default|SetManager _returnvalue_2)
  (Pawn|Possess _returnvalue _returnvalue_2)
  (Default|SetManager _returnvalue_2)
  (bind _returnvalue_3 (UserInterface|CreateWidget "/Game/ShadowDuckStudio/UI/Widgets/HUD_WBP.HUD_WBP_C" _returnvalue))
  (UserInterface|Viewport|AddtoViewport _returnvalue_3 0)
  (bind _returnvalue_4 (UserInterface|CreateWidget "/Game/ShadowDuckStudio/UI/Widgets/BuildableHotBar_WBP.BuildableHotBar_WBP_C" _returnvalue (Variables|/Game/ShadowDuckStudio/Blueprints/BuildSystem/AC_BuildComponent.AC_BuildComponent_C|GetSelectedHotbar (Variables|/Game/ShadowDuckStudio/Blueprints/Player/BP_HMCharacter.BP_HMCharacter_C|GetAC_BuildComponent _returnvalue_2)) (Variables|/Game/ShadowDuckStudio/Blueprints/BuildSystem/AC_BuildComponent.AC_BuildComponent_C|GetBuildList (Variables|/Game/ShadowDuckStudio/Blueprints/Player/BP_HMCharacter.BP_HMCharacter_C|GetAC_BuildComponent _returnvalue_2))))
  (UserInterface|Viewport|AddtoViewport _returnvalue_4 0)
  (Default|EquipUIRefresh (Variables|/Game/ShadowDuckStudio/Blueprints/Player/BP_HMCharacter.BP_HMCharacter_C|GetAC_EquipComponent _returnvalue_2))
  (Default|UpdateHotbarUI (Variables|/Game/ShadowDuckStudio/Blueprints/Player/BP_HMCharacter.BP_HMCharacter_C|GetAC_BuildComponent _returnvalue_2)))

(event EventSetRespawnLocation
  (params (DeathPoint :type Vector :default "0, 0, 0"))
  (Variables|Default|SetDeathPoint DeathPoint))

(fn ConstructionScript)