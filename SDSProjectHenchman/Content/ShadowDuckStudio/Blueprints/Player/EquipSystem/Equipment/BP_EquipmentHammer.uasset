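; Hammer equipment Blueprint that knocks away and damages what its head hits.
; A timeline grows and shrinks the head and base mesh through IncreaseSize and DecreaseSize.
; Head cylinder overlaps skip ignored classes, the player and already-hit actors, and only register while CanHit is false.
; Hits launch characters or impulse physics components along the Arrow's forward vector, then send damage to any AC_HealthComponent.
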(event OnComponentBeginOverlap(HeadCollisionCylinder)
  (params (OverlappedComponent :type Primitive%20Component%20Object%20Reference) (OtherActor :type Actor%20Object%20Reference) (OtherComp :type Primitive%20Component%20Object%20Reference) (OtherBodyIndex :type Integer) (bFromSweep :type Boolean) (SweepResult :type Hit%20Result%20Structure%20%28by%20ref%29))
  (bind _returnvalue (Actor|GetComponentbyClass OtherActor "/Game/ShadowDuckStudio/Blueprints/HealthSystem/AC_HealthComponent.AC_HealthComponent_C"))
  (bind _impulsestrength (Variables|Default|GetImpulseStrength))
  (bind _arrow (Variables|Default|GetArrow))
  (bind _returnvalue_2 (Math|Vector|GetForwardVector _arrow))
  (bind _returnvalue_3 (* _returnvalue_2 _impulsestrength))
  (Development|PrintString (Utilities|GetDisplayName OtherActor))
  (if (not (Math|Boolean|ORBoolean (Utilities|Array|ContainsItem (Variables|Default|GetIgnoredClasses) (Utilities|GetClass OtherActor)) (== OtherActor (Game|GetPlayerCharacter 0)) (Utilities|Array|ContainsItem (Variables|Default|GetAllHitActors) OtherActor) (Variables|Default|GetCanHit?)))
    (bind _output_get (Variables|Default|SetHitActor OtherActor))
    (Utilities|Array|AddUnique (Variables|Default|GetAllHitActors) _output_get)
    (bind _ascharacter (Utilities|Casting|CastToCharacter OtherActor)
      (:then
        (Character|Jump _ascharacter)
        (Character|StopJumping _ascharacter)
        (Character|LaunchCharacter _ascharacter _returnvalue_3 false false))
      (:CastFailed
        (if (Class|SceneComponent|IsAnySimulatingPhysics OtherComp)
          (Physics|AddImpulse OtherComp _returnvalue_3 "None" true))))
    (Utilities|IsValid _returnvalue
      (:Is%20Valid
        (Class|BIHealthInterface|Damage(Message) _returnvalue (Variables|Default|GetDamageTaken))))))

(event Custom|Increase%20Size
  (bind _size (Timeline|Timeline_0 PlayFromStart)
    (:Update
      (Transformation|SetRelativeTransform (Variables|Default|GetHead) (Math|Transform|MakeTransform "0, 0, 0" "0, 0, 0" (Math|Vector|Lerp(Vector) "1.000000,1.000000,1.000000" "2.000000,2.000000,2.000000" _size)) false false)
      (Transformation|SetRelativeTransform (Variables|Default|GetBaseStatic) (Math|Transform|MakeTransform "0, 0, 0" "0, 0, 0" (Math|Vector|Lerp(Vector) "0.020000,0.020000,0.020000" "0.050000,0.050000,0.050000" _size)) false false))))

(event Custom|Decrease%20Size
  (bind _size (Timeline|Timeline_0 Reverse)
    (:Update
      (Transformation|SetRelativeTransform (Variables|Default|GetHead) (Math|Transform|MakeTransform "0, 0, 0" "0, 0, 0" (Math|Vector|Lerp(Vector) "1.000000,1.000000,1.000000" "2.000000,2.000000,2.000000" _size)) false false)
      (Transformation|SetRelativeTransform (Variables|Default|GetBaseStatic) (Math|Transform|MakeTransform "0, 0, 0" "0, 0, 0" (Math|Vector|Lerp(Vector) "0.020000,0.020000,0.020000" "0.050000,0.050000,0.050000" _size)) false false))))

(event EventBeginPlay
  (|CallParentFunction) ; This node is disabled and will not be called.\nDrag off pins to build functionality.
)

(event Collision|EventActorBeginOverlap
  (params (OtherActor :type Actor%20Object%20Reference))
  (|CallParentFunction OtherActor) ; This node is disabled and will not be called.\nDrag off pins to build functionality.
)

(event EventTick
  (params (DeltaSeconds :type Float%20%28single-precision%29))
  (|CallParentFunction DeltaSeconds) ; This node is disabled and will not be called.\nDrag off pins to build functionality.
)

(fn ConstructionScript
  (|CallParentFunction))