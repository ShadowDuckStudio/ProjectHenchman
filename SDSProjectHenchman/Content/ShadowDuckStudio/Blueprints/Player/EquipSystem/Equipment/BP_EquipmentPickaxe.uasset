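; Pickaxe equipment actor for the player equip system that can grow and shrink its mesh.
; IncreaseSize plays a timeline from the start, using its Size track to lerp the BaseStatic component's relative scale from small to larger.
; DecreaseSize reverses the same timeline from its current position to shrink it back.
; No other active logic lives here beyond the parent construction script call.
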(event Custom|Increase%20Size
  (bind _size (Timeline|Timeline PlayFromStart)
    (:Update
      (Transformation|SetRelativeTransform (Variables|Default|GetBaseStatic) (Math|Transform|MakeTransform "0, 0, 0" "0, 0, 0" (Math|Vector|Lerp(Vector) "0.200000,0.200000,0.200000" "0.600000,0.600000,0.600000" _size)) false false))))

(event Custom|DecreaseSize
  (bind _size (Timeline|Timeline Reverse)
    (:Update
      (Transformation|SetRelativeTransform (Variables|Default|GetBaseStatic) (Math|Transform|MakeTransform "0, 0, 0" "0, 0, 0" (Math|Vector|Lerp(Vector) "0.200000,0.200000,0.200000" "0.600000,0.600000,0.600000" _size)) false false))))

(event EventBeginPlay
  (|CallParentFunction) ; This node is disabled and will not be called.\nDrag off pins to build functionality.
)

(event Collision|EventActorBeginOverlap
  (params (OtherActor :type Actor%20Object%20Reference))
  (|CallParentFunction OtherActor) ; This node is disabled and will not be called.\nDrag off pins to build functionality.
)

(event EventTick
  (params (DeltaSeconds :type Float%20%28single-precision%29))
  (|CallParentFunction DeltaSeconds) ; This node is disabled and will not be called.\nDrag off pins to build functionality.
)

(fn ConstructionScript
  (|CallParentFunction))