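; Player equipment component that manages a hammer and pickaxe for attacking and mining.
; It spawns both tools, attaches pickups to mesh sockets, and swaps them through draw/sheath montages that update flags and refresh the toolbar widget.
; Action input plays the equipped tool's montage, enabling hammer hits or collecting the targeted resource.
; Mining-range overlaps maintain a resource list; entering actors can retarget the nearest resource, highlighted with an overlay material.
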(event Custom|HammerSwap
  ;[0.04417 1 0] Equip/Unequip Equipment based on Equipment Name
  (Variables|Default|GetEquipment_Pickup
    (:then
      (Variables|Default|GetHammer
        (:then
          (if (not (Variables|Default|GetIsSwitchingEquipment))
            (Variables|Default|SetIsSwitchingEquipment true)
            (switch name (Variables|Default|GetEquipmentName)
              (:Hammer
                (CallFunction|SheathHammer))
              (:None
                (CallFunction|DrawHammer))
              (:Pickaxe
                (CallFunction|SheathPickaxe)
                (Utilities|FlowControl|Delay 0.5)
                (CallFunction|DrawHammer)))))
        (:else)))
    (:else)))

(event Custom|PickaxeSwap
  ;[0.04417 1 0] Equip/Unequip Equipment based on Equipment Name
  (Variables|Default|GetEquipment_Pickup
    (:then
      (Variables|Default|GetPickaxe
        (:then
          (if (not (Variables|Default|GetIsSwitchingEquipment))
            (Variables|Default|SetIsSwitchingEquipment true)
            (switch name (Variables|Default|GetEquipmentName)
              (:Hammer
                (CallFunction|SheathHammer)
                (Utilities|FlowControl|Delay 0.5)
                (CallFunction|DrawPickaxe))
              (:None
                (CallFunction|DrawPickaxe))
              (:Pickaxe
                (CallFunction|SheathPickaxe)))))
        (:else)))
    (:else)))

(event Custom|HammerAttack
  (bind _hammer (Variables|Default|GetHammer))
  (bind _asbp_equipment_hammer (Utilities|Casting|CastToBP_EquipmentHammer _hammer))
  ;[0 1 1] Equipment Use
  ;;[0 1 0] Hammer Primary Use
  (Variables|/Game/ShadowDuckStudio/Blueprints/Player/EquipSystem/Equipment/BP_EquipmentHammer.BP_EquipmentHammer_C|SetAllHitActors _asbp_equipment_hammer (Utilities|Array|MakeArray 0))
  (Variables|/Game/ShadowDuckStudio/Blueprints/Player/EquipSystem/Equipment/BP_EquipmentHammer.BP_EquipmentHammer_C|SetCanHit? _asbp_equipment_hammer true)
  (Variables|Default|SetActionInput true)
  (Animation|Montage|PlayMontage (Variables|Default|GetMesh) "/Game/ShadowDuckStudio/Assets/Characters/Player/P_Anim/SK_Player_P_HammerAttack_Montage.SK_Player_P_HammerAttack_Montage"
    (:OnCompleted
      _)
    (:OnInterrupted
      _))
  (Variables|/Game/ShadowDuckStudio/Blueprints/Player/EquipSystem/Equipment/BP_EquipmentHammer.BP_EquipmentHammer_C|SetCanHit? _asbp_equipment_hammer false)
  (Variables|Default|SetActionInput false))

(event Custom|MiningAction
  (params (Actor :type Object%20Object%20Reference))
  ;[0 1 1] Equipment Use
  ;;[0 1 0] Pickaxe Primary Use
  (Variables|Default|SetActionInput true)
  (Animation|Montage|PlayMontage (Variables|Default|GetMesh) "/Game/ShadowDuckStudio/Assets/Characters/Player/P_Anim/SK_Player_P_PickaxeAttack_Montage.SK_Player_P_PickaxeAttack_Montage"
    (:then
      (Utilities|FlowControl|DoOnce false :!label _label
        (:Completed
          (Utilities|FlowControl|Delay 1.0)
          (Variables|Default|SetActionInput false)
          (Variables|Default|SetMining true)
          (bind _resourceref (Variables|Default|GetResourceRef)
            (:then
              (Default|Collect _resourceref)
              (Variables|Default|SetMining false))
            (:else
              (Development|PrintString (Utilities|String|Append "HitResource: " (Utilities|GetDisplayName _resourceref))))))))
    (:OnCompleted
      (goto _label Reset))
    (:OnInterrupted
      (Variables|Default|SetActionInput false))))

(event Custom|Draw%20Pickaxe
  ;[0 1 1] Pickaxe Equip Code
  ;;[0.04417 1 0] Equip Pickaxe Montage
  (Animation|Montage|PlayMontage (Variables|Default|GetMesh) "/Game/ShadowDuckStudio/Blueprints/Player/EquipSystem/Animation/Montages/PickaxeEquipMontage.PickaxeEquipMontage"
    (:then
      (Variables|Default|SetEquipmentName "Pickaxe")
      (Variables|Default|SetHasPickaxeEquipped? true)
      (CallFunction|EquipUIRefresh))
    (:OnCompleted
      (Variables|Default|SetIsSwitchingEquipment false))
    (:OnNotifyEnd
      (Default|IncreaseSize (stale Custom|MakeEquipment _returnvalue_3)))))

(event Custom|Sheath%20Pickaxe
  ;[0 1 1] Pickaxe Equip Code
  ;;[0.04417 1 0] Unequip Pickaxe Montage
  (Animation|Montage|PlayMontage (Variables|Default|GetMesh) "/Game/ShadowDuckStudio/Blueprints/Player/EquipSystem/Animation/Montages/PickaxeSheathMontage.PickaxeSheathMontage"
    (:then
      (Variables|Default|SetEquipmentName "None")
      (Variables|Default|SetHasPickaxeEquipped? false)
      (CallFunction|EquipUIRefresh))
    (:OnCompleted
      (Variables|Default|SetIsSwitchingEquipment false))))

(event Custom|DestroyPick
  ;[0 1 0] Destroy Equipment Actors
  (bind _pickaxe (Variables|Default|GetPickaxe)
    (:then
      (Actor|DestroyActor _pickaxe))
    (:else)))

(event Custom|DestroyHammer
  ;[0 1 0] Destroy Equipment Actors
  (bind _hammer (Variables|Default|GetHammer)
    (:then
      (Actor|DestroyActor _hammer))
    (:else)))

(event Custom|DestroyPickup
  ;[0 1 0] Destroy Equipment Actors
  (bind _equipment_pickup (Variables|Default|GetEquipment_Pickup)
    (:then
      (Actor|DestroyActor _equipment_pickup))
    (:else)))

(event Custom|RemoveBlue
  (params (NewParam :type Array%20of%20Actor%20Object%20References))
  (Utilities|Array|RemoveItem NewParam (stale _array_element)))

(event Custom|BeginMiningOverlap
  (params (OverlappedComponent :type Primitive%20Component%20Object%20Reference) (OtherActor :type Actor%20Object%20Reference) (OtherComp :type Primitive%20Component%20Object%20Reference) (OtherBodyIndex :type Integer) (bFromSweep :type Boolean) (SweepResult :type Hit%20Result%20Structure%20%28by%20ref%29))
  (bind _arrayempty_ (CallFunction|Add/RemoveArray (Variables|Default|GetResourcesInRange) OtherActor "NewEnumerator0" (Variables|Default|GetSpecial%20Classes) "NewEnumerator1"))
  (if (not _arrayempty_)
    (CallFunction|SetClosestResource)))

(event Custom|EndMiningOverlap
  (params (OverlappedComponent :type Primitive%20Component%20Object%20Reference) (OtherActor :type Actor%20Object%20Reference) (OtherComp :type Primitive%20Component%20Object%20Reference) (OtherBodyIndex :type Integer))
  (CallFunction|Add/RemoveArray (Variables|Default|GetResourcesInRange) OtherActor "NewEnumerator1" (Variables|Default|GetSpecial%20Classes) "NewEnumerator1"))

(event Custom|AttachEquipment
  (bind _owner (Variables|Default|GetOwner))
  ;[1 0 0.9168] Spawns collided actor to character using the attach to player function using the name of the socket that the equipment has set
  (bind _returnvalue (Game|SpawnActorfromClass (Utilities|GetClass (Variables|Default|GetEquipment_Pickup)) (Transformation|GetActorTransform _owner) "AlwaysSpawn" "MultiplyWithRoot" _owner 0))
  (Variables|Default|SetEquipment_Pickup _returnvalue)
  (switch name (Variables|/Game/ShadowDuckStudio/Blueprints/Player/EquipSystem/Equipment/BP_Equipment_Base.BP_Equipment_Base_C|GetEquipment%20Name _returnvalue)
    (:Hammer
      (bind _output_get (Variables|Default|SetHammer (Variables|Default|GetEquipment_Pickup)))
      (CallFunction|AttachEquipment _output_get))
    (:Pickaxe
      (bind _output_get_2 (Variables|Default|SetPickaxe (Variables|Default|GetEquipment_Pickup)))
      (CallFunction|AttachEquipment _output_get_2))))

(event Custom|MakeEquipment
  (bind _returnvalue (Math|Transform|MakeTransform "0, 0, 0"))
  ;[0 1 0] Make Equipment
  (bind _returnvalue_2 (Game|SpawnActorfromClass "/Game/ShadowDuckStudio/Blueprints/Player/EquipSystem/Equipment/BP_EquipmentHammer.BP_EquipmentHammer_C" _returnvalue "Undefined" "MultiplyWithRoot" 0 0))
  (bind _returnvalue_3 (Game|SpawnActorfromClass "/Game/ShadowDuckStudio/Blueprints/Player/EquipSystem/Equipment/BP_EquipmentPickaxe.BP_EquipmentPickaxe_C" _returnvalue "Undefined" "MultiplyWithRoot" 0 0))
  (Variables|Default|SetHammer _returnvalue_2)
  (Variables|Default|SetPickaxe _returnvalue_3)
  (Class|BIInteract|BeginInteract(Message) _returnvalue_3 (Variables|Default|GetOwner))
  (Default|BeginInteract _returnvalue_2 (Variables|Default|GetOwner)))

(event Custom|SheathHammer
  ;[0 1 1] Hammer Equip Code
  ;;[0.04417 1 0] Unequip Hammer Montage
  (Animation|Montage|PlayMontage (Variables|Default|GetMesh) "/Game/ShadowDuckStudio/Blueprints/Player/EquipSystem/Animation/Montages/HammerSheathMontage.HammerSheathMontage"
    (:then
      (Variables|Default|SetEquipmentName "None")
      (Variables|Default|SetHasHammerEquipped? false)
      (CallFunction|EquipUIRefresh))
    (:OnCompleted
      (Variables|Default|SetIsSwitchingEquipment false))
    (:OnNotifyBegin
      (Default|DecreaseSize (.AsBP%20Equipment%20Hammer (Utilities|Casting|CastToBP_EquipmentHammer (Variables|Default|GetHammer)))))))

(event Custom|DestroyAllEquipment
  ;[0 1 0] Destroy Equipment Actors
  (CallFunction|DestroyPick)
  (CallFunction|DestroyHammer)
  (CallFunction|DestroyPickup))

(event Custom|DrawHammer
  ;[0 1 1] Hammer Equip Code
  ;;[0.04417 1 0] Equip Hammer Montage
  (Animation|Montage|PlayMontage (Variables|Default|GetMesh) "/Game/ShadowDuckStudio/Blueprints/Player/EquipSystem/Animation/Montages/HammerEquipMontage.HammerEquipMontage"
    (:then
      (Variables|Default|SetEquipmentName "Hammer")
      (Variables|Default|SetHasHammerEquipped? true)
      (CallFunction|EquipUIRefresh))
    (:OnCompleted
      (Variables|Default|SetIsSwitchingEquipment false))
    (:OnNotifyEnd
      (Default|IncreaseSize (stale Custom|MakeEquipment _returnvalue_2)))))

(event EventBeginPlay
  (bind _miningrange (Variables|Default|GetMiningRange))
  (Variables|Default|SetOwner (Components|GetOwner))
  (Utilities|FlowControl|Delay 0.2)
  (CallFunction|MakeEquipment)
  (CallFunction|EquipUIRefresh)
  (Collision|BindEventtoOnComponentBeginOverlap _miningrange (delegate Custom|BeginMiningOverlap))
  (Collision|BindEventtoOnComponentEndOverlap _miningrange (delegate Custom|EndMiningOverlap)))

(fn AttachEquipment
  (params (Equipment :type BP%20Equipment%20Base%20Object%20Reference))
  (for _array_element (Actor|GetComponentsByClass Equipment "/Script/Engine.PrimitiveComponent")
    _)
  (Default|AttachtoPlayer Equipment (Variables|/Game/ShadowDuckStudio/Blueprints/Player/EquipSystem/Equipment/BP_Equipment_Base.BP_Equipment_Base_C|GetAttachEquipmentToBack Equipment) (Variables|Default|GetMesh)))

(fn ActionInputEvent
  (if (not (Variables|Default|GetActionInput))
    (Utilities|IsValid (Variables|Default|GetEquipment_Pickup)
      (:Is%20Valid
        (if (not (Variables|Default|GetIsSwitchingEquipment))
          (switch name (Variables|Default|GetEquipmentName)
            (:Hammer
              (CallFunction|HammerAttack))
            (:Pickaxe
              (CallFunction|MiningAction))))))))

(fn EquipUIRefresh
  (bind _toolbarref (Variables|Default|GetToolbarRef)
    (:then
      (Default|RefreshToolbar _toolbarref))
    (:else
      (bind _returnvalue (UserInterface|CreateWidget "/Game/ShadowDuckStudio/UI/Archived/ToolHotBar_WBP.ToolHotBar_WBP_C" 0 self))
      (bind _output_get (Variables|Default|SetToolbarRef _returnvalue))
      (Default|RefreshToolbar _output_get))))

(fn SetClosestResource
  (bind _resourcesinrange (Variables|Default|GetResourcesInRange))
  (bind _owner (Variables|Default|GetOwner))
  (bind _returnvalue (Transformation|GetActorLocation _owner))
  (bind _returnvalue_2 (Actor|FindNearestActor _returnvalue _resourcesinrange))
  (bind _asbp_resource_base (Utilities|Casting|CastToBP_ResourceBase _returnvalue_2))
  (Development|PrintString (Utilities|String|Append "FoundResource: " (Utilities|GetDisplayName _returnvalue_2)))
  (bind _resourceref (Variables|Default|GetResourceRef)
    (:then
      (if (not (== _resourceref _returnvalue_2))
        (for _array_element (Actor|GetComponentsByClass _resourceref "/Script/Engine.MeshComponent")
          (Rendering|Material|SetOverlayMaterial _array_element 0 :!class /Script/Engine.MeshComponent))
        (Utilities|IsValid _asbp_resource_base :!label _label
          (:Is%20Valid
            (bind _output_get (Variables|Default|SetResourceRef _asbp_resource_base))
            (for _array_element_2 (Actor|GetComponentsByClass _output_get "/Script/Engine.MeshComponent")
              (Rendering|Material|SetOverlayMaterial _array_element_2 "/Engine/ArtTools/RenderToTexture/Materials/M_RadiusDebugTranslucent.M_RadiusDebugTransLucent" :!class /Script/Engine.MeshComponent)))
          (:Is%20Not%20Valid
            (Variables|Default|SetResourceRef 0)))
        (return)))
    (:else
      (goto _label))))