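; BP_Wall_Base is a base wall actor that can be repaired through interaction and is destroyed on death.
; Beginning an interaction starts a looping timer that calls RepairTick, which heals the wall's health component by a set amount until the interaction ends.
; The Death event destroys the actor, while GetOverlayMeshes and the construction script are left empty.
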(event EventBeginPlay)

(event Collision|EventActorBeginOverlap
  (params (OtherActor :type Actor%20Object%20Reference)))

(event EventTick
  (params (DeltaSeconds :type Float%20%28single-precision%29)))

(event EventBeginInteract
  (params (Source :type Actor%20Object%20Reference))
  (Utilities|Time|SetTimerbyFunctionName 0 "RepairTick" (Variables|Default|GetRepairTickTime) true))

(event EventEndInteract
  (params (Source :type Actor%20Object%20Reference))
  (Utilities|Time|ClearTimerbyFunctionName 0 "RepairTick"))

(event EventDeath
  (Actor|DestroyActor))

(fn ConstructionScript)

(fn RepairTick
  (Class|BIHealthInterface|Heal(Message) (Variables|Default|GetAC_HealthComponent) (Variables|Default|GetRepairTickAmount)))

(fn GetOverlayMeshes
  (return 0))