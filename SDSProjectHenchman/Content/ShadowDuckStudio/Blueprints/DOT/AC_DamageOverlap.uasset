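; Actor component that turns supplied meshes into lava-style damage-over-time areas.
; MakeLava binds mesh overlap events, which add or remove actors in OverlappedActors and use that result to start or clear a looping DamageTick timer.
; Each tick sends Damage to every overlapped actor's AC_HealthComponent.
; Entering also plays a lava sound and triggers on-fire VFX on tagged players and enemies.
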(event Custom|MakeLava
  (params (Meshes :type Array%20of%20Primitive%20Component%20Object%20References))
  (for _array_element Meshes
    (Collision|BindEventtoOnComponentBeginOverlap _array_element (EventDispatchers|CreateEvent :!event Custom|LavaBeginOverlap))
    (Collision|BindEventtoOnComponentEndOverlap _array_element (EventDispatchers|CreateEvent :!event Custom|LavaEndOverlap))))

(event Custom|LavaBeginOverlap
  (params (OverlappedComponent :type Primitive%20Component%20Object%20Reference) (OtherActor :type Actor%20Object%20Reference) (OtherComp :type Primitive%20Component%20Object%20Reference) (OtherBodyIndex :type Integer) (bFromSweep :type Boolean) (SweepResult :type Hit%20Result%20Structure%20%28by%20ref%29))
  (bind _arrayempty_ (CallFunction|Add/RemoveArray (Variables|Default|GetOverlappedActors) OtherActor "NewEnumerator0" 0 "NewEnumerator0"))
  (bind _returnvalue (Audio|CreateSound2D "/Game/ShadowDuckStudio/SFX/LairSFX/LavaDeathLonger.LavaDeathLonger" 1.0 1.0 0.0 0))
  (Audio|Components|Audio|Play _returnvalue 0.0)
  (CallFunction|DamageTimerHandler _arrayempty_)
  (if (Actor|ActorHasTag OtherActor "Player")
    (bind _asbp_hmcharacter (Utilities|Casting|CastToBP_HMCharacter OtherActor))
    (Default|VFXonFire _asbp_hmcharacter)
    (elif (Actor|ActorHasTag OtherActor "Enemy")
      (bind _asbp_enemy_base (Utilities|Casting|CastToBP_Enemy_Base OtherActor))
      (Default|VFXonFire _asbp_enemy_base))))

(event Custom|LavaEndOverlap
  (params (OverlappedComponent :type Primitive%20Component%20Object%20Reference) (OtherActor :type Actor%20Object%20Reference) (OtherComp :type Primitive%20Component%20Object%20Reference) (OtherBodyIndex :type Integer))
  (bind _arrayempty_ (CallFunction|Add/RemoveArray (Variables|Default|GetOverlappedActors) OtherActor "NewEnumerator1" 0 "NewEnumerator0"))
  (CallFunction|DamageTimerHandler _arrayempty_))

(event EventBeginPlay)

(event EventTick
  (params (DeltaSeconds :type Float%20%28single-precision%29)))

(fn DamageTimerHandler
  (params (Start/Stop :type Boolean))
  (if Start/Stop
    (Utilities|Time|ClearTimerbyFunctionName 0 "DamageTick")
    (else
      (Utilities|Time|SetTimerbyFunctionName 0 "DamageTick" (Variables|Default|GetDamageTickTime) true))))

(fn DamageTick
  (for _array_element (Variables|Default|GetOverlappedActors)
    (Class|BIHealthInterface|Damage(Message) (Actor|GetComponentbyClass _array_element "/Game/ShadowDuckStudio/Blueprints/HealthSystem/AC_HealthComponent.AC_HealthComponent_C") (Variables|Default|GetDamage))))