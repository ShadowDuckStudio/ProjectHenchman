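; Base actor component that applies damage over time to the owning actor through its AC_HealthComponent, destroying itself if none exists.
; On BeginPlay it ends other components of its own class on the owner, so a new application replaces the old, then sends itself the begin message.
; BeginDOT starts a looping timer that deals DPS scaled by DamageFrequency each tick until Duration is reached, when EndDOT clears it and destroys the component.
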(event EventBeginPlay
  (bind _returnvalue (Components|GetOwner))
  (bind _self self)
  (bind _returnvalue_2 (Actor|GetComponentbyClass _returnvalue "/Game/ShadowDuckStudio/Blueprints/HealthSystem/AC_HealthComponent.AC_HealthComponent_C"))
  (Utilities|IsValid _returnvalue_2
    (:Is%20Valid
      (for _array_element (Actor|GetComponentsByClass _returnvalue (Utilities|GetClass self))
        (Utilities|IsValid _array_element
          (:Is%20Valid
            (if (not (== _array_element _self))
              (Class|BIDOTInterface|EndDOT(Message) _array_element)))))
      (Variables|Default|SetHealthComponent _returnvalue_2)
      (Class|BIDOTInterface|BeginDOT(Message) _self))
    (:Is%20Not%20Valid
      (Components|DestroyComponent))))

(event EventTick
  (params (DeltaSeconds :type Float%20%28single-precision%29)))

(event EventBeginDOT
  (Utilities|Time|SetTimerbyFunctionName 0 "DOT" (Variables|Default|GetDamage%20Frequency) true))

(event EventEndDOT
  (Utilities|Time|ClearTimerbyFunctionName 0 "DOT")
  (Components|DestroyComponent))

(fn DOT
  (if (< (Variables|Default|GetCurrentTime) (Variables|Default|GetDuration))
    (Variables|Default|SetCurrentTime (+ (Variables|Default|GetCurrentTime) (Variables|Default|GetDamage%20Frequency)))
    (Class|BIHealthInterface|Damage(Message) (Variables|Default|GetHealthComponent) (* (Variables|Default|GetDamage%20Frequency) (Variables|Default|GetDPS)))
    (else
      (CallFunction|EndDOT))))