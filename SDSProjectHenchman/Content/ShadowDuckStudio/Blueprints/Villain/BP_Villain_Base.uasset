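; Base Blueprint for the villain, handling scripted movement and the boss popup and game-over screens.
; Two custom events use AI MoveTo to send it to exposed, customisable locations behind the chair or at the front gate.
; Damage shows a boss popup for ten seconds, with a DoOnce that resets a minute after removal to limit repeats.
; Death adds the game-over widget to the viewport once.
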(event Custom|Villian%20moves%20behind%20chair
  ;[0.04417 1 0] 2 custom events moving the villian behind the chair and back in front of the gate (both locations can be customised and they are both exposed
  (AI|AIMoveTo self (Variables|Default|GetBehind%20Chair%20Loc) 0 5.0 false))

(event Custom|Villian%20moves%20to%20front%20gate
  ;[0.04417 1 0] 2 custom events moving the villian behind the chair and back in front of the gate (both locations can be customised and they are both exposed
  (AI|AIMoveTo self (Variables|Default|GetAt%20Front%20Gate%20Loc) 0 5.0 false))

(event EventBeginPlay)

(event Collision|EventActorBeginOverlap
  (params (OtherActor :type Actor%20Object%20Reference)))

(event EventTick
  (params (DeltaSeconds :type Float%20%28single-precision%29)))

(event EventDamage
  (params (Damage :type Float%20%28double-precision%29))
  (Utilities|FlowControl|DoOnce false :!label _label
    (:Completed
      (bind _returnvalue (UserInterface|CreateWidget "/Game/ShadowDuckStudio/UI/Widgets/BossPopup_WBP.BossPopup_WBP_C"))
      (UserInterface|Viewport|AddtoViewport _returnvalue 0)
      (Utilities|FlowControl|Delay 1e+01)
      (Widget|RemovefromParent _returnvalue)
      (Utilities|FlowControl|Delay 6e+01)
      (goto _label Reset))))

(event EventDeath
  (Utilities|FlowControl|DoOnce false
    (:Completed
      (bind _returnvalue (UserInterface|CreateWidget "/Game/ShadowDuckStudio/UI/Widgets/GameOver_WBP.GameOver_WBP_C"))
      (UserInterface|Viewport|AddtoViewport _returnvalue 1))))

(fn ConstructionScript)