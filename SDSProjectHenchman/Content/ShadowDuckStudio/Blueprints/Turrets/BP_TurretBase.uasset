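; BP_TurretBase is the base turret Blueprint, which loads build data and plays a build dust effect when spawned.
; BeginPlay, or the Ref event, loops over every DT_BuildInfo row and appends each found row to DefenceInfo.
; Each found row also activates FXSBuildDust and reaches a three-second Delay inside the loop, after which the effect is deactivated and destroyed.
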(event Custom|Ref
  (bind _fxs_builddust (Variables|Default|GetFXS_BuildDust))
  (bind _outrownames (DataTable|GetDataTableRowNames "/Game/ShadowDuckStudio/Blueprints/DataTables/DT_BuildInfo.DT_BuildInfo"))
  (for _array_element _outrownames
    (bind _returnvalue (Utilities|GetDataTableRow "/Game/ShadowDuckStudio/Blueprints/DataTables/DT_BuildInfo.DT_BuildInfo" _array_element)
      (:then
        (Utilities|Array|Add (Variables|Default|GetDefenceInfo) _returnvalue)
        (Components|Activation|Activate _fxs_builddust false)
        (Utilities|FlowControl|Delay 3.0)
        (Components|Activation|Deactivate _fxs_builddust)
        (Components|DestroyComponent _fxs_builddust)))))

(event EventBeginPlay
  (bind _fxs_builddust (Variables|Default|GetFXS_BuildDust))
  (bind _outrownames (DataTable|GetDataTableRowNames "/Game/ShadowDuckStudio/Blueprints/DataTables/DT_BuildInfo.DT_BuildInfo"))
  (for _array_element _outrownames
    (bind _returnvalue (Utilities|GetDataTableRow "/Game/ShadowDuckStudio/Blueprints/DataTables/DT_BuildInfo.DT_BuildInfo" _array_element)
      (:then
        (Utilities|Array|Add (Variables|Default|GetDefenceInfo) _returnvalue)
        (Components|Activation|Activate _fxs_builddust false)
        (Utilities|FlowControl|Delay 3.0)
        (Components|Activation|Deactivate _fxs_builddust)
        (Components|DestroyComponent _fxs_builddust)))))

(event Collision|EventActorBeginOverlap
  (params (OtherActor :type Actor%20Object%20Reference)))

(event EventTick
  (params (DeltaSeconds :type Float%20%28single-precision%29)))

(fn ConstructionScript)