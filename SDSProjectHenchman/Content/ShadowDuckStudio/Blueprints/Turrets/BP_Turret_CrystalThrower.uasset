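; Crystal thrower turret that automatically fires at the nearest target of allowed classes within its range and is reloaded through interaction.
; Range overlaps maintain the target list and run a looping aim timer while it is non-empty.
; Each aim tick picks the closest target, rotates toward it and begins charging ACProjectileShooter when a line trace hits it.
; Interacting runs a reload timer that refills the shooter on completion; ending interaction cancels it.
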(event OnComponentBeginOverlap(Range)
  (params (OverlappedComponent :type Primitive%20Component%20Object%20Reference) (OtherActor :type Actor%20Object%20Reference) (OtherComp :type Primitive%20Component%20Object%20Reference) (OtherBodyIndex :type Integer) (bFromSweep :type Boolean) (SweepResult :type Hit%20Result%20Structure%20%28by%20ref%29))
  (if (Utilities|Array|ContainsItem (Variables|Target|GetTargetClassesArray) (Utilities|GetClass OtherActor))
    (Utilities|Array|AddUnique (Variables|Target|GetTargetArray) OtherActor)
    (CallFunction|TargetCheck)))

(event OnComponentEndOverlap(Range)
  (params (OverlappedComponent :type Primitive%20Component%20Object%20Reference) (OtherActor :type Actor%20Object%20Reference) (OtherComp :type Primitive%20Component%20Object%20Reference) (OtherBodyIndex :type Integer))
  (if (Utilities|Array|ContainsItem (Variables|Target|GetTargetClassesArray) (Utilities|GetClass OtherActor))
    (Utilities|Array|RemoveItem (Variables|Target|GetTargetArray) OtherActor)
    (CallFunction|TargetCheck)))

(event EventBeginPlay
  (Variables|/Game/ShadowDuckStudio/Blueprints/Turrets/AC_ProjectileShooter.AC_ProjectileShooter_C|SetFiringPoint (Variables|Default|GetAC_ProjectileShooter) (Variables|Default|GetArrow))
  (Variables|Default|SetRotationPoint (Variables|Default|GetScene)))

(event EventBeginInteract
  (params (Source :type Actor%20Object%20Reference))
  (Variables|Reload|SetCurrentReloadTime 0.0)
  (Utilities|Time|SetTimerbyFunctionName 0 "ReloadTick" (Variables|Reload|GetReloadTickTime) true))

(event EventEndInteract
  (params (Source :type Actor%20Object%20Reference))
  (Utilities|Time|ClearTimerbyFunctionName 0 "ReloadTick"))

(fn ConstructionScript)

(fn AimTick
  (bind _target (Variables|Target|GetTarget))
  (bind _rotationpoint (Variables|Default|GetRotationPoint))
  (bind _returnvalue (Transformation|GetWorldLocation _rotationpoint))
  (bind _returnvalue_2 (Transformation|GetActorLocation _target))
  (bind _returnvalue_3 (Math|Rotator|FindLookatRotation _returnvalue _returnvalue_2))
  (CallFunction|SetClosestTarget)
  (Transformation|SetWorldRotation _rotationpoint _returnvalue_3 false false)
  (bind _outhit (Collision|LineTraceByChannel (Transformation|GetWorldLocation (Variables|Default|GetArrow)) (+ _returnvalue_2 (* (Math|Vector|GetForwardVector _returnvalue_3) 1e+02)) "TraceTypeQuery2" false 0 "ForOneFrame"))
  (if (== (.HitActor (Collision|BreakHitResult _outhit)) _target)
    (Default|BeginCharge (Variables|Default|GetAC_ProjectileShooter))))

(fn TargetCheck
  (if (Utilities|Array|IsNotEmpty (Variables|Target|GetTargetArray))
    (CallFunction|ChooseTarget)
    (if (not (Class|KismetSystemLibrary|TimerExists 0 "AimTick"))
      (Utilities|Time|SetTimerbyFunctionName 0 "AimTick" (Variables|Default|GetAimTickTime) true))
    (else
      (Utilities|Time|ClearTimerbyFunctionName 0 "AimTick"))))

(fn ChooseTarget
  (Variables|Target|SetTarget (Utilities|Array|Get(acopy) (Variables|Target|GetTargetArray))))

(fn ReloadTick
  (if (< (Variables|Reload|GetCurrentReloadTime) (Variables|Reload|GetMaxReloadTime))
    (Variables|Reload|SetCurrentReloadTime (+ (Variables|Reload|GetCurrentReloadTime) (Variables|Reload|GetReloadTickTime)))
    (else
      (Default|Reload (Variables|Default|GetAC_ProjectileShooter) (Variables|Reload|GetReloadAmount))
      (Utilities|Time|ClearTimerbyFunctionName 0 "ReloadTick"))))

(fn SetClosestTarget
  (bind _returnvalue (Transformation|GetActorLocation))
  (bind _targetarray (Variables|Target|GetTargetArray))
  (bind _returnvalue_2 (Actor|FindNearestActor _returnvalue _targetarray))
  (bind _target (Variables|Target|GetTarget)
    (:then
      (if (not (== _target _returnvalue_2))
        (Utilities|IsValid _returnvalue_2 :!label _label
          (:Is%20Valid
            (Variables|Target|SetTarget _returnvalue_2))
          (:Is%20Not%20Valid
            (Variables|Target|SetTarget 0)))
        (return)))
    (:else
      (goto _label))))

(fn GetOverlayMeshes
  (return 0))