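; Spinning hammer turret that runs during waves, launching, stunning and damaging characters it hits, and knocking away physics objects.
; Stats come from a DefenceInfo row, though StartSpin hardcodes rotation speed.
; Its health component acts as durability, draining on a timer and per hit until spinning stops.
; Hold-to-repair spends player resources, at half cost above half health, then restarts the spin; proximity spheres drive repair and durability widgets.
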(event OnComponentBeginOverlap(LeftCollision)
  (params (OverlappedComponent :type Primitive%20Component%20Object%20Reference) (OtherActor :type Actor%20Object%20Reference) (OtherComp :type Primitive%20Component%20Object%20Reference) (OtherBodyIndex :type Integer) (bFromSweep :type Boolean) (SweepResult :type Hit%20Result%20Structure%20%28by%20ref%29))
  (bind _returnvalue (Actor|GetComponentbyClass OtherActor "/Game/ShadowDuckStudio/Blueprints/HealthSystem/AC_HealthComponent.AC_HealthComponent_C"))
  (bind _leftforcepoint (Variables|Default|GetLeftForcePoint))
  (bind _charhorizontalimpulse (Variables|Default|GetCharHorizontalImpulse))
  (bind _objhorizontalimpulse (Variables|Default|GetObjHorizontalImpulse))
  (bind _returnvalue_2 (Math|Vector|GetForwardVector _leftforcepoint))
  (bind _returnvalue_3 (* _returnvalue_2 _charhorizontalimpulse))
  (bind _returnvalue_4 (* _returnvalue_2 _objhorizontalimpulse))
  (bind (_x _y) (Math|Vector|BreakVector _returnvalue_4))
  (bind (_x_2 _y_2) (Math|Vector|BreakVector _returnvalue_3))
  (if (Variables|Default|GetSpinning?)
    (if (not (Utilities|Array|ContainsItem (Variables|Default|GetIgnoredClasses) (Utilities|GetClass OtherActor)))
      (bind _ascharacter (Utilities|Casting|CastToCharacter OtherActor)
        (:then
          (AI|Logic|StopLogic (Variables|/Script/AIModule.AIController|GetBrainComponent (AI|GetAIController _ascharacter)) "")
          (Character|Jump _ascharacter)
          (Character|LaunchCharacter _ascharacter (Math|Vector|MakeVector _x_2 _y_2 (Variables|Default|GetCharVerticalImpulse)) false false)
          (Character|StopJumping _ascharacter)
          (AI|Logic|StartLogic (Variables|/Script/AIModule.AIController|GetBrainComponent (AI|GetAIController _ascharacter)))
          (bind _asbp_enemy_base (Utilities|Casting|CastToBP_Enemy_Base _ascharacter)
            (:then
              (Default|Stun _asbp_enemy_base (Variables|Default|GetStun%20Duration)))
            (:CastFailed
              _)))
        (:CastFailed
          (if (Class|SceneComponent|IsAnySimulatingPhysics OtherComp)
            (Physics|AddImpulseatLocation OtherComp (Math|Vector|MakeVector _x _y (Variables|Default|GetObjVerticalImpulse)) (Transformation|GetWorldLocation _leftforcepoint) "None"))))
      (Utilities|IsValid _returnvalue
        (:Is%20Valid
          (Class|BIHealthInterface|Damage(Message) _returnvalue (Variables|Default|GetDamageTaken))
          (Class|BIHealthInterface|Damage(Message) (Variables|Default|GetAC_HealthComponent) (Variables|Default|GetDurabilityOnHit))
          (if (not (CallFunction|HealthCheck))
            (CallFunction|StopSpin)))))))

(event OnComponentBeginOverlap(CollisionforDur)
  (params (OverlappedComponent :type Primitive%20Component%20Object%20Reference) (OtherActor :type Actor%20Object%20Reference) (OtherComp :type Primitive%20Component%20Object%20Reference) (OtherBodyIndex :type Integer) (bFromSweep :type Boolean) (SweepResult :type Hit%20Result%20Structure%20%28by%20ref%29))
  (if (Actor|ActorHasTag OtherActor "Player")
    (Variables|Default|SetInSmallerRadius true)
    (Rendering|SetVisibility (Variables|Default|GetDurCounterIcon) true false)
    (CallFunction|CheckSmallerRadius)))

(event OnComponentEndOverlap(Sphere)
  (params (OverlappedComponent :type Primitive%20Component%20Object%20Reference) (OtherActor :type Actor%20Object%20Reference) (OtherComp :type Primitive%20Component%20Object%20Reference) (OtherBodyIndex :type Integer))
  (if (Actor|ActorHasTag OtherActor "Player")
    (Variables|Default|SetInVisibleRadius false)
    (CallFunction|CheckRepairVisible)))

(event OnComponentEndOverlap(CollisionforDur)
  (params (OverlappedComponent :type Primitive%20Component%20Object%20Reference) (OtherActor :type Actor%20Object%20Reference) (OtherComp :type Primitive%20Component%20Object%20Reference) (OtherBodyIndex :type Integer))
  (if (Actor|ActorHasTag OtherActor "Player")
    (Variables|Default|SetInSmallerRadius false)
    (Rendering|SetVisibility (Variables|Default|GetDurCounterIcon) false false)
    (CallFunction|CheckSmallerRadius)))

(event OnComponentBeginOverlap(Sphere)
  (params (OverlappedComponent :type Primitive%20Component%20Object%20Reference) (OtherActor :type Actor%20Object%20Reference) (OtherComp :type Primitive%20Component%20Object%20Reference) (OtherBodyIndex :type Integer) (bFromSweep :type Boolean) (SweepResult :type Hit%20Result%20Structure%20%28by%20ref%29))
  (if (Actor|ActorHasTag OtherActor "Player")
    (Variables|Default|SetInVisibleRadius true)
    (CallFunction|CheckRepairVisible)))

(event Custom|StartSpin
  (Utilities|Time|SetTimerbyFunctionName 0 "SpinTick" (Variables|Default|GetDurabilityTickTime) true)
  (Variables|/Script/Engine.RotatingMovementComponent|SetRotationRate (Variables|Default|GetRotatingMovement) "0.000000,1200.000000,0.000000")
  (Variables|Default|SetSpinning? true))

(event Custom|StopSpin
  (Utilities|Time|ClearTimerbyFunctionName 0 "SpinTick")
  (Variables|/Script/Engine.RotatingMovementComponent|SetRotationRate (Variables|Default|GetRotatingMovement) "0, 0, 0")
  (Variables|Default|SetSpinning? false))

(event Custom|CheckRepairVisible
  (bind _needsrepairiconwidget (Variables|Default|GetNeedsRepairIconWidget))
  (bind _repairiconminimap (Variables|Default|GetRepairIconMinimap))
  (bind _ac_healthcomponent (Variables|Default|GetAC_HealthComponent))
  (bind _currenthealth (Variables|/Game/ShadowDuckStudio/Blueprints/HealthSystem/AC_HealthComponent.AC_HealthComponent_C|GetCurrentHealth _ac_healthcomponent))
  (bind _returnvalue (<= _currenthealth 0.0))
  (if _returnvalue
    (Rendering|SetVisibility _repairiconminimap true false)
    (else
      (Rendering|SetVisibility _repairiconminimap false false)))
  (if (and (Variables|Default|GetInVisibleRadius) _returnvalue)
    (Rendering|SetVisibility _needsrepairiconwidget true false)
    (else
      (Rendering|SetVisibility _needsrepairiconwidget false false))))

(event Custom|CanRepair
  (bind _ac_healthcomponent (Variables|Default|GetAC_HealthComponent))
  (bind _repairprogress (Variables|Default|GetRepairProgress))
  (bind _currenthealth (Variables|/Game/ShadowDuckStudio/Blueprints/HealthSystem/AC_HealthComponent.AC_HealthComponent_C|GetCurrentHealth _ac_healthcomponent))
  (if (== (Math|Vector|VectorLength (Transformation|GetVelocity (Game|Player|GetPlayerPawn 0))) 0.0)
    (if (and (< _currenthealth (Variables|/Game/ShadowDuckStudio/Blueprints/HealthSystem/AC_HealthComponent.AC_HealthComponent_C|GetMaxHealth _ac_healthcomponent)) (>= (.resource1 (Variables|/Game/ShadowDuckStudio/Blueprints/ResourcesSystem/AC_ResourceComponent.AC_ResourceComponent_C|GetResources (Variables|/Game/ShadowDuckStudio/Blueprints/Player/BP_HMCharacter.BP_HMCharacter_C|GetAC_ResourceComponent (.AsBP%20HMCharacter (Utilities|Casting|CastToBP_HMCharacter (Game|Player|GetPlayerPawn 0)))))) (Variables|Default|GetResources%20Taken%20)))
      (Rendering|SetVisibility _repairprogress true false)
      (if (== _currenthealth 3e+02)
        (Utilities|FlowControl|Delay 1.2)
        (Rendering|SetVisibility _repairprogress false false)))
    (else
      (Utilities|Time|ClearTimerbyFunctionName 0 "ReloadTick")
      (Rendering|SetVisibility _repairprogress false false))))

(event Custom|CheckSmallerRadius
  (bind _holdtorepairtextwidget (Variables|Default|GetHoldtoRepairTextWidget))
  (if (and (<= (Variables|/Game/ShadowDuckStudio/Blueprints/HealthSystem/AC_HealthComponent.AC_HealthComponent_C|GetCurrentHealth (Variables|Default|GetAC_HealthComponent)) 0.0) (Variables|Default|GetInSmallerRadius))
    (Rendering|SetVisibility _holdtorepairtextwidget true false)
    (else
      (Rendering|SetVisibility _holdtorepairtextwidget false false))))

(event Custom|End%20Progress
  (Rendering|SetVisibility (Variables|Default|GetRepairProgress) false false))

(event Custom|BeginDeconstruct_1
  (params (Source :type Actor%20Object%20Reference))
  (CallFunction|BeginDeconstructTimer self Source (Variables|Default|GetRefund)))

(event EventBeginPlay
  (bind _self self)
  (bind _defenceinfo (Variables|Default|GetDefenceInfo))
  (bind _output (Utilities|Array|Get(acopy) _defenceinfo 2))
  (bind (_slot _built _cost _angleconstraints _buildiconinfo _tag _def_dmg _def_attackspeed _def_repairamount _def_health _def_dmgpertickself _def_spawnspeed _def_pushstrength _def_dmgperhitself) (Utilities|Struct|BreakF_BuildInfo _output))
  (|CallParentFunction)
  (Variables|/Game/ShadowDuckStudio/UI/Widgets/TrapsandTurrets/AmmoCounterHammer_WBP.AmmoCounterHammer_WBP_C|SetHammerRef (.AsAmmo%20Counter%20Hammer%20WBP (Utilities|Casting|CastToAmmoCounterHammer_WBP (UserInterface|GetWidget (Variables|Default|GetDurCounterIcon)))) _self)
  (Variables|/Game/ShadowDuckStudio/UI/Widgets/TrapsandTurrets/RepairProgressSymbolHammer_WBP.RepairProgressSymbolHammer_WBP_C|SetHammerReference (.AsRepair%20Progress%20Symbol%20Hammer%20WBP (Utilities|Casting|CastToRepairProgressSymbolHammer_WBP (UserInterface|GetWidget (Variables|Default|GetRepairProgress)))) _self)
  (bind _returnvalue (Actor|GetActorOfClass "/Game/ShadowDuckStudio/Blueprints/Player/BP_HMCharacter.BP_HMCharacter_C"))
  (Variables|Default|SetPlayerRef _returnvalue)
  (Variables|Default|SetDamageTaken _def_dmg)
  (Variables|/Script/Engine.RotatingMovementComponent|SetRotationRate (Variables|Default|GetRotatingMovement) (Math|Rotator|MakeRotator 0.0 0.0 _def_attackspeed))
  (Variables|Default|SetReloadAmount _def_repairamount)
  (Variables|/Game/ShadowDuckStudio/Blueprints/HealthSystem/AC_HealthComponent.AC_HealthComponent_C|SetMaxHealth (Variables|Default|GetAC_HealthComponent) _def_health)
  (Variables|Default|SetDurabilityPerTick _def_dmgpertickself)
  (Variables|Default|SetImpulseStrength _def_pushstrength)
  (Variables|Default|SetDurabilityOnHit _def_dmgperhitself)
  (Class|NiagaraFunctionLibrary|OverrideSystemUserVariableSkeletalMeshComponent (Variables|Default|GetFX_BeamTrail) "" (Variables|Default|GetSkeletalMesh))
  (bind _returnvalue_2 (Actor|GetActorOfClass "/Game/ShadowDuckStudio/Blueprints/WaveSystem/WaveSystem.WaveSystem_C"))
  (bind _output_get (Variables|Default|SetWaveManager _returnvalue_2))
  (if (Variables|/Game/ShadowDuckStudio/Blueprints/WaveSystem/WaveSystem.WaveSystem_C|GetWaveInProgress? _output_get)
    (CallFunction|StartSpin)
    (else
      (CallFunction|StopSpin))))

(event Collision|EventActorBeginOverlap
  (params (OtherActor :type Actor%20Object%20Reference))
  (|CallParentFunction OtherActor) ; This node is disabled and will not be called.\nDrag off pins to build functionality.
)

(event EventStartWave
  (params (WaveNo :type Integer))
  (CallFunction|StartSpin))

(event EventEndWave
  (CallFunction|StopSpin))

(event EventTick
  (params (DeltaSeconds :type Float%20%28single-precision%29))
  (|CallParentFunction DeltaSeconds) ; This node is disabled and will not be called.\nDrag off pins to build functionality.
)

(event EventHeal
  (params (Amount :type Float%20%28double-precision%29))
  (CallFunction|CheckRepairVisible)
  (CallFunction|CheckSmallerRadius))

(event EventDeath
  (CallFunction|CheckRepairVisible)
  (CallFunction|CheckSmallerRadius))

(event EventDamage
  (params (Damage :type Float%20%28double-precision%29))
  (CallFunction|CheckRepairVisible)
  (CallFunction|CheckSmallerRadius))

(event EventBeginInteract
  (params (Source :type Actor%20Object%20Reference))
  (Variables|Default|SetCurrentReloadTime 0.0)
  (Utilities|Time|SetTimerbyFunctionName 0 "ReloadTick" (Variables|Default|GetReloadTickTime) true))

(event EventEndInteract
  (params (Source :type Actor%20Object%20Reference))
  (Utilities|Time|ClearTimerbyFunctionName 0 "ReloadTick")
  (CallFunction|EndProgress))

(fn ConstructionScript
  (|CallParentFunction))

(fn ReloadTick
  (bind _returnvalue (Game|Player|GetPlayerPawn 0))
  (bind _resources_taken_ (Variables|Default|GetResources%20Taken%20))
  (bind _ac_healthcomponent (Variables|Default|GetAC_HealthComponent))
  (bind _asbp_hmcharacter (Utilities|Casting|CastToBP_HMCharacter _returnvalue))
  (bind _ac_resourcecomponent (Variables|/Game/ShadowDuckStudio/Blueprints/Player/BP_HMCharacter.BP_HMCharacter_C|GetAC_ResourceComponent _asbp_hmcharacter))
  (CallFunction|CanRepair)
  (if (< (Variables|Default|GetCurrentReloadTime) (Variables|Default|GetMaxReloadTime))
    (Variables|Default|SetCurrentReloadTime (+ (Variables|Default|GetCurrentReloadTime) (Variables|Default|GetReloadTickTime)))
    (else
      (Variables|Default|GetPlayerRef
        (:then
          _)
        (:else
          (bind _returnvalue_2 (Actor|GetActorOfClass "/Game/ShadowDuckStudio/Blueprints/Player/BP_HMCharacter.BP_HMCharacter_C"))
          (Variables|Default|SetPlayerRef _returnvalue_2)))
      (if (< (.resource1 (Variables|/Game/ShadowDuckStudio/Blueprints/ResourcesSystem/AC_ResourceComponent.AC_ResourceComponent_C|GetResources _ac_resourcecomponent)) _resources_taken_)
        (Development|PrintString "Returning true")
        (else
          (if (> (Variables|/Game/ShadowDuckStudio/Blueprints/HealthSystem/AC_HealthComponent.AC_HealthComponent_C|GetCurrentHealth _ac_healthcomponent) (/ (Variables|/Game/ShadowDuckStudio/Blueprints/HealthSystem/AC_HealthComponent.AC_HealthComponent_C|GetMaxHealth _ac_healthcomponent) 2.0))
            (Default|TakeResource _ac_resourcecomponent (Utilities|Struct|MakeF_Resources (/ (Variables|Default|GetResources%20Taken%20) 2)))
            (else
              (Default|TakeResource _ac_resourcecomponent (Utilities|Struct|MakeF_Resources _resources_taken_))))
          (Class|BIHealthInterface|Heal(Message) (Variables|Default|GetAC_HealthComponent) (Variables|Default|GetReloadAmount))
          (Utilities|Time|ClearTimerbyFunctionName 0 "ReloadTick")
          (if true
            (CallFunction|StartSpin)
            (CallFunction|CheckRepairVisible)
            (CallFunction|CheckSmallerRadius)))))))

(fn SpinTick
  (Class|BIHealthInterface|Damage(Message) (Variables|Default|GetAC_HealthComponent) (Variables|Default|GetDurabilityPerTick))
  (if (CallFunction|HealthCheck)
    (CallFunction|CheckRepairVisible)
    (else
      (CallFunction|StopSpin)
      (CallFunction|CheckRepairVisible))))

(fn HealthCheck
  (return (> (Variables|/Game/ShadowDuckStudio/Blueprints/HealthSystem/AC_HealthComponent.AC_HealthComponent_C|GetCurrentHealth (Variables|Default|GetAC_HealthComponent)) 0.0)))

(fn GetOverlayMeshes
  (return 0))