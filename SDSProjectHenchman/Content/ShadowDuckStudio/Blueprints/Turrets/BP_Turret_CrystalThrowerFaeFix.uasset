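; Crystal-throwing fae turret that fires at targets in range, with health doubling as its ammo display and stats read from DefenceInfo.
; Range overlaps start a looping AimTick that faces the nearest target, line-traces to it and charges ACProjectileShooter while health remains.
; Player interaction runs a timed repair costing resources, halved above half health.
; Proximity spheres toggle ammo and refill widgets; deconstruction passes a refund.
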(event OnComponentBeginOverlap(Range)
  (params (OverlappedComponent :type Primitive%20Component%20Object%20Reference) (OtherActor :type Actor%20Object%20Reference) (OtherComp :type Primitive%20Component%20Object%20Reference) (OtherBodyIndex :type Integer) (bFromSweep :type Boolean) (SweepResult :type Hit%20Result%20Structure%20%28by%20ref%29))
  (CallFunction|Add/RemoveArray (Variables|Target|GetTargetArray) OtherActor "NewEnumerator0" (Variables|Target|GetTargetClassesArray) "NewEnumerator1")
  (CallFunction|TargetCheck)
  (CallFunction|CheckRepairVisible))

(event OnComponentEndOverlap(Range)
  (params (OverlappedComponent :type Primitive%20Component%20Object%20Reference) (OtherActor :type Actor%20Object%20Reference) (OtherComp :type Primitive%20Component%20Object%20Reference) (OtherBodyIndex :type Integer))
  (CallFunction|Add/RemoveArray (Variables|Target|GetTargetArray) OtherActor "NewEnumerator1" (Variables|Target|GetTargetClassesArray) "NewEnumerator1")
  (CallFunction|TargetCheck)
  (CallFunction|CheckRepairVisible))

(event OnComponentEndOverlap(Sphere)
  (params (OverlappedComponent :type Primitive%20Component%20Object%20Reference) (OtherActor :type Actor%20Object%20Reference) (OtherComp :type Primitive%20Component%20Object%20Reference) (OtherBodyIndex :type Integer))
  (if (Actor|ActorHasTag OtherActor "Player")
    (Variables|Default|SetInVisibleRadius false)
    (CallFunction|CheckRepairVisible)))

(event OnComponentEndOverlap(CollisionforAmmo)
  (params (OverlappedComponent :type Primitive%20Component%20Object%20Reference) (OtherActor :type Actor%20Object%20Reference) (OtherComp :type Primitive%20Component%20Object%20Reference) (OtherBodyIndex :type Integer))
  (if (Actor|ActorHasTag OtherActor "Player")
    (Variables|Default|SetInSmallerRadius false)
    (Rendering|SetVisibility (Variables|Default|GetAmmoCounterIcon) false false)
    (CallFunction|CheckSmallerRadius)))

(event OnComponentBeginOverlap(CollisionforAmmo)
  (params (OverlappedComponent :type Primitive%20Component%20Object%20Reference) (OtherActor :type Actor%20Object%20Reference) (OtherComp :type Primitive%20Component%20Object%20Reference) (OtherBodyIndex :type Integer) (bFromSweep :type Boolean) (SweepResult :type Hit%20Result%20Structure%20%28by%20ref%29))
  (if (Actor|ActorHasTag OtherActor "Player")
    (Variables|Default|SetInSmallerRadius true)
    (Rendering|SetVisibility (Variables|Default|GetAmmoCounterIcon) true false)
    (CallFunction|CheckSmallerRadius)))

(event OnComponentBeginOverlap(Sphere)
  (params (OverlappedComponent :type Primitive%20Component%20Object%20Reference) (OtherActor :type Actor%20Object%20Reference) (OtherComp :type Primitive%20Component%20Object%20Reference) (OtherBodyIndex :type Integer) (bFromSweep :type Boolean) (SweepResult :type Hit%20Result%20Structure%20%28by%20ref%29))
  (if (Actor|ActorHasTag OtherActor "Player")
    (Variables|Default|SetInVisibleRadius true)
    (CallFunction|CheckRepairVisible)))

(event Custom|Throw%20Animation)

(event Custom|Reset%20FIre
  (Utilities|FlowControl|Delay 1.0)
  (Variables|/Game/ShadowDuckStudio/Blueprints/Turrets/AC_ProjectileShooter.AC_ProjectileShooter_C|SetCanFire? (Variables|Default|GetAC_ProjectileShooter) false)
  (CallFunction|CheckSmallerRadius))

(event Custom|CheckRepairVisible
  (bind _ammoiconwidget (Variables|Default|GetAmmoIconWidget))
  (bind _ac_healthcomponent (Variables|Default|GetAC_HealthComponent))
  (bind _repairiconminimap (Variables|Default|GetRepairIconMinimap))
  (bind _currenthealth (Variables|/Game/ShadowDuckStudio/Blueprints/HealthSystem/AC_HealthComponent.AC_HealthComponent_C|GetCurrentHealth _ac_healthcomponent))
  (bind _returnvalue (<= _currenthealth 0.0))
  (if _returnvalue
    (Rendering|SetVisibility _repairiconminimap true false)
    (else
      (Rendering|SetVisibility _repairiconminimap false false)))
  (if (and (Variables|Default|GetInVisibleRadius) _returnvalue)
    (Rendering|SetVisibility _ammoiconwidget true false)
    (else
      (Rendering|SetVisibility _ammoiconwidget false false))))

(event Custom|CanRepair
  (bind _ac_healthcomponent (Variables|Default|GetAC_HealthComponent))
  (bind _repairprogress (Variables|Default|GetRepairProgress))
  (bind _currenthealth (Variables|/Game/ShadowDuckStudio/Blueprints/HealthSystem/AC_HealthComponent.AC_HealthComponent_C|GetCurrentHealth _ac_healthcomponent))
  (if (== (Math|Vector|VectorLength (Transformation|GetVelocity (Game|Player|GetPlayerPawn 0))) 0.0)
    (if (and (< _currenthealth (Variables|/Game/ShadowDuckStudio/Blueprints/HealthSystem/AC_HealthComponent.AC_HealthComponent_C|GetMaxHealth _ac_healthcomponent)) (>= (.resource1 (Variables|/Game/ShadowDuckStudio/Blueprints/ResourcesSystem/AC_ResourceComponent.AC_ResourceComponent_C|GetResources (Variables|/Game/ShadowDuckStudio/Blueprints/Player/BP_HMCharacter.BP_HMCharacter_C|GetAC_ResourceComponent (Variables|Default|GetPlayerRef)))) (Variables|Default|GetResources%20Taken)))
      (Rendering|SetVisibility _repairprogress true false)
      (if (== _currenthealth 3e+02)
        (Utilities|FlowControl|Delay 1.2)
        (Rendering|SetVisibility _repairprogress false false)))
    (else
      (Utilities|Time|ClearTimerbyFunctionName 0 "ReloadTick")
      (Rendering|SetVisibility _repairprogress false false))))

(event Custom|CheckSmallerRadius
  (bind _refillammowidget (Variables|Default|GetRefillAmmoWidget))
  (if (and (<= (Variables|/Game/ShadowDuckStudio/Blueprints/HealthSystem/AC_HealthComponent.AC_HealthComponent_C|GetCurrentHealth (Variables|Default|GetAC_HealthComponent)) 0.0) (Variables|Default|GetInSmallerRadius))
    (Rendering|SetVisibility _refillammowidget true false)
    (else
      (Rendering|SetVisibility _refillammowidget false false))))

(event Custom|Can%20Fire
  (Variables|/Game/ShadowDuckStudio/Blueprints/Turrets/AC_ProjectileShooter.AC_ProjectileShooter_C|SetCanFire? (Variables|Default|GetAC_ProjectileShooter) true)
  (CallFunction|CheckSmallerRadius))

(event Custom|End%20Progress
  (Rendering|SetVisibility (Variables|Default|GetRepairProgress) false false))

(event Custom|BeginDeconstruct_1
  (params (Source :type Actor%20Object%20Reference))
  (CallFunction|BeginDeconstructTimer self Source (Variables|Default|GetRefund)))

(event EventBeginPlay
  (bind _self self)
  (bind _defenceinfo (Variables|Default|GetDefenceInfo))
  (bind _output (Utilities|Array|Get(acopy) _defenceinfo 1))
  (bind (_slot _built _cost _angleconstraints _buildiconinfo _tag _def_dmg _def_attackspeed _def_repairamount _def_health _def_dmgpertickself) (Utilities|Struct|BreakF_BuildInfo _output))
  (Utilities|FlowControl|Sequence
    (:then_0
      (Variables|/Game/ShadowDuckStudio/UI/Widgets/TrapsandTurrets/AmmoCounterTurret_WBP.AmmoCounterTurret_WBP_C|SetTurretRef (.AsAmmo%20Counter%20Turret%20WBP (Utilities|Casting|CastToAmmoCounterTurret_WBP (UserInterface|GetWidget (Variables|Default|GetAmmoCounterIcon)))) _self)
      (Variables|/Game/ShadowDuckStudio/UI/Widgets/TrapsandTurrets/RepairProgressSymbolTurret_WBP.RepairProgressSymbolTurret_WBP_C|SetCrystalRef (.AsRepair%20Progress%20Symbol%20Turret%20WBP (Utilities|Casting|CastToRepairProgressSymbolTurret_WBP (UserInterface|GetWidget (Variables|Default|GetRepairProgress)))) _self)
      (bind _returnvalue (Actor|GetActorOfClass "/Game/ShadowDuckStudio/Blueprints/Enemies/BP_Enemy_Base.BP_Enemy_Base_C"))
      (Variables|Default|SetEnemyRef _returnvalue)
      (if (Utilities|Array|IsEmpty _defenceinfo)
        (CallFunction|Ref))
      (bind _returnvalue_2 (Actor|GetActorOfClass "/Game/ShadowDuckStudio/Blueprints/Player/BP_HMCharacter.BP_HMCharacter_C"))
      (Variables|Default|SetPlayerRef _returnvalue_2)
      (Variables|/Game/ShadowDuckStudio/Blueprints/Turrets/AC_ProjectileShooter.AC_ProjectileShooter_C|SetFiringPoint (Variables|Default|GetAC_ProjectileShooter) (Variables|Default|GetArrow))
      (Variables|Default|SetRotationPoint (Variables|Default|GetScene))
      (Actor|GetActorOfClass "/Game/ShadowDuckStudio/Blueprints/Turrets/Projectiles/BP_ProjectileBase.BP_ProjectileBase_C")
      (Variables|Default|SetAimTickTime _def_attackspeed)
      (Variables|Reload|SetReloadAmount _def_repairamount)
      (Variables|/Game/ShadowDuckStudio/Blueprints/HealthSystem/AC_HealthComponent.AC_HealthComponent_C|SetMaxHealth (Variables|Default|GetAC_HealthComponent) _def_health)
      (Variables|Default|SetAmmoUsePerShot _def_dmgpertickself))
    (:then_1
      (Utilities|FlowControl|Delay 1.0)
      (Audio|PlaySound2D (Variables|Default|GetLaughSFX) 1.0 1.0 0.0 0 0))))

(event EventHeal
  (params (Amount :type Float%20%28double-precision%29))
  (CallFunction|CheckRepairVisible)
  (CallFunction|CheckSmallerRadius))

(event EventBeginInteract
  (params (Source :type Actor%20Object%20Reference))
  (Variables|Reload|SetCurrentReloadTime 0.0)
  (Utilities|Time|SetTimerbyFunctionName 0 "ReloadTick" (Variables|Reload|GetReloadTickTime) true))

(event EventEndInteract
  (params (Source :type Actor%20Object%20Reference))
  (Utilities|Time|ClearTimerbyFunctionName 0 "ReloadTick")
  (CallFunction|EndProgress))

(event EventDeath
  (CallFunction|CheckRepairVisible)
  (CallFunction|CheckSmallerRadius))

(event EventDamage
  (params (Damage :type Float%20%28double-precision%29))
  (CallFunction|CheckRepairVisible)
  (CallFunction|CheckSmallerRadius))

(fn ConstructionScript)

(fn AimTick
  (bind _target (Variables|Target|GetTarget))
  (bind _rotationpoint (Variables|Default|GetRotationPoint))
  (bind _returnvalue (Transformation|GetWorldLocation _rotationpoint))
  (bind _returnvalue_2 (Transformation|GetActorLocation _target))
  (bind _returnvalue_3 (Math|Rotator|FindLookatRotation _returnvalue _returnvalue_2))
  (if (> (Variables|/Game/ShadowDuckStudio/Blueprints/HealthSystem/AC_HealthComponent.AC_HealthComponent_C|GetCurrentHealth (Variables|Default|GetAC_HealthComponent)) 0.0)
    (CallFunction|SetClosestTarget)
    (Transformation|SetWorldRotation _rotationpoint _returnvalue_3 false false)
    (bind _outhit (Collision|LineTraceByChannel (Transformation|GetWorldLocation (Variables|Default|GetArrow)) (+ _returnvalue_2 (* (Math|Vector|GetForwardVector _returnvalue_3) 1e+02)) "TraceTypeQuery2" false 0 "None"))
    (if (== (.HitActor (Collision|BreakHitResult _outhit)) _target)
      (Default|BeginCharge (Variables|Default|GetAC_ProjectileShooter))
      (CallFunction|ThrowAnimation))))

(fn TargetCheck
  (if (Utilities|Array|IsNotEmpty (Variables|Target|GetTargetArray))
    (CallFunction|ChooseTarget)
    (if (not (Class|KismetSystemLibrary|TimerExists 0 "AimTick"))
      (Utilities|Time|SetTimerbyFunctionName 0 "AimTick" (Variables|Default|GetAimTickTime) true))
    (else
      (Utilities|Time|ClearTimerbyFunctionName 0 "AimTick"))))

(fn ChooseTarget
  (Variables|Target|SetTarget (Utilities|Array|Get(acopy) (Variables|Target|GetTargetArray))))

(fn ReloadTick
  (bind _ac_healthcomponent (Variables|Default|GetAC_HealthComponent))
  (bind _resources_taken (Variables|Default|GetResources%20Taken))
  (bind _ac_healthcomponent_2 (Variables|Default|GetAC_HealthComponent))
  (CallFunction|CanRepair)
  (if (not (>= (Variables|/Game/ShadowDuckStudio/Blueprints/HealthSystem/AC_HealthComponent.AC_HealthComponent_C|GetCurrentHealth _ac_healthcomponent) (Variables|/Game/ShadowDuckStudio/Blueprints/HealthSystem/AC_HealthComponent.AC_HealthComponent_C|GetMaxHealth _ac_healthcomponent)))
    (if (< (Variables|Reload|GetCurrentReloadTime) (Variables|Reload|GetMaxReloadTime))
      (Variables|Reload|SetCurrentReloadTime (+ (Variables|Reload|GetCurrentReloadTime) (Variables|Reload|GetReloadTickTime)))
      (else
        (Variables|Default|GetPlayerRef
          (:then
            _)
          (:else
            (bind _returnvalue (Actor|GetActorOfClass "/Game/ShadowDuckStudio/Blueprints/Player/BP_HMCharacter.BP_HMCharacter_C"))
            (Variables|Default|SetPlayerRef _returnvalue)))
        (if (not (< (.resource1 (Variables|/Game/ShadowDuckStudio/Blueprints/ResourcesSystem/AC_ResourceComponent.AC_ResourceComponent_C|GetResources (Variables|/Game/ShadowDuckStudio/Blueprints/Player/BP_HMCharacter.BP_HMCharacter_C|GetAC_ResourceComponent (Variables|Default|GetPlayerRef)))) _resources_taken))
          (if (> (Variables|/Game/ShadowDuckStudio/Blueprints/HealthSystem/AC_HealthComponent.AC_HealthComponent_C|GetCurrentHealth _ac_healthcomponent_2) (/ (Variables|/Game/ShadowDuckStudio/Blueprints/HealthSystem/AC_HealthComponent.AC_HealthComponent_C|GetMaxHealth _ac_healthcomponent_2) 2.0))
            (Default|TakeResource (Variables|/Game/ShadowDuckStudio/Blueprints/Player/BP_HMCharacter.BP_HMCharacter_C|GetAC_ResourceComponent (Variables|Default|GetPlayerRef)) (Utilities|Struct|MakeF_Resources (/ (Variables|Default|GetResources%20Taken) 2)))
            (else
              (Default|TakeResource (Variables|/Game/ShadowDuckStudio/Blueprints/Player/BP_HMCharacter.BP_HMCharacter_C|GetAC_ResourceComponent (Variables|Default|GetPlayerRef)) (Utilities|Struct|MakeF_Resources _resources_taken))))
          (Class|BIHealthInterface|Heal(Message) (Variables|Default|GetAC_HealthComponent) (Variables|Reload|GetReloadAmount))
          (Utilities|Time|ClearTimerbyFunctionName 0 "ReloadTick")
          (CallFunction|CheckRepairVisible)
          (CallFunction|CheckSmallerRadius))))))

(fn SetClosestTarget
  (bind _returnvalue (Transformation|GetActorLocation))
  (bind _targetarray (Variables|Target|GetTargetArray))
  (bind _returnvalue_2 (Actor|FindNearestActor _returnvalue _targetarray))
  (bind _target (Variables|Target|GetTarget)
    (:then
      (if (not (== _target _returnvalue_2))
        (Utilities|IsValid _returnvalue_2 :!label _label
          (:Is%20Valid
            (Variables|Target|SetTarget _returnvalue_2))
          (:Is%20Not%20Valid
            (Variables|Target|SetTarget 0)))
        (return)))
    (:else
      (goto _label))))

(fn EndTrap)

(fn BeginTrap)

(fn GetOverlayMeshes
  (return 0))