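; BP_ProjectileBase is a base turret projectile that damages what its BulletMesh overlaps, as either a single target or an area explosion.
; A positive ExplosionRadius gathers unique actors by sphere trace (with debug drawing), otherwise only the overlapped actor counts; IgnoredClasses are filtered out.
; Hit sends Damage through BI_HealthInterface components, optionally adds a ComponentOnHit component to each victim, and destroys the projectile only when something was hit.
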(event OnComponentBeginOverlap(BulletMesh)
  (params (OverlappedComponent :type Primitive%20Component%20Object%20Reference) (OtherActor :type Actor%20Object%20Reference) (OtherComp :type Primitive%20Component%20Object%20Reference) (OtherBodyIndex :type Integer) (bFromSweep :type Boolean) (SweepResult :type Hit%20Result%20Structure%20%28by%20ref%29))
  (Variables|Default|SetOriginallyHitActor OtherActor)
  (if (> (Variables|Default|GetExplosionRadius) 0.0)
    (CallFunction|Explosion)
    (else
      (CallFunction|SingleTarget))))

(event Custom|Hit
  (bind _componentonhit (Variables|Default|GetComponentOnHit))
  (bind _hitactors (Variables|Default|GetHitActors))
  (if (not (Utilities|Array|IsEmpty _hitactors))
    (for _array_element _hitactors
      (Utilities|IsValid _array_element
        (:Is%20Valid
          (for _array_element_2 (Class|Actor|GetComponentsbyInterface _array_element "/Game/ShadowDuckStudio/Blueprints/HealthSystem/BI_HealthInterface.BI_HealthInterface_C")
            (Utilities|IsValid _array_element_2
              (:Is%20Valid
                (Class|BIHealthInterface|Damage(Message) _array_element_2 (Variables|Default|GetDamage)))))
          (if (Utilities|IsValidClass _componentonhit)
            (Utilities|IsValid _array_element
              (:Is%20Valid
                (Game|AddComponentbyClass _array_element _componentonhit)))))))
    (Actor|DestroyActor)))

(event Custom|SingleTarget
  (bind _originallyhitactor (Variables|Default|GetOriginallyHitActor))
  (Utilities|IsValid _originallyhitactor
    (:Is%20Valid
      (if (not (Utilities|Array|ContainsItem (Variables|Default|GetIgnoredClasses) (Utilities|GetClass _originallyhitactor)))
        (Variables|Default|SetHitActors (Utilities|Array|MakeArray _originallyhitactor))
        (CallFunction|Hit)))))

(event Custom|Explosion
  (bind _returnvalue (Transformation|GetActorLocation))
  (bind _outhits (Collision|MultiSphereTraceByChannel _returnvalue _returnvalue (Variables|Default|GetExplosionRadius) "TraceTypeQuery1" false 0 "ForDuration"))
  (for _array_element _outhits
    (if (not (Utilities|Array|ContainsItem (Variables|Default|GetIgnoredClasses) (Utilities|GetClass (.HitActor (Collision|BreakHitResult _array_element)))))
      (Utilities|Array|AddUnique (Variables|Default|GetHitActors) (.HitActor (Collision|BreakHitResult _array_element)))))
  (CallFunction|Hit))

(event EventBeginPlay)

(event Collision|EventActorBeginOverlap
  (params (OtherActor :type Actor%20Object%20Reference)))

(event EventTick
  (params (DeltaSeconds :type Float%20%28single-precision%29)))

(fn ConstructionScript)