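; Base turret projectile that flies straight forward and damages what it hits.
; A looping timer calls MoveTick, which moves the actor a fixed step along its forward vector with a swept move.
; Sphere hits ignore actors of exactly the base projectile or turret class, not their subclasses.
; Other hits send damage to every component implementing BI_HealthInterface, then destroy the projectile.
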(event OnComponentBeginOverlap(Sphere)
  (params (OverlappedComponent :type Primitive%20Component%20Object%20Reference) (OtherActor :type Actor%20Object%20Reference) (OtherComp :type Primitive%20Component%20Object%20Reference) (OtherBodyIndex :type Integer) (bFromSweep :type Boolean) (SweepResult :type Hit%20Result%20Structure%20%28by%20ref%29)))

(event OnComponentHit(Sphere)
  (params (HitComponent :type Primitive%20Component%20Object%20Reference) (OtherActor :type Actor%20Object%20Reference) (OtherComp :type Primitive%20Component%20Object%20Reference) (NormalImpulse :type Vector :default "0, 0, 0") (Hit :type Hit%20Result%20Structure%20%28by%20ref%29))
  (bind _returnvalue (Utilities|GetClass OtherActor))
  (Utilities|IsValid OtherActor
    (:Is%20Valid
      (if (not (or (== _returnvalue "BP_Projectile_Base_C") (== _returnvalue "/Game/ShadowDuckStudio/Blueprints/Turrets/BP_Turret_Base.BP_Turret_Base_C")))
        (for _array_element (Class|Actor|GetComponentsbyInterface OtherActor "/Game/ShadowDuckStudio/Blueprints/HealthSystem/BI_HealthInterface.BI_HealthInterface_C")
          (Utilities|IsValid _array_element
            (:Is%20Valid
              (Class|BIHealthInterface|Damage(Message) _array_element (Variables|Default|GetDamage)))))
        (Actor|DestroyActor)))))

(event EventBeginPlay
  (Utilities|Time|SetTimerbyFunctionName 0 "MoveTick" (Variables|Movement|GetMoveTickTime) true))

(fn ConstructionScript)

(fn MoveTick
  (Transformation|SetActorLocation (+ (Transformation|GetActorLocation) (* (Transformation|GetActorForwardVector) (Variables|Movement|GetMoveSpeed))) true false))