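; Turret actor component that fires projectiles in bursts, gated by CanFire and a cooldown.
; BeginCharge starts a charge timer only if TotalChargeTime is negative; otherwise it bursts immediately and damages the first BP_Turret_CrystalThrower found.
; Bursts loop Fire with a Delay, spawning several projectiles per shot at FiringPoint with random rotational spread.
; EndBurst runs a looping cooldown timer that re-enables firing.
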(event Custom|Fire
  (for _index (range 1 (Variables|Spread|GetTotalSpreadCount))
    (Game|SpawnActorfromClass (Variables|Projectile|GetProjectileClass) (CallFunction|SetProjectileTransform) "Undefined" "MultiplyWithRoot" 0 0)))

(event Custom|BeginCharge
  (if (Variables|Default|GetCanFire?)
    (Variables|Default|SetCanFire? false)
    (Variables|Charge|SetCurrentChargeTime 0.0)
    (if (> 0.0 (Variables|Charge|GetTotalChargeTime))
      (Utilities|Time|SetTimerbyFunctionName 0 "ChargeTick" (Variables|Charge|GetChargeTickTime) true)
      (else
        (CallFunction|BeginBurst)
        (bind _returnvalue (Actor|GetActorOfClass "/Game/ShadowDuckStudio/Blueprints/Turrets/BP_Turret_CrystalThrower.BP_Turret_CrystalThrower_C"))
        (Default|Damage (Variables|/Game/ShadowDuckStudio/Blueprints/Turrets/BP_Turret_CrystalThrower.BP_Turret_CrystalThrower_C|GetAC_HealthComponent _returnvalue) (Variables|Default|GetDamage))))))

(event Custom|EndCharge
  (params (ShouldFire? :type Boolean))
  (Utilities|Time|ClearTimerbyFunctionName 0 "Charge Tick")
  (if ShouldFire?
    (CallFunction|BeginBurst)))

(event Custom|BeginBurst
  (Variables|Burst|SetCurrentBurstCount 0)
  (if (< (Variables|Burst|GetCurrentBurstCount) (Variables|Burst|GetTotalBurstCount)) :!label _label
    (CallFunction|Fire)
    (Utilities|FlowControl|Delay (Variables|Burst|GetBurstCooldown))
    (Variables|Burst|SetCurrentBurstCount (+ (Variables|Burst|GetCurrentBurstCount) 1))
    (goto _label)
    (else
      (CallFunction|EndBurst))))

(event Custom|EndBurst
  (Variables|Cooldown|SetCurrentCooldownTime 0.0)
  (Utilities|Time|SetTimerbyFunctionName 0 "CooldownTick" (Variables|Cooldown|GetCooldownTickTime) true))

(event EventBeginPlay)

(fn ChargeTick
  (Variables|Charge|SetCurrentChargeTime (+ (Variables|Charge|GetCurrentChargeTime) (Variables|Charge|GetChargeTickTime)))
  (if (>= (Variables|Charge|GetTotalChargeTime) (Variables|Charge|GetCurrentChargeTime))
    (CallFunction|EndCharge (>= (Variables|Charge|GetTotalChargeTime) (Variables|Charge|GetCurrentChargeTime)))))

(fn SetProjectileTransform
  (bind _firingpoint (Variables|Default|GetFiringPoint))
  (bind _returnvalue (Transformation|GetWorldRotation _firingpoint))
  (bind (_roll _pitch _yaw) (Math|Rotator|BreakRotator _returnvalue))
  (return (Math|Transform|MakeTransform (Transformation|GetWorldLocation _firingpoint) (Math|Rotator|MakeRotator (+ _roll (Math|Random|RandomFloatinRange (Variables|Spread|GetMinSpreadX) (Variables|Spread|GetMaxSpreadX))) (+ _pitch (Math|Random|RandomFloatinRange (Variables|Spread|GetMinSpreadY) (Variables|Spread|GetMaxSpreadY))) (+ _yaw (Math|Random|RandomFloatinRange (Variables|Spread|GetMinSpreadZ) (Variables|Spread|GetMaxSpreadZ)))))))

(fn CooldownTick
  (Variables|Cooldown|SetCurrentCooldownTime (+ (Variables|Cooldown|GetCurrentCooldownTime) (Variables|Cooldown|GetCooldownTickTime)))
  (if (not (> (Variables|Cooldown|GetTotalCooldownTime) (Variables|Cooldown|GetCurrentCooldownTime)))
    (Variables|Default|SetCanFire? true)
    (Utilities|Time|ClearTimerbyFunctionName 0 "CooldownTick")))