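; BP_EnemyFast is an enemy Blueprint, named as the fast variant, that takes its stats from the current wave's data.
; On BeginPlay it runs the parent logic, then sets damage, health, damage tick time and walk speed from the "2"-suffixed fields of that wave entry.
; An OnFire event binds a Niagara burn effect to the skeletal mesh and deactivates it after a fixed delay.
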(event EventBeginPlay
  (bind _wavedata (Variables|Default|GetWaveData))
  (bind _ac_healthcomponent (Variables|Default|GetAC_HealthComponent))
  (bind _wavemanager (Variables|Default|GetWaveManager))
  (bind _currentwave (Variables|/Game/ShadowDuckStudio/Blueprints/WaveSystem/WaveSystem.WaveSystem_C|GetCurrentWave _wavemanager))
  (bind _output (Utilities|Array|Get(acopy) _wavedata _currentwave))
  (bind (_enemyclass_1 _amount_1 _dps_1 _health_1 _movementspeed_1 _attackspeed_1 _enemyclass_2 _amount_2 _dps_2 _health_2 _attackspeed_2 _movement_2) (Utilities|Struct|BreakF_WaveData _output))
  (|CallParentFunction)
  (Variables|Default|SetDamage_0 _dps_2)
  (bind _output_get (Variables|/Game/ShadowDuckStudio/Blueprints/HealthSystem/AC_HealthComponent.AC_HealthComponent_C|SetMaxHealth _ac_healthcomponent _health_2))
  (Variables|/Game/ShadowDuckStudio/Blueprints/HealthSystem/AC_HealthComponent.AC_HealthComponent_C|SetCurrentHealth _ac_healthcomponent _output_get)
  (Variables|Default|SetDamageTickTime _attackspeed_2)
  (Variables|/Script/Engine.CharacterMovementComponent|SetMaxWalkSpeed (Variables|Character|GetCharacterMovement) _movement_2))

(event Collision|EventActorBeginOverlap
  (params (OtherActor :type Actor%20Object%20Reference))
  (|CallParentFunction OtherActor) ; This node is disabled and will not be called.\nDrag off pins to build functionality.
)

(event EventTick
  (params (DeltaSeconds :type Float%20%28single-precision%29))
  (|CallParentFunction DeltaSeconds) ; This node is disabled and will not be called.\nDrag off pins to build functionality.
)

(event EventOnFire
  (bind _fxs_onfire (Variables|Default|GetFXS_OnFIre))
  (Class|NiagaraFunctionLibrary|OverrideSystemUserVariableSkeletalMeshComponent _fxs_onfire "" (Variables|Character|GetMesh))
  (Components|Activation|Activate _fxs_onfire true)
  (Utilities|FlowControl|Delay 5.0)
  (Components|Activation|Deactivate _fxs_onfire))

(fn ConstructionScript
  (|CallParentFunction))