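; Base enemy Blueprint that registers with the WaveSystem on spawn and deregisters on death.
; BeginPlay also loads DT_WaveData rows and copies damage and attack speed into the AI Blackboard.
; Box overlaps maintain class-filtered melee targets and publish the nearest as MeleeTarget; Stun sets a timed Blackboard flag.
; DamageTick damages every melee target through AC_HealthComponent and launches Characters away from the enemy.
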(event OnComponentBeginOverlap(Box)
  (params (OverlappedComponent :type Primitive%20Component%20Object%20Reference) (OtherActor :type Actor%20Object%20Reference) (OtherComp :type Primitive%20Component%20Object%20Reference) (OtherBodyIndex :type Integer) (bFromSweep :type Boolean) (SweepResult :type Hit%20Result%20Structure%20%28by%20ref%29))
  (CallFunction|Add/RemoveArray (Variables|Default|GetMeleeTargets) OtherActor "NewEnumerator0" (Variables|Default|GetMeleeTargetClasses) "NewEnumerator1")
  (CallFunction|SetClosestInteractable)
  (AI|Components|Blackboard|SetValueasObject (AI|GetBlackboard 0) (Utilities|Name|MakeLiteralName "MeleeTarget") (Variables|Default|GetMainTarget)))

(event OnComponentEndOverlap(Box)
  (params (OverlappedComponent :type Primitive%20Component%20Object%20Reference) (OtherActor :type Actor%20Object%20Reference) (OtherComp :type Primitive%20Component%20Object%20Reference) (OtherBodyIndex :type Integer))
  (CallFunction|Add/RemoveArray (Variables|Default|GetMeleeTargets) OtherActor "NewEnumerator1" (Variables|Default|GetMeleeTargetClasses) "NewEnumerator1")
  (CallFunction|SetClosestInteractable)
  (AI|Components|Blackboard|SetValueasObject (AI|GetBlackboard 0) (Utilities|Name|MakeLiteralName "MeleeTarget") (Variables|Default|GetMainTarget)))

(event Custom|Stun
  (params (StunDuration :type Float%20%28double-precision%29))
  (bind _returnvalue (Utilities|Name|MakeLiteralName "Stun?"))
  (bind _returnvalue_2 (AI|GetBlackboard 0))
  (AI|Components|Blackboard|SetValueasBool _returnvalue_2 _returnvalue true)
  (Utilities|FlowControl|Delay StunDuration)
  (AI|Components|Blackboard|SetValueasBool _returnvalue_2 _returnvalue false))

(event EventBeginPlay
  (bind _returnvalue (AI|GetBlackboard 0))
  (bind _returnvalue_2 (Actor|GetActorOfClass "/Game/ShadowDuckStudio/Blueprints/WaveSystem/WaveSystem.WaveSystem_C"))
  (bind _output_get (Variables|Default|SetWaveManager _returnvalue_2))
  (Class|BIWaveInterface|AddEnemytoWave(Message) _output_get self)
  (bind _outrownames (DataTable|GetDataTableRowNames "/Game/ShadowDuckStudio/Blueprints/DataTables/DT_WaveData.DT_WaveData"))
  (for _array_element _outrownames
    (bind _returnvalue_3 (Utilities|GetDataTableRow "/Game/ShadowDuckStudio/Blueprints/DataTables/DT_WaveData.DT_WaveData" _array_element)
      (:then
        (Utilities|Array|Add (Variables|Default|GetWaveData) _returnvalue_3))))
  (AI|Components|Blackboard|SetValueasFloat _returnvalue (Utilities|Name|MakeLiteralName "Damage") (Variables|Default|GetDamage_0))
  (AI|Components|Blackboard|SetValueasFloat _returnvalue (Utilities|Name|MakeLiteralName "AttackSpeed") (Variables|Default|GetDamageTickTime)))

(event EventDeath
  (Class|BIWaveInterface|RemoveEnemyfromWave(Message) (Variables|Default|GetWaveManager) self)
  (Actor|DestroyActor)
  (bind _enemyminimapicon (Variables|Default|GetEnemyMinimapIcon)
    (:then
      (Components|DestroyComponent _enemyminimapicon))
    (:else)))

(fn ConstructionScript)

(fn DamageTick
  (bind _self self)
  (bind _returnvalue (Transformation|GetActorLocation _self))
  (for _array_element (Variables|Default|GetMeleeTargets)
    (Class|BIHealthInterface|Damage(Message) (Actor|GetComponentbyClass _array_element "/Game/ShadowDuckStudio/Blueprints/HealthSystem/AC_HealthComponent.AC_HealthComponent_C") (Variables|Default|GetDamage_0))
    (bind _ascharacter (Utilities|Casting|CastToCharacter _array_element))
    (Character|LaunchCharacter _ascharacter (* (Math|Rotator|GetRotationXVector (Math|Rotator|FindLookatRotation (Math|Vector|MakeVector (.x _returnvalue) (.y _returnvalue) 0.0) (Math|Vector|MakeVector (.x (Transformation|GetActorLocation _ascharacter)) (.y (Transformation|GetActorLocation _ascharacter)) 0.0))) (Variables|Default|GetHitImpulse)) false false)))

(fn SetClosestInteractable
  (bind _returnvalue (Transformation|GetActorLocation))
  (bind _meleetargets (Variables|Default|GetMeleeTargets))
  (bind _returnvalue_2 (Actor|FindNearestActor _returnvalue _meleetargets))
  (bind _maintarget (Variables|Default|GetMainTarget)
    (:then
      (if (not (== _maintarget _returnvalue_2))
        (Utilities|IsValid _returnvalue_2 :!label _label
          (:Is%20Valid
            (Variables|Default|SetMainTarget _returnvalue_2))
          (:Is%20Not%20Valid
            (Variables|Default|SetMainTarget 0)))
        (return)))
    (:else
      (goto _label))))