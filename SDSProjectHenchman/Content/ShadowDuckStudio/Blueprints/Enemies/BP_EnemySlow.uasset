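; BP_EnemySlow is a slow enemy variant that inherits its behavior from a parent enemy class.
; On BeginPlay, after the parent logic, it reads the current wave's entry from WaveData using WaveManager.CurrentWave.
; The third stat set there (DPS, Health, MovementSpeed, AttackSpeed) sets its damage, max health, walk speed and damage tick time.
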(event EventBeginPlay
  (bind _wavedata (Variables|Default|GetWaveData))
  (bind _wavemanager (Variables|Default|GetWaveManager))
  (bind _currentwave (Variables|/Game/ShadowDuckStudio/Blueprints/WaveSystem/WaveSystem.WaveSystem_C|GetCurrentWave _wavemanager))
  (bind _output (Utilities|Array|Get(acopy) _wavedata _currentwave))
  (bind (_enemyclass_1 _amount_1 _dps_1 _health_1 _movementspeed_1 _attackspeed_1 _enemyclass_2 _amount_2 _dps_2 _health_2 _attackspeed_2 _movement_2 _enemyclass_3 _amount_3 _dps_3 _health_3 _movementspeed_3 _attackspeed_3) (Utilities|Struct|BreakF_WaveData _output))
  (|CallParentFunction)
  (Variables|Default|SetDamage_0 _dps_3)
  (Variables|/Game/ShadowDuckStudio/Blueprints/HealthSystem/AC_HealthComponent.AC_HealthComponent_C|SetMaxHealth (Variables|Default|GetAC_HealthComponent) _health_3)
  (Variables|/Script/Engine.CharacterMovementComponent|SetMaxWalkSpeed (Variables|Character|GetCharacterMovement) _movementspeed_3)
  (Variables|Default|SetDamageTickTime _attackspeed_3))

(event Collision|EventActorBeginOverlap
  (params (OtherActor :type Actor%20Object%20Reference))
  (|CallParentFunction OtherActor) ; This node is disabled and will not be called.\nDrag off pins to build functionality.
)

(event EventTick
  (params (DeltaSeconds :type Float%20%28single-precision%29))
  (|CallParentFunction DeltaSeconds) ; This node is disabled and will not be called.\nDrag off pins to build functionality.
)

(fn ConstructionScript
  (|CallParentFunction))