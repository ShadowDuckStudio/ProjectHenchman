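; Fire trap that burns actors inside its Box while spending its own health as durability.
; Overlaps update a filtered occupant list, and CheckIsEmpty starts a looping DamageTick with fire FX or stops it after a delay.
; Each tick damages occupants and the trap through AC_HealthComponent, with a cube material swap.
; Interacting runs a reload timer that heals the trap on completion, and ending interaction cancels it.
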(event OnComponentBeginOverlap(Box)
  (params (OverlappedComponent :type Primitive%20Component%20Object%20Reference) (OtherActor :type Actor%20Object%20Reference) (OtherComp :type Primitive%20Component%20Object%20Reference) (OtherBodyIndex :type Integer) (bFromSweep :type Boolean) (SweepResult :type Hit%20Result%20Structure%20%28by%20ref%29))
  (Development|PrintString (Utilities|GetDisplayName OtherActor))
  (CallFunction|Add/RemoveArray (Variables|Default|GetActorsInCollision) OtherActor "NewEnumerator0" (Variables|Default|GetSpecial%20Classes) "NewEnumerator0")
  (CallFunction|CheckIsEmpty?))

(event OnComponentEndOverlap(Box)
  (params (OverlappedComponent :type Primitive%20Component%20Object%20Reference) (OtherActor :type Actor%20Object%20Reference) (OtherComp :type Primitive%20Component%20Object%20Reference) (OtherBodyIndex :type Integer))
  (CallFunction|Add/RemoveArray (Variables|Default|GetActorsInCollision) OtherActor "NewEnumerator1" (Variables|Default|GetSpecial%20Classes) "NewEnumerator0")
  (CallFunction|CheckIsEmpty?))

(event Custom|BeginTrap
  (Utilities|Time|SetTimerbyFunctionName 0 "DamageTick" (Variables|Default|GetDamageTickTime) true)
  (Components|Activation|Activate (Variables|Default|GetFXS_FrieTrap) true))

(event Custom|EndTrap
  (Utilities|FlowControl|Delay (Variables|Default|GetActiveTimeAfterLeft))
  (Utilities|Time|ClearTimerbyFunctionName 0 "DamageTick")
  (Components|Activation|Deactivate (Variables|Default|GetFXS_FrieTrap)))

(event EventBeginPlay)

(event Collision|EventActorBeginOverlap
  (params (OtherActor :type Actor%20Object%20Reference)))

(event EventTick
  (params (DeltaSeconds :type Float%20%28single-precision%29)))

(event EventBeginInteract
  (params (Source :type Actor%20Object%20Reference))
  (Variables|Default|SetCurrentReloadTime 0.0)
  (Utilities|Time|SetTimerbyFunctionName 0 "ReloadTick" (Variables|Default|GetReloadTickTime) true))

(event EventEndInteract
  (params (Source :type Actor%20Object%20Reference))
  (Utilities|Time|ClearTimerbyFunctionName 0 "ReloadTick"))

(fn ConstructionScript
  (|CallParentFunction))

(fn CheckIsEmpty?
  (if (> (Variables|/Game/ShadowDuckStudio/Blueprints/HealthSystem/AC_HealthComponent.AC_HealthComponent_C|GetCurrentHealth (Variables|Default|GetAC_HealthComponent)) 0.0)
    (if (Utilities|Array|IsEmpty (Variables|Default|GetActorsInCollision))
      (CallFunction|EndTrap :!label _label)
      (elif (not (Class|KismetSystemLibrary|TimerExists 0 "DamageTick"))
        (CallFunction|BeginTrap)))
    (else
      (goto _label))))

(fn DamageTick
  (bind _cube (Variables|Default|GetCube))
  (Rendering|Material|SetMaterial _cube 0 "/Engine/MapTemplates/Materials/BasicAsset01.BasicAsset01")
  (for _array_element (Variables|Default|GetActorsInCollision)
    (Class|BIHealthInterface|Damage(Message) (Actor|GetComponentbyClass _array_element "/Game/ShadowDuckStudio/Blueprints/HealthSystem/AC_HealthComponent.AC_HealthComponent_C") (Variables|Default|GetDamage)))
  (Rendering|Material|SetMaterial _cube 0 "/Engine/ArtTools/RenderToTexture/Materials/Debug/M_BaseColor_Constant.M_BaseColor_Constant")
  (Class|BIHealthInterface|Damage(Message) (Variables|Default|GetAC_HealthComponent) (Variables|Default|GetDurabilityPerTick)))

(fn ReloadTick
  (if (< (Variables|Default|GetCurrentReloadTime) (Variables|Default|GetMaxReloadTime))
    (Variables|Default|SetCurrentReloadTime (+ (Variables|Default|GetCurrentReloadTime) (Variables|Default|GetReloadTickTime)))
    (else
      (Class|BIHealthInterface|Heal(Message) (Variables|Default|GetAC_HealthComponent) (Variables|Default|GetReloadAmount))
      (Utilities|Time|ClearTimerbyFunctionName 0 "ReloadTick"))))

(fn GetOverlayMeshes
  (return 0))