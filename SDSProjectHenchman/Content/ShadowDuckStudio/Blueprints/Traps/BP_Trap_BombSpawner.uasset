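; Bomb spawner trap that spawns slime minions on a looping timer while valid targets are in range, with stats read from DefenceInfo.
; Health doubles as ammo: each spawn damages the trap, and spawning yields nothing at zero.
; Player interaction runs a timed reload that spends resources to restore health, at half cost above half health.
; Proximity spheres and health events toggle fuel, refill and minimap repair widgets.
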(event OnComponentBeginOverlap(Range)
  (params (OverlappedComponent :type Primitive%20Component%20Object%20Reference) (OtherActor :type Actor%20Object%20Reference) (OtherComp :type Primitive%20Component%20Object%20Reference) (OtherBodyIndex :type Integer) (bFromSweep :type Boolean) (SweepResult :type Hit%20Result%20Structure%20%28by%20ref%29))
  (bind _arrayempty_ (CallFunction|Add/RemoveArray (Variables|Default|GetTargetArray) OtherActor "NewEnumerator0" (Variables|Default|GetTargetClassesArray) "NewEnumerator1"))
  (if (not _arrayempty_)
    (CallFunction|StartSpawning)
    (CallFunction|TargetCheck)
    (CallFunction|CheckRepairVisible)))

(event OnComponentEndOverlap(Range)
  (params (OverlappedComponent :type Primitive%20Component%20Object%20Reference) (OtherActor :type Actor%20Object%20Reference) (OtherComp :type Primitive%20Component%20Object%20Reference) (OtherBodyIndex :type Integer))
  (bind _arrayempty_ (CallFunction|Add/RemoveArray (Variables|Default|GetTargetArray) OtherActor "NewEnumerator1" (Variables|Default|GetTargetClassesArray) "NewEnumerator1"))
  (if _arrayempty_
    (CallFunction|StopSpawning)
    (CallFunction|TargetCheck)
    (CallFunction|CheckRepairVisible)))

(event OnComponentEndOverlap(Sphere)
  (params (OverlappedComponent :type Primitive%20Component%20Object%20Reference) (OtherActor :type Actor%20Object%20Reference) (OtherComp :type Primitive%20Component%20Object%20Reference) (OtherBodyIndex :type Integer))
  (if (Actor|ActorHasTag OtherActor "Player")
    (Variables|Default|SetInVisibleRadius false)
    (CallFunction|CheckRepairVisible)))

(event OnComponentBeginOverlap(CollisionforFuel)
  (params (OverlappedComponent :type Primitive%20Component%20Object%20Reference) (OtherActor :type Actor%20Object%20Reference) (OtherComp :type Primitive%20Component%20Object%20Reference) (OtherBodyIndex :type Integer) (bFromSweep :type Boolean) (SweepResult :type Hit%20Result%20Structure%20%28by%20ref%29))
  (if (Actor|ActorHasTag OtherActor "Player")
    (Variables|Default|SetInSmallerRadius true)
    (Rendering|SetVisibility (Variables|Default|GetFuelCounterIcon) true false)
    (CallFunction|CheckSmallerRadius)))

(event OnComponentEndOverlap(CollisionforFuel)
  (params (OverlappedComponent :type Primitive%20Component%20Object%20Reference) (OtherActor :type Actor%20Object%20Reference) (OtherComp :type Primitive%20Component%20Object%20Reference) (OtherBodyIndex :type Integer))
  (if (Actor|ActorHasTag OtherActor "Player")
    (Variables|Default|SetInSmallerRadius false)
    (Rendering|SetVisibility (Variables|Default|GetFuelCounterIcon) false false)
    (CallFunction|CheckSmallerRadius)))

(event OnComponentBeginOverlap(Sphere)
  (params (OverlappedComponent :type Primitive%20Component%20Object%20Reference) (OtherActor :type Actor%20Object%20Reference) (OtherComp :type Primitive%20Component%20Object%20Reference) (OtherBodyIndex :type Integer) (bFromSweep :type Boolean) (SweepResult :type Hit%20Result%20Structure%20%28by%20ref%29))
  (if (Actor|ActorHasTag OtherActor "Player")
    (Variables|Default|SetInVisibleRadius true)
    (CallFunction|CheckRepairVisible)))

(event Custom|StopSpawning
  (Utilities|Time|ClearTimerbyFunctionName 0 "SpawnTick"))

(event Custom|StartSpawning
  (Utilities|Time|SetTimerbyFunctionName 0 "SpawnTick" (Variables|Default|GetSpawnTickTime) true))

(event Custom|CheckRepairVisible
  (bind _ammominimapwidget (Variables|Default|GetAmmoMinimapWidget))
  (bind _ac_healthcomponent (Variables|Default|GetAC_HealthComponent))
  (bind _repairiconminimap (Variables|Default|GetRepairIconMinimap))
  (bind _currenthealth (Variables|/Game/ShadowDuckStudio/Blueprints/HealthSystem/AC_HealthComponent.AC_HealthComponent_C|GetCurrentHealth _ac_healthcomponent))
  (bind _returnvalue (<= _currenthealth 0.0))
  (if _returnvalue
    (Rendering|SetVisibility _repairiconminimap true false)
    (else
      (Rendering|SetVisibility _repairiconminimap false false)))
  (if (and (Variables|Default|GetInVisibleRadius) _returnvalue)
    (Rendering|SetVisibility _ammominimapwidget true false)
    (else
      (Rendering|SetVisibility _ammominimapwidget false false))))

(event Custom|CanRepair
  (bind _ac_healthcomponent (Variables|Default|GetAC_HealthComponent))
  (bind _repairprogress (Variables|Default|GetRepairProgress))
  (bind _currenthealth (Variables|/Game/ShadowDuckStudio/Blueprints/HealthSystem/AC_HealthComponent.AC_HealthComponent_C|GetCurrentHealth _ac_healthcomponent))
  (if (== (Math|Vector|VectorLength (Transformation|GetVelocity (Game|Player|GetPlayerPawn 0))) 0.0)
    (if (and (< _currenthealth (Variables|/Game/ShadowDuckStudio/Blueprints/HealthSystem/AC_HealthComponent.AC_HealthComponent_C|GetMaxHealth _ac_healthcomponent)) (>= (.resource1 (Variables|/Game/ShadowDuckStudio/Blueprints/ResourcesSystem/AC_ResourceComponent.AC_ResourceComponent_C|GetResources (Variables|/Game/ShadowDuckStudio/Blueprints/Player/BP_HMCharacter.BP_HMCharacter_C|GetAC_ResourceComponent (.AsBP%20HMCharacter (Utilities|Casting|CastToBP_HMCharacter (Game|Player|GetPlayerPawn 0)))))) (Variables|Default|GetResources%20Taken%20)))
      (Rendering|SetVisibility _repairprogress true false)
      (if (== _currenthealth 2e+01)
        (Utilities|FlowControl|Delay 1.2)
        (Rendering|SetVisibility _repairprogress false false)))
    (else
      (Utilities|Time|ClearTimerbyFunctionName 0 "ReloadTick")
      (Rendering|SetVisibility _repairprogress false false))))

(event Custom|CheckSmallerRadius
  (bind _refillammowidget (Variables|Default|GetRefillAmmoWidget))
  (if (and (<= (Variables|/Game/ShadowDuckStudio/Blueprints/HealthSystem/AC_HealthComponent.AC_HealthComponent_C|GetCurrentHealth (Variables|Default|GetAC_HealthComponent)) 0.0) (Variables|Default|GetInSmallerRadius))
    (Rendering|SetVisibility _refillammowidget true false)
    (else
      (Rendering|SetVisibility _refillammowidget false false))))

(event Custom|End%20Progress
  (Rendering|SetVisibility (Variables|Default|GetRepairProgress) false false))

(event EventBeginPlay
  (bind _self self)
  (bind _defenceinfo (Variables|Default|GetDefenceInfo))
  (bind _output (Utilities|Array|Get(acopy) _defenceinfo 3))
  (bind (_slot _built _cost _angleconstraints _buildiconinfo _tag _def_dmg _def_attackspeed _def_repairamount _def_health _def_dmgpertickself _def_spawnspeed _def_pushstrength _def_dmgperhitself) (Utilities|Struct|BreakF_BuildInfo _output))
  (Variables|/Game/ShadowDuckStudio/UI/Widgets/TrapsandTurrets/AmmoCounterSpawner_WBP.AmmoCounterSpawner_WBP_C|SetSpawnerRef (.AsAmmo%20Counter%20Spawner%20WBP (Utilities|Casting|CastToAmmoCounterSpawner_WBP (UserInterface|GetWidget (Variables|Default|GetFuelCounterIcon)))) _self)
  (Variables|/Game/ShadowDuckStudio/UI/Widgets/TrapsandTurrets/RepairProgressSymbolSpawner_WBP.RepairProgressSymbolSpawner_WBP_C|SetBombSpawnerRef (.AsRepair%20Progress%20Symbol%20Spawner%20WBP (Utilities|Casting|CastToRepairProgressSymbolSpawner_WBP (UserInterface|GetWidget (Variables|Default|GetRepairProgress)))) _self)
  (bind _returnvalue (Actor|GetActorOfClass "/Game/ShadowDuckStudio/Blueprints/Minion/BP_SlimeMinion.BP_SlimeMinion_C"))
  (Variables|Default|SetMinionRef _returnvalue)
  (bind _returnvalue_2 (Actor|GetActorOfClass "/Game/ShadowDuckStudio/Blueprints/Player/BP_HMCharacter.BP_HMCharacter_C"))
  (Variables|Default|SetPlayerRef _returnvalue_2)
  (|CallParentFunction)
  (bind _minionref (Variables|Default|GetMinionRef)
    (:then
      (Variables|/Game/ShadowDuckStudio/Blueprints/Minion/BP_SlimeMinion.BP_SlimeMinion_C|SetInitialDamage _minionref _def_dmg))
    (:else
      _))
  (Variables|Default|SetSpawnTickTime _def_attackspeed)
  (Variables|Default|SetReloadAmount _def_repairamount)
  (bind _ac_healthcomponent (Variables|Default|GetAC_HealthComponent)
    (:then
      (Variables|/Game/ShadowDuckStudio/Blueprints/HealthSystem/AC_HealthComponent.AC_HealthComponent_C|SetMaxHealth _ac_healthcomponent _def_health))
    (:else
      _))
  (Variables|Default|SetDurabilityPerSpawn _def_dmgperhitself))

(event Collision|EventActorBeginOverlap
  (params (OtherActor :type Actor%20Object%20Reference))
  (|CallParentFunction OtherActor) ; This node is disabled and will not be called.\nDrag off pins to build functionality.
)

(event EventDamage
  (params (Damage :type Float%20%28double-precision%29))
  (CallFunction|CheckRepairVisible)
  (CallFunction|CheckSmallerRadius))

(event EventTick
  (params (DeltaSeconds :type Float%20%28single-precision%29))
  (|CallParentFunction DeltaSeconds) ; This node is disabled and will not be called.\nDrag off pins to build functionality.
)

(event EventDeath
  (CallFunction|CheckRepairVisible)
  (CallFunction|CheckSmallerRadius))

(event EventEndInteract
  (params (Source :type Actor%20Object%20Reference))
  (Utilities|Time|ClearTimerbyFunctionName 0 "ReloadTick"))

(event EventBeginInteract
  (params (Source :type Actor%20Object%20Reference))
  (Variables|Default|SetCurrentReloadTime 0.0)
  (Utilities|Time|SetTimerbyFunctionName 0 "ReloadTick" (Variables|Default|GetReloadTickTime) true))

(event EventBeginDeconstruct
  (params (Source :type Actor%20Object%20Reference))
  (CallFunction|BeginDeconstructTimer self Source (Variables|Default|GetRefund)))

(event EventHeal
  (params (Amount :type Float%20%28double-precision%29))
  (CallFunction|CheckRepairVisible)
  (CallFunction|CheckSmallerRadius))

(fn ConstructionScript
  (|CallParentFunction))

(fn SpawnTick
  (if (> (Variables|/Game/ShadowDuckStudio/Blueprints/HealthSystem/AC_HealthComponent.AC_HealthComponent_C|GetCurrentHealth (Variables|Default|GetAC_HealthComponent)) 0.0)
    (Game|SpawnActorfromClass "/Game/ShadowDuckStudio/Blueprints/Minion/BP_SlimeMinion.BP_SlimeMinion_C" (Transformation|GetWorldTransform (Variables|Default|GetBombMinionMesh)) "AdjustIfPossibleButAlwaysSpawn" "MultiplyWithRoot" 0 0)
    (Class|BIHealthInterface|Damage(Message) (Variables|Default|GetAC_HealthComponent) (Variables|Default|GetDurabilityPerSpawn))))

(fn ReloadTick
  (bind _ac_healthcomponent (Variables|Default|GetAC_HealthComponent))
  (bind _resources_taken_ (Variables|Default|GetResources%20Taken%20))
  (bind _ac_healthcomponent_2 (Variables|Default|GetAC_HealthComponent))
  (CallFunction|CanRepair)
  (if (not (>= (Variables|/Game/ShadowDuckStudio/Blueprints/HealthSystem/AC_HealthComponent.AC_HealthComponent_C|GetCurrentHealth _ac_healthcomponent) (Variables|/Game/ShadowDuckStudio/Blueprints/HealthSystem/AC_HealthComponent.AC_HealthComponent_C|GetMaxHealth _ac_healthcomponent)))
    (if (< (Variables|Default|GetCurrentReloadTime) (Variables|Default|GetMaxReloadTime))
      (Variables|Default|SetCurrentReloadTime (+ (Variables|Default|GetCurrentReloadTime) (Variables|Default|GetReloadTickTime)))
      (else
        (Variables|Default|GetPlayerRef
          (:then
            _)
          (:else
            (bind _returnvalue (Actor|GetActorOfClass "/Game/ShadowDuckStudio/Blueprints/Player/BP_HMCharacter.BP_HMCharacter_C"))
            (Variables|Default|SetPlayerRef _returnvalue)))
        (if (< (.resource1 (Variables|/Game/ShadowDuckStudio/Blueprints/ResourcesSystem/AC_ResourceComponent.AC_ResourceComponent_C|GetResources (Variables|/Game/ShadowDuckStudio/Blueprints/Player/BP_HMCharacter.BP_HMCharacter_C|GetAC_ResourceComponent (Variables|Default|GetPlayerRef)))) _resources_taken_)
          (Development|PrintString "Returning true")
          (else
            (if (> (Variables|/Game/ShadowDuckStudio/Blueprints/HealthSystem/AC_HealthComponent.AC_HealthComponent_C|GetCurrentHealth _ac_healthcomponent_2) (/ (Variables|/Game/ShadowDuckStudio/Blueprints/HealthSystem/AC_HealthComponent.AC_HealthComponent_C|GetMaxHealth _ac_healthcomponent_2) 2.0))
              (Default|TakeResource (Variables|/Game/ShadowDuckStudio/Blueprints/Player/BP_HMCharacter.BP_HMCharacter_C|GetAC_ResourceComponent (Variables|Default|GetPlayerRef)) (Utilities|Struct|MakeF_Resources (/ (Variables|Default|GetResources%20Taken%20) 2)))
              (else
                (Default|TakeResource (Variables|/Game/ShadowDuckStudio/Blueprints/Player/BP_HMCharacter.BP_HMCharacter_C|GetAC_ResourceComponent (Variables|Default|GetPlayerRef)) (Utilities|Struct|MakeF_Resources _resources_taken_))))
            (Class|BIHealthInterface|Heal(Message) (Variables|Default|GetAC_HealthComponent) (Variables|Default|GetReloadAmount))
            (Utilities|Time|ClearTimerbyFunctionName 0 "ReloadTick")
            (CallFunction|CheckRepairVisible)
            (CallFunction|CheckSmallerRadius)))))))

(fn TargetCheck
  (if (Utilities|Array|IsNotEmpty (Variables|Default|GetTargetArray))
    (CallFunction|ChooseTarget)
    (if (not (Class|KismetSystemLibrary|TimerExists 0 "AimTick"))
      (Utilities|Time|SetTimerbyFunctionName 0 "AimTick" (Variables|Default|GetAimTickTime) true))
    (else
      (Utilities|Time|ClearTimerbyFunctionName 0 "AimTick"))))

(fn ChooseTarget
  (Variables|Default|SetTarget (Utilities|Array|Get(acopy) (Variables|Default|GetTargetArray))))

(fn SetClosestTarget
  (bind _returnvalue (Transformation|GetActorLocation))
  (bind _targetarray (Variables|Default|GetTargetArray))
  (bind _returnvalue_2 (Actor|FindNearestActor _returnvalue _targetarray))
  (bind _target (Variables|Default|GetTarget)
    (:then
      (if (not (== _target _returnvalue_2))
        (Utilities|IsValid _returnvalue_2 :!label _label
          (:Is%20Valid
            (Variables|Default|SetTarget _returnvalue_2))
          (:Is%20Not%20Valid
            (Variables|Default|SetTarget 0)))
        (return)))
    (:else
      (goto _label))))

(fn GetOverlayMeshes
  (return 0))