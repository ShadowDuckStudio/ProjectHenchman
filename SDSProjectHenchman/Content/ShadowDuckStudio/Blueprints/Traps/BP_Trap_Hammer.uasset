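; BP_Trap_Hammer is a hammer trap that knocks back and damages what touches its LeftCollision component.
; On overlap, characters are launched and other physics-simulating components receive an impulse, both along LeftForcePoint's forward vector scaled by ImpulseStrength.
; Any overlapping actor with an AC_HealthComponent is also sent Damage through DamageMessage.
; The graphs contain no swing logic and handle only the left-side collision.
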(event OnComponentBeginOverlap(LeftCollision)
  (params (OverlappedComponent :type Primitive%20Component%20Object%20Reference) (OtherActor :type Actor%20Object%20Reference) (OtherComp :type Primitive%20Component%20Object%20Reference) (OtherBodyIndex :type Integer) (bFromSweep :type Boolean) (SweepResult :type Hit%20Result%20Structure%20%28by%20ref%29))
  (bind _returnvalue (Actor|GetComponentbyClass OtherActor "/Game/ShadowDuckStudio/Blueprints/HealthSystem/AC_HealthComponent.AC_HealthComponent_C"))
  (bind _leftforcepoint (Variables|Default|GetLeftForcePoint))
  (bind _impulsestrength (Variables|Default|GetImpulseStrength))
  (bind _returnvalue_2 (Math|Vector|GetForwardVector _leftforcepoint))
  (bind _returnvalue_3 (* _returnvalue_2 _impulsestrength))
  (bind _ascharacter (Utilities|Casting|CastToCharacter OtherActor)
    (:then
      (Character|LaunchCharacter _ascharacter _returnvalue_3 false false))
    (:CastFailed
      (if (Class|SceneComponent|IsAnySimulatingPhysics OtherComp)
        (Physics|AddImpulseatLocation OtherComp _returnvalue_3 (Transformation|GetWorldLocation _leftforcepoint) "None"))))
  (Utilities|IsValid _returnvalue
    (:Is%20Valid
      (Class|BIHealthInterface|Damage(Message) _returnvalue (Variables|Default|GetDamage)))))

(event EventBeginPlay
  (|CallParentFunction) ; This node is disabled and will not be called.\nDrag off pins to build functionality.
)

(event Collision|EventActorBeginOverlap
  (params (OtherActor :type Actor%20Object%20Reference))
  (|CallParentFunction OtherActor) ; This node is disabled and will not be called.\nDrag off pins to build functionality.
)

(event EventTick
  (params (DeltaSeconds :type Float%20%28single-precision%29))
  (|CallParentFunction DeltaSeconds) ; This node is disabled and will not be called.\nDrag off pins to build functionality.
)

(fn ConstructionScript
  (|CallParentFunction))