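; Fire trap defence that burns actors in its box with flame FX and sound, configured from DefenceInfo.
; Tracked overlaps start a looping damage timer that hurts occupants, begins damage-over-time and drains the trap's own health; it stops when empty or broken.
; Any box overlap also briefly activates the player's on-fire FX.
; Holding interact repairs it for player resources via a reload timer, with minimap icon and proximity widgets shown when broken.
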(event OnComponentEndOverlap(Sphere)
  (params (OverlappedComponent :type Primitive%20Component%20Object%20Reference) (OtherActor :type Actor%20Object%20Reference) (OtherComp :type Primitive%20Component%20Object%20Reference) (OtherBodyIndex :type Integer))
  (if (Actor|ActorHasTag OtherActor "Player")
    (Variables|Default|SetInVisibleRadius false)
    (CallFunction|CheckRepairVisible)))

(event OnComponentBeginOverlap(Box)
  (params (OverlappedComponent :type Primitive%20Component%20Object%20Reference) (OtherActor :type Actor%20Object%20Reference) (OtherComp :type Primitive%20Component%20Object%20Reference) (OtherBodyIndex :type Integer) (bFromSweep :type Boolean) (SweepResult :type Hit%20Result%20Structure%20%28by%20ref%29))
  (bind _playerref (Variables|Default|GetPlayerRef))
  (bind _fxs_onfire (Variables|/Game/ShadowDuckStudio/Blueprints/Player/BP_HMCharacter.BP_HMCharacter_C|GetFXS_OnFIre _playerref))
  (CallFunction|Add/RemoveArray (Variables|Default|GetActorsInCollision) OtherActor "NewEnumerator0" (Variables|Default|GetSpecial%20Classes) "NewEnumerator0")
  (CallFunction|CheckIsEmpty?)
  (CallFunction|CheckRepairVisible)
  (Components|Activation|Activate _fxs_onfire true)
  (Utilities|FlowControl|Delay 5.0)
  (Components|Activation|Deactivate _fxs_onfire)
  (Default|DOT (Variables|Default|GetAC_DOT_Base)))

(event OnComponentEndOverlap(Box)
  (params (OverlappedComponent :type Primitive%20Component%20Object%20Reference) (OtherActor :type Actor%20Object%20Reference) (OtherComp :type Primitive%20Component%20Object%20Reference) (OtherBodyIndex :type Integer))
  (CallFunction|Add/RemoveArray (Variables|Default|GetActorsInCollision) OtherActor "NewEnumerator1" (Variables|Default|GetSpecial%20Classes) "NewEnumerator0")
  (CallFunction|CheckIsEmpty?)
  (CallFunction|CheckRepairVisible))

(event OnComponentBeginOverlap(Sphere)
  (params (OverlappedComponent :type Primitive%20Component%20Object%20Reference) (OtherActor :type Actor%20Object%20Reference) (OtherComp :type Primitive%20Component%20Object%20Reference) (OtherBodyIndex :type Integer) (bFromSweep :type Boolean) (SweepResult :type Hit%20Result%20Structure%20%28by%20ref%29))
  (if (Actor|ActorHasTag OtherActor "Player")
    (Variables|Default|SetInVisibleRadius true)
    (CallFunction|CheckRepairVisible)))

(event Custom|BeginTrap
  (bind _fxs_frietrap (Variables|Default|GetFXS_FrieTrap))
  (Utilities|Time|SetTimerbyFunctionName 0 "DamageTick" (Variables|Default|GetDamageTickTime) true)
  (Components|Activation|Activate _fxs_frietrap true)
  (bind _returnvalue (Audio|SpawnSoundatLocation "/Game/ShadowDuckStudio/SFX/TurretSFX/FlameTrapFire.FlameTrapFire" (Transformation|GetWorldLocation _fxs_frietrap) "0, 0, 0" 1.0 1.0 0.0 0 0))
  (Audio|Components|Audio|Play _returnvalue 0.0))

(event Custom|EndTrap
  (Utilities|FlowControl|Delay (Variables|Default|GetActiveTimeAfterLeft))
  (Utilities|Time|ClearTimerbyFunctionName 0 "DamageTick")
  (Components|Activation|Deactivate (Variables|Default|GetFXS_FrieTrap))
  (Audio|Components|Audio|Stop (stale Custom|BeginTrap _returnvalue)))

(event Custom|CheckRepairVisible
  (bind _repairiconminimap (Variables|Default|GetRepairIconMinimap))
  (bind _ac_healthcomponent (Variables|Default|GetAC_HealthComponent))
  (bind _repairwidget (Variables|Default|GetRepairWidget))
  (bind _currenthealth (Variables|/Game/ShadowDuckStudio/Blueprints/HealthSystem/AC_HealthComponent.AC_HealthComponent_C|GetCurrentHealth _ac_healthcomponent))
  (bind _returnvalue (<= _currenthealth 0.0))
  (if _returnvalue
    (Rendering|SetVisibility _repairiconminimap true false)
    (else
      (Rendering|SetVisibility _repairiconminimap false false)))
  (if (and (Variables|Default|GetInVisibleRadius) _returnvalue)
    (Rendering|SetVisibility _repairwidget true false)
    (else
      (Rendering|SetVisibility _repairwidget false false))))

(event EventBeginPlay
  (bind _defenceinfo (Variables|Default|GetDefenceInfo))
  (bind _output (Utilities|Array|Get(acopy) _defenceinfo))
  (bind (_slot _built _cost _angleconstraints _buildiconinfo _tag _def_dmg _def_attackspeed _def_repairamount _def_health _def_dmgpertickself) (Utilities|Struct|BreakF_BuildInfo _output))
  (Utilities|FlowControl|Sequence
    (:then_0
      (if (Utilities|Array|IsEmpty _defenceinfo)
        (CallFunction|Ref))
      (bind _returnvalue (Actor|GetActorOfClass "/Game/ShadowDuckStudio/Blueprints/Player/BP_HMCharacter.BP_HMCharacter_C"))
      (Variables|Default|SetPlayerRef _returnvalue)
      (CallFunction|CheckRepairVisible)
      (bind _returnvalue_2 (Actor|GetActorOfClass "/Game/ShadowDuckStudio/Blueprints/Enemies/BP_Enemy_Base.BP_Enemy_Base_C"))
      (Variables|Default|SetEnemyBaseRef _returnvalue_2)
      (Variables|Default|SetDamageTaken _def_dmg)
      (Variables|Default|SetDamageTickTime _def_attackspeed)
      (Variables|Default|SetReloadAmount _def_repairamount)
      (Variables|/Game/ShadowDuckStudio/Blueprints/HealthSystem/AC_HealthComponent.AC_HealthComponent_C|SetMaxHealth (Variables|Default|GetAC_HealthComponent) _def_health)
      (Variables|Default|SetDurabilityPerTick _def_dmgpertickself))
    (:then_1
      (Utilities|FlowControl|Delay 1.0)
      (bind _returnvalue_3 (Audio|SpawnSoundAttached "/Game/ShadowDuckStudio/SFX/TurretSFX/FlameTrapPlacement.FlameTrapPlacement" (Variables|Default|GetDefaultSceneRoot) "None" "0, 0, 0" "0, 0, 0" "KeepRelativeOffset" false 1.0 1.0 0.0 0 0))
      (Audio|Components|Audio|Play _returnvalue_3 0.0))))

(event EventTick
  (params (DeltaSeconds :type Float%20%28single-precision%29)))

(event EventBeginInteract
  (params (Source :type Actor%20Object%20Reference))
  (Variables|Default|SetCurrentReloadTime 0.0)
  (Utilities|Time|SetTimerbyFunctionName 0 "ReloadTick" (Variables|Default|GetReloadTickTime) true))

(event EventEndInteract
  (params (Source :type Actor%20Object%20Reference))
  (Utilities|Time|ClearTimerbyFunctionName 0 "ReloadTick"))

(event EventHeal
  (params (Amount :type Float%20%28double-precision%29))
  (CallFunction|CheckRepairVisible))

(event EventDamage
  (params (Damage :type Float%20%28double-precision%29))
  (CallFunction|CheckRepairVisible))

(fn ConstructionScript
  (|CallParentFunction))

(fn CheckIsEmpty?
  (if (> (Variables|/Game/ShadowDuckStudio/Blueprints/HealthSystem/AC_HealthComponent.AC_HealthComponent_C|GetCurrentHealth (Variables|Default|GetAC_HealthComponent)) 0.0)
    (if (Utilities|Array|IsEmpty (Variables|Default|GetActorsInCollision))
      (CallFunction|EndTrap :!label _label)
      (elif (not (Class|KismetSystemLibrary|TimerExists 0 "DamageTick"))
        (CallFunction|BeginTrap)))
    (else
      (goto _label))))

(fn DamageTick
  (for _array_element (Variables|Default|GetActorsInCollision)
    (Class|BIHealthInterface|Damage(Message) (Actor|GetComponentbyClass _array_element "/Game/ShadowDuckStudio/Blueprints/HealthSystem/AC_HealthComponent.AC_HealthComponent_C") (Variables|Default|GetDamageTaken))
    (Default|BeginDOT (Variables|Default|GetAC_DOT_Base)))
  (Class|BIHealthInterface|Damage(Message) (Variables|Default|GetAC_HealthComponent) (Variables|Default|GetDurabilityPerTick)))

(fn ReloadTick
  (bind _ac_healthcomponent (Variables|Default|GetAC_HealthComponent))
  (bind _resources_taken (Variables|Default|GetResources%20Taken))
  (if (not (>= (Variables|/Game/ShadowDuckStudio/Blueprints/HealthSystem/AC_HealthComponent.AC_HealthComponent_C|GetCurrentHealth _ac_healthcomponent) (Variables|/Game/ShadowDuckStudio/Blueprints/HealthSystem/AC_HealthComponent.AC_HealthComponent_C|GetMaxHealth _ac_healthcomponent)))
    (if (< (Variables|Default|GetCurrentReloadTime) (Variables|Default|GetMaxReloadTime))
      (Variables|Default|SetCurrentReloadTime (+ (Variables|Default|GetCurrentReloadTime) (Variables|Default|GetReloadTickTime)))
      (else
        (Variables|Default|GetPlayerRef
          (:then
            _)
          (:else
            (bind _returnvalue (Actor|GetActorOfClass "/Game/ShadowDuckStudio/Blueprints/Player/BP_HMCharacter.BP_HMCharacter_C"))
            (Variables|Default|SetPlayerRef _returnvalue)))
        (if (not (< (.resource1 (Variables|/Game/ShadowDuckStudio/Blueprints/ResourcesSystem/AC_ResourceComponent.AC_ResourceComponent_C|GetResources (Variables|/Game/ShadowDuckStudio/Blueprints/Player/BP_HMCharacter.BP_HMCharacter_C|GetAC_ResourceComponent (Variables|Default|GetPlayerRef)))) _resources_taken))
          (Default|TakeResource (Variables|/Game/ShadowDuckStudio/Blueprints/Player/BP_HMCharacter.BP_HMCharacter_C|GetAC_ResourceComponent (Variables|Default|GetPlayerRef)) (Utilities|Struct|MakeF_Resources _resources_taken))
          (Class|BIHealthInterface|Heal(Message) (Variables|Default|GetAC_HealthComponent) (Variables|Default|GetReloadAmount))
          (Utilities|Time|ClearTimerbyFunctionName 0 "ReloadTick")
          (CallFunction|CheckRepairVisible))))))

(fn GetOverlayMeshes
  (return 0))