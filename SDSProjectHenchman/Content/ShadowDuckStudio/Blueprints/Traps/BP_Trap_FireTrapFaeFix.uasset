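; Fire trap defence that burns players and enemies in its box, with stats read from DefenceInfo.
; Overlaps apply damage-over-time and fire VFX; while occupied, a looping timer damages occupants and drains the trap's health, shutting off after a delay once empty or depleted.
; Holding interact runs a reload timer that spends player resources to restore health.
; Proximity volumes and health toggle fuel, repair and minimap indicators; deconstruction supports refunds.
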(event OnComponentBeginOverlap(Box)
  (params (OverlappedComponent :type Primitive%20Component%20Object%20Reference) (OtherActor :type Actor%20Object%20Reference) (OtherComp :type Primitive%20Component%20Object%20Reference) (OtherBodyIndex :type Integer) (bFromSweep :type Boolean) (SweepResult :type Hit%20Result%20Structure%20%28by%20ref%29))
  (CallFunction|Add/RemoveArray (Variables|Default|GetActorsInCollision) OtherActor "NewEnumerator0" (Variables|Default|GetSpecial%20Classes) "NewEnumerator0")
  (CallFunction|CheckIsEmpty?)
  (CallFunction|CheckRepairVisible)
  (if (not (<= (Variables|/Game/ShadowDuckStudio/Blueprints/HealthSystem/AC_HealthComponent.AC_HealthComponent_C|GetCurrentHealth (Variables|Default|GetAC_HealthComponent)) 1.0))
    (AddComponent|AddACDOTBase OtherActor 5.0 1.0 0.1)
    (if (Actor|ActorHasTag OtherActor "Player")
      (bind _asbp_hmcharacter (Utilities|Casting|CastToBP_HMCharacter OtherActor))
      (Default|VFXonFire _asbp_hmcharacter)
      (elif (Actor|ActorHasTag OtherActor "Enemy")
        (bind _asbp_enemy_base (Utilities|Casting|CastToBP_Enemy_Base OtherActor))
        (Default|VFXonFire _asbp_enemy_base)))))

(event OnComponentEndOverlap(Box)
  (params (OverlappedComponent :type Primitive%20Component%20Object%20Reference) (OtherActor :type Actor%20Object%20Reference) (OtherComp :type Primitive%20Component%20Object%20Reference) (OtherBodyIndex :type Integer))
  (CallFunction|Add/RemoveArray (Variables|Default|GetActorsInCollision) OtherActor "NewEnumerator1" (Variables|Default|GetSpecial%20Classes) "NewEnumerator0")
  (CallFunction|CheckIsEmpty?)
  (CallFunction|CheckRepairVisible))

(event OnComponentEndOverlap(Sphere)
  (params (OverlappedComponent :type Primitive%20Component%20Object%20Reference) (OtherActor :type Actor%20Object%20Reference) (OtherComp :type Primitive%20Component%20Object%20Reference) (OtherBodyIndex :type Integer))
  (if (Actor|ActorHasTag OtherActor "Player")
    (Variables|Default|SetInVisibleRadius false)
    (CallFunction|CheckRepairVisible)
    (CallFunction|EndProgress)))

(event OnComponentBeginOverlap(CollisionforAmmo)
  (params (OverlappedComponent :type Primitive%20Component%20Object%20Reference) (OtherActor :type Actor%20Object%20Reference) (OtherComp :type Primitive%20Component%20Object%20Reference) (OtherBodyIndex :type Integer) (bFromSweep :type Boolean) (SweepResult :type Hit%20Result%20Structure%20%28by%20ref%29))
  (if (Actor|ActorHasTag OtherActor "Player")
    (Variables|Default|SetInSmallerRadius true)
    (Rendering|SetVisibility (Variables|Default|GetFuelCounterIcon) true false)
    (CallFunction|CheckSmallerRadius)))

(event OnComponentEndOverlap(CollisionforAmmo)
  (params (OverlappedComponent :type Primitive%20Component%20Object%20Reference) (OtherActor :type Actor%20Object%20Reference) (OtherComp :type Primitive%20Component%20Object%20Reference) (OtherBodyIndex :type Integer))
  (if (Actor|ActorHasTag OtherActor "Player")
    (Variables|Default|SetInSmallerRadius false)
    (Rendering|SetVisibility (Variables|Default|GetFuelCounterIcon) false false)
    (CallFunction|CheckSmallerRadius)))

(event OnComponentBeginOverlap(Sphere)
  (params (OverlappedComponent :type Primitive%20Component%20Object%20Reference) (OtherActor :type Actor%20Object%20Reference) (OtherComp :type Primitive%20Component%20Object%20Reference) (OtherBodyIndex :type Integer) (bFromSweep :type Boolean) (SweepResult :type Hit%20Result%20Structure%20%28by%20ref%29))
  (if (Actor|ActorHasTag OtherActor "Player")
    (Variables|Default|SetInVisibleRadius true)
    (CallFunction|CheckRepairVisible)))

(event Custom|BeginTrap
  (Utilities|Time|SetTimerbyFunctionName 0 "DamageTick" (Variables|Default|GetDamageTickTime) true)
  (Components|Activation|Activate (Variables|Default|GetFXS_FrieTrap) true)
  (bind _returnvalue (Audio|SpawnSoundAttached "/Game/ShadowDuckStudio/SFX/TurretSFX/FlameTrapFire_Cue.FlameTrapFire_Cue" (Variables|Default|GetCube) "None" "0, 0, 0" "0, 0, 0" "KeepRelativeOffset" false 1.0 1.0 0.0 0 0))
  (Audio|Components|Audio|Play _returnvalue 0.0))

(event Custom|EndTrap
  (Utilities|FlowControl|Delay (Variables|Default|GetActiveTimeAfterLeft))
  (Utilities|Time|ClearTimerbyFunctionName 0 "DamageTick")
  (Components|Activation|Deactivate (Variables|Default|GetFXS_FrieTrap))
  (Audio|Components|Audio|Stop (stale Custom|BeginTrap _returnvalue)))

(event Custom|CheckRepairVisible
  (bind _repairiconminimap (Variables|Default|GetRepairIconMinimap))
  (bind _ac_healthcomponent (Variables|Default|GetAC_HealthComponent))
  (bind _repairtextwidget (Variables|Default|GetRepairTextWidget))
  (bind _currenthealth (Variables|/Game/ShadowDuckStudio/Blueprints/HealthSystem/AC_HealthComponent.AC_HealthComponent_C|GetCurrentHealth _ac_healthcomponent))
  (bind _returnvalue (<= _currenthealth 0.0))
  (if _returnvalue
    (Rendering|SetVisibility _repairiconminimap true false)
    (else
      (Rendering|SetVisibility _repairiconminimap false false)))
  (if (and (Variables|Default|GetInVisibleRadius) _returnvalue)
    (Rendering|SetVisibility _repairtextwidget true false)
    (else
      (Rendering|SetVisibility _repairtextwidget false false))))

(event Custom|CheckSmallerRadius
  (bind _holdtorepairtextwidget (Variables|Default|GetHoldtoRepairTextWidget))
  (if (and (<= (Variables|/Game/ShadowDuckStudio/Blueprints/HealthSystem/AC_HealthComponent.AC_HealthComponent_C|GetCurrentHealth (Variables|Default|GetAC_HealthComponent)) 0.0) (Variables|Default|GetInSmallerRadius))
    (Rendering|SetVisibility _holdtorepairtextwidget true false)
    (else
      (Rendering|SetVisibility _holdtorepairtextwidget false false))))

(event Custom|Repairing
  (bind _ac_healthcomponent (Variables|Default|GetAC_HealthComponent))
  (bind _repairprogress (Variables|Default|GetRepairProgress))
  (bind _currenthealth (Variables|/Game/ShadowDuckStudio/Blueprints/HealthSystem/AC_HealthComponent.AC_HealthComponent_C|GetCurrentHealth _ac_healthcomponent))
  (if (== (Math|Vector|VectorLength (Transformation|GetVelocity (Game|Player|GetPlayerPawn 0))) 0.0)
    (if (and (< _currenthealth (Variables|/Game/ShadowDuckStudio/Blueprints/HealthSystem/AC_HealthComponent.AC_HealthComponent_C|GetMaxHealth _ac_healthcomponent)) (>= (.resource1 (Variables|/Game/ShadowDuckStudio/Blueprints/ResourcesSystem/AC_ResourceComponent.AC_ResourceComponent_C|GetResources (Variables|/Game/ShadowDuckStudio/Blueprints/Player/BP_HMCharacter.BP_HMCharacter_C|GetAC_ResourceComponent (Variables|Default|GetPlayerRef)))) (Variables|Default|GetResources%20Taken)))
      (Rendering|SetVisibility _repairprogress true false)
      (if (== _currenthealth 3e+02)
        (Utilities|FlowControl|Delay 1.2)
        (Rendering|SetVisibility _repairprogress false false)))
    (else
      (Utilities|Time|ClearTimerbyFunctionName 0 "ReloadTick")
      (Rendering|SetVisibility _repairprogress false false))))

(event Custom|End%20Progress
  (Rendering|SetVisibility (Variables|Default|GetRepairProgress) false false))

(event Custom|BeginDeconstruct_1
  (params (Source :type Actor%20Object%20Reference))
  (CallFunction|BeginDeconstructTimer self Source (Variables|Default|GetRefund)))

(event EventBeginPlay
  (bind _self self)
  (bind _defenceinfo (Variables|Default|GetDefenceInfo))
  (bind _output (Utilities|Array|Get(acopy) _defenceinfo))
  (bind (_slot _built _cost _angleconstraints _buildiconinfo _tag _def_dmg _def_attackspeed _def_repairamount _def_health _def_dmgpertickself) (Utilities|Struct|BreakF_BuildInfo _output))
  (Utilities|FlowControl|Sequence
    (:then_0
      (if (Utilities|Array|IsEmpty _defenceinfo)
        (Variables|/Game/ShadowDuckStudio/UI/Widgets/TrapsandTurrets/AmmoCounterFireTrap_WBP.AmmoCounterFireTrap_WBP_C|SetTrapRef (.AsAmmo%20Counter%20Fire%20Trap%20WBP (Utilities|Casting|CastToAmmoCounterFireTrap_WBP (UserInterface|GetWidget (Variables|Default|GetFuelCounterIcon)))) _self)
        (Variables|/Game/ShadowDuckStudio/UI/Widgets/TrapsandTurrets/RepairProgressSymbolFireTrap_WBP.RepairProgressSymbolFireTrap_WBP_C|SetFireTrapRef (.AsRepair%20Progress%20Symbol%20Fire%20Trap%20WBP (Utilities|Casting|CastToRepairProgressSymbolFireTrap_WBP (UserInterface|GetWidget (Variables|Default|GetRepairProgress)))) _self)
        (CallFunction|Ref))
      (bind _returnvalue (Actor|GetActorOfClass "/Game/ShadowDuckStudio/Blueprints/Player/BP_HMCharacter.BP_HMCharacter_C"))
      (Variables|Default|SetPlayerRef _returnvalue)
      (bind _returnvalue_2 (Actor|GetActorOfClass "/Game/ShadowDuckStudio/Blueprints/Enemies/BP_Enemy_Base.BP_Enemy_Base_C"))
      (Variables|Default|SetEnemyBaseRef _returnvalue_2)
      (Variables|Default|SetDamageTaken _def_dmg)
      (Variables|Default|SetDamageTickTime _def_attackspeed)
      (Variables|Default|SetReloadAmount _def_repairamount)
      (Variables|/Game/ShadowDuckStudio/Blueprints/HealthSystem/AC_HealthComponent.AC_HealthComponent_C|SetMaxHealth (Variables|Default|GetAC_HealthComponent) _def_health)
      (Variables|Default|SetDurabilityPerTick _def_dmgpertickself))
    (:then_1
      (bind _returnvalue_3 (Audio|SpawnSoundatLocation "/Game/ShadowDuckStudio/SFX/TurretSFX/FlameTrapFire.FlameTrapFire" "0, 0, 0" "0, 0, 0" 1.0 1.0 0.0 0 0))
      (Audio|Components|Audio|Play _returnvalue_3 0.0)
      (Audio|Components|Audio|Stop _returnvalue_3))))

(event Collision|EventActorBeginOverlap
  (params (OtherActor :type Actor%20Object%20Reference)))

(event EventTick
  (params (DeltaSeconds :type Float%20%28single-precision%29)))

(event EventBeginInteract
  (params (Source :type Actor%20Object%20Reference))
  (Variables|Default|SetCurrentReloadTime 0.0)
  (Utilities|Time|SetTimerbyFunctionName 0 "ReloadTick" (Variables|Default|GetReloadTickTime) true))

(event EventEndInteract
  (params (Source :type Actor%20Object%20Reference))
  (Utilities|Time|ClearTimerbyFunctionName 0 "ReloadTick")
  (CallFunction|EndProgress))

(event EventDeath
  (CallFunction|CheckRepairVisible)
  (CallFunction|CheckSmallerRadius))

(event EventHeal
  (params (Amount :type Float%20%28double-precision%29))
  (CallFunction|CheckRepairVisible)
  (CallFunction|CheckSmallerRadius))

(event EventDamage
  (params (Damage :type Float%20%28double-precision%29))
  (CallFunction|CheckRepairVisible)
  (CallFunction|CheckSmallerRadius))

(fn ConstructionScript
  (|CallParentFunction))

(fn CheckIsEmpty?
  (if (> (Variables|/Game/ShadowDuckStudio/Blueprints/HealthSystem/AC_HealthComponent.AC_HealthComponent_C|GetCurrentHealth (Variables|Default|GetAC_HealthComponent)) 0.0)
    (if (Utilities|Array|IsEmpty (Variables|Default|GetActorsInCollision))
      (CallFunction|EndTrap :!label _label)
      (elif (not (Class|KismetSystemLibrary|TimerExists 0 "DamageTick"))
        (CallFunction|BeginTrap)))
    (else
      (goto _label))))

(fn DamageTick
  (for _array_element (Variables|Default|GetActorsInCollision)
    (Class|BIHealthInterface|Damage(Message) (Actor|GetComponentbyClass _array_element "/Game/ShadowDuckStudio/Blueprints/HealthSystem/AC_HealthComponent.AC_HealthComponent_C") (Variables|Default|GetDamageTaken))
    (Default|BeginDOT (Variables|Default|GetAC_DOT_Base)))
  (Class|BIHealthInterface|Damage(Message) (Variables|Default|GetAC_HealthComponent) (Variables|Default|GetDurabilityPerTick)))

(fn ReloadTick
  (bind _resources_taken (Variables|Default|GetResources%20Taken))
  (bind _ac_healthcomponent (Variables|Default|GetAC_HealthComponent))
  (bind _ac_healthcomponent_2 (Variables|Default|GetAC_HealthComponent))
  (CallFunction|Repairing)
  (if (not (>= (Variables|/Game/ShadowDuckStudio/Blueprints/HealthSystem/AC_HealthComponent.AC_HealthComponent_C|GetCurrentHealth _ac_healthcomponent) (Variables|/Game/ShadowDuckStudio/Blueprints/HealthSystem/AC_HealthComponent.AC_HealthComponent_C|GetMaxHealth _ac_healthcomponent)))
    (if (< (Variables|Default|GetCurrentReloadTime) (Variables|Default|GetMaxReloadTime))
      (Variables|Default|SetCurrentReloadTime (+ (Variables|Default|GetCurrentReloadTime) (Variables|Default|GetReloadTickTime)))
      (else
        (Variables|Default|GetPlayerRef
          (:then
            _)
          (:else
            (bind _returnvalue (Actor|GetActorOfClass "/Game/ShadowDuckStudio/Blueprints/Player/BP_HMCharacter.BP_HMCharacter_C"))
            (Variables|Default|SetPlayerRef _returnvalue)))
        (if (not (< (.resource1 (Variables|/Game/ShadowDuckStudio/Blueprints/ResourcesSystem/AC_ResourceComponent.AC_ResourceComponent_C|GetResources (Variables|/Game/ShadowDuckStudio/Blueprints/Player/BP_HMCharacter.BP_HMCharacter_C|GetAC_ResourceComponent (Variables|Default|GetPlayerRef)))) _resources_taken))
          (if (> (Variables|/Game/ShadowDuckStudio/Blueprints/HealthSystem/AC_HealthComponent.AC_HealthComponent_C|GetCurrentHealth _ac_healthcomponent_2) (/ (Variables|/Game/ShadowDuckStudio/Blueprints/HealthSystem/AC_HealthComponent.AC_HealthComponent_C|GetMaxHealth _ac_healthcomponent_2) 2.0))
            (Default|TakeResource (Variables|/Game/ShadowDuckStudio/Blueprints/Player/BP_HMCharacter.BP_HMCharacter_C|GetAC_ResourceComponent (Variables|Default|GetPlayerRef)) (Utilities|Struct|MakeF_Resources (/ (Variables|Default|GetResources%20Taken) 2)))
            (else
              (Default|TakeResource (Variables|/Game/ShadowDuckStudio/Blueprints/Player/BP_HMCharacter.BP_HMCharacter_C|GetAC_ResourceComponent (Variables|Default|GetPlayerRef)) (Utilities|Struct|MakeF_Resources _resources_taken))))
          (Class|BIHealthInterface|Heal(Message) (Variables|Default|GetAC_HealthComponent) (Variables|Default|GetReloadAmount))
          (Utilities|Time|ClearTimerbyFunctionName 0 "ReloadTick")
          (CallFunction|CheckRepairVisible)
          (CallFunction|CheckSmallerRadius))))))

(fn GetOverlayMeshes
  (return 0))