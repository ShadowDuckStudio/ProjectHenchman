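; Spike trap actor that deals repeated damage to actors standing inside its Box volume.
; Box overlap begin and end events add or remove each actor's AC_HealthComponent in ActorsInCollision.
; A looping DamageTick timer runs only while that list is non-empty, sending a Damage interface message to each entry.
; Each tick swaps the Cube material and restores it within the same call.
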(event OnComponentBeginOverlap(Box)
  (params (OverlappedComponent :type Primitive%20Component%20Object%20Reference) (OtherActor :type Actor%20Object%20Reference) (OtherComp :type Primitive%20Component%20Object%20Reference) (OtherBodyIndex :type Integer) (bFromSweep :type Boolean) (SweepResult :type Hit%20Result%20Structure%20%28by%20ref%29))
  (Utilities|Array|AddUnique (Variables|Default|GetActorsInCollision) (Actor|GetComponentbyClass OtherActor "/Game/ShadowDuckStudio/Blueprints/HealthSystem/AC_HealthComponent.AC_HealthComponent_C"))
  (CallFunction|CheckIsEmpty?))

(event OnComponentEndOverlap(Box)
  (params (OverlappedComponent :type Primitive%20Component%20Object%20Reference) (OtherActor :type Actor%20Object%20Reference) (OtherComp :type Primitive%20Component%20Object%20Reference) (OtherBodyIndex :type Integer))
  (Utilities|Array|RemoveItem (Variables|Default|GetActorsInCollision) (Actor|GetComponentbyClass OtherActor "/Game/ShadowDuckStudio/Blueprints/HealthSystem/AC_HealthComponent.AC_HealthComponent_C"))
  (CallFunction|CheckIsEmpty?))

(event EventBeginPlay)

(event Collision|EventActorBeginOverlap
  (params (OtherActor :type Actor%20Object%20Reference)))

(event EventTick
  (params (DeltaSeconds :type Float%20%28single-precision%29)))

(fn ConstructionScript
  (|CallParentFunction))

(fn CheckIsEmpty?
  (if (Utilities|Array|IsEmpty (Variables|Default|GetActorsInCollision))
    (Utilities|Time|ClearTimerbyFunctionName 0 "DamageTick")
    (elif (not (Class|KismetSystemLibrary|TimerExists 0 "DamageTick"))
      (Utilities|Time|SetTimerbyFunctionName 0 "DamageTick" (Variables|Default|GetDamageTickTime) true))))

(fn DamageTick
  (bind _cube (Variables|Default|GetCube))
  (Rendering|Material|SetMaterial _cube 0 "/Engine/MapTemplates/Materials/BasicAsset01.BasicAsset01")
  (for _array_element (Variables|Default|GetActorsInCollision)
    (Class|BIHealthInterface|Damage(Message) _array_element (Variables|Default|GetDamage)))
  (Rendering|Material|SetMaterial _cube 0 "/Engine/ArtTools/RenderToTexture/Materials/Debug/M_BaseColor_Constant.M_BaseColor_Constant"))