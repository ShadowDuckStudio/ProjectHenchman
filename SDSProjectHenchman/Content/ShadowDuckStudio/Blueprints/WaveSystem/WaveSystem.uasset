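; Wave manager that sequences enemy waves, with countdown and wave start/end popup widgets.
; StartNextWave runs on timers, broadcasting the wave number to BI_WaveInterface actors and incrementing it.
; An enemy list triggers an end-wave broadcast when removals empty it; EndWave schedules the next wave if allowed.
; StartWave also activates the level's BP_LavaMechanic on waves two and four.
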(event Custom|SetCanEndWave_1
  (params (CanEndWave? :type Boolean))
  (Variables|Default|SetCan%20End%20Wave? CanEndWave?))

(event EventBeginPlay
  (bind _timebeforefirstwave (Variables|Default|GetTimeBeforeFirstWave))
  (bind _returnvalue (Actor|GetActorOfClass "/Game/ShadowDuckStudio/Blueprints/WorldMechanics/BP_LavaMechanic.BP_LavaMechanic_C"))
  (Variables|Default|SetLavaMechanic _returnvalue)
  (if (> _timebeforefirstwave 0.0)
    (Utilities|Time|SetTimerbyFunctionName 0 "StartNextWave" _timebeforefirstwave)
    (bind _returnvalue_2 (UserInterface|CreateWidget "/Game/ShadowDuckStudio/UI/Widgets/CountdownTimer_WBP.CountdownTimer_WBP_C"))
    (UserInterface|Viewport|AddtoViewport _returnvalue_2 0)
    (Utilities|FlowControl|Delay (Variables|Default|GetTimeBeforeFirstWave))
    (Widget|RemovefromParent _returnvalue_2)
    (else
      (CallFunction|StartNextWave))))

(event EventStartWave
  (params (WaveNo :type Integer))
  (bind _lavamechanic (Variables|Default|GetLavaMechanic))
  (if (== WaveNo 2)
    (Default|ActivateWorldMechanic _lavamechanic)
    (elif (== WaveNo 4)
      (Default|ActivateWorldMechanic _lavamechanic)))
  (bind _returnvalue (UserInterface|CreateWidget "/Game/ShadowDuckStudio/UI/Widgets/WaveIncoming_WBP.WaveIncoming_WBP_C" 0 WaveNo))
  (UserInterface|Viewport|AddtoViewport _returnvalue 0)
  (Utilities|FlowControl|Delay (Variables|Default|GetDurationPopupText))
  (Widget|RemovefromParent _returnvalue))

(event EventEndWave
  (if (Variables|Default|GetCan%20End%20Wave?)
    (Utilities|Time|SetTimerbyFunctionName 0 "StartNextWave" (Variables|Default|GetTimeBetweenWaves))
    (bind _returnvalue (UserInterface|CreateWidget "/Game/ShadowDuckStudio/UI/Widgets/WaveEnding_WBP.WaveEnding_WBP_C" 0 (Variables|Default|GetCurrentWave)))
    (UserInterface|Viewport|AddtoViewport _returnvalue 0)
    (bind _returnvalue_2 (UserInterface|CreateWidget "/Game/ShadowDuckStudio/UI/Widgets/CountdownTimer_WBP.CountdownTimer_WBP_C"))
    (UserInterface|Viewport|AddtoViewport _returnvalue_2 0)
    (Utilities|FlowControl|Delay (Variables|Default|GetDurationPopupText))
    (Widget|RemovefromParent _returnvalue)
    (Utilities|FlowControl|Delay (- (Variables|Default|GetTimeBetweenWaves) 1e+01))
    (Widget|RemovefromParent _returnvalue_2)))

(event EventAddEnemytoWave
  (params (Enemy :type Actor%20Object%20Reference))
  (Utilities|IsValid Enemy
    (:Is%20Valid
      (Utilities|Array|AddUnique (Variables|Default|GetEnemiesInWave) Enemy))))

(event EventRemoveEnemyfromWave
  (params (Enemy :type Actor%20Object%20Reference))
  (bind _enemiesinwave (Variables|Default|GetEnemiesInWave))
  (bind _returnvalue (Utilities|Array|Length _enemiesinwave))
  (bind _returnvalue_2 (== _returnvalue 0))
  (Utilities|IsValid Enemy
    (:Is%20Valid
      (Utilities|Array|RemoveItem _enemiesinwave Enemy)
      (if _returnvalue_2
        (Variables|Default|SetCan%20End%20Wave? _returnvalue_2)
        (bind _outactors (Actor|GetAllActorswithInterface "/Game/ShadowDuckStudio/Blueprints/WaveSystem/BI_WaveInterface.BI_WaveInterface_C"))
        (for _array_element _outactors
          (Class|BIWaveInterface|EndWave(Message) _array_element))))))

(fn ConstructionScript)

(fn StartNextWave
  (bind _outactors (Actor|GetAllActorswithInterface "/Game/ShadowDuckStudio/Blueprints/WaveSystem/BI_WaveInterface.BI_WaveInterface_C"))
  (for _array_element _outactors
    (Class|BIWaveInterface|StartWave(Message) _array_element (Variables|Default|GetCurrentWave)))
  (Variables|Default|SetCurrentWave (+ (Variables|Default|GetCurrentWave) 1)))