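; Blueprint function library with two general-purpose helpers for filtered array editing and rotator math.
; AddRemoveArray adds an item uniquely or removes it, gated by a blacklist or whitelist check on the item's exact class, and returns whether the array is empty when the check passes.
; RotateRotatorOnAxis rotates a rotator around one of its own local X, Y or Z axes by rotating all three basis vectors and rebuilding the rotation.
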(fn Add/RemoveArray
  (params (Array :type Array%20of%20Actor%20Object%20References) (Item :type Actor%20Object%20Reference) (Add/Remove :type E_Add-Remove%20Enum :default "NewEnumerator0") (SpecialClasses :type Array%20of%20Actor%20Class%20References) (Blacklist/Whitelist :type E_Blacklist-Whitelist%20Enum :default "NewEnumerator0"))
  (bind _returnvalue (Utilities|GetClass Item))
  (bind _returnvalue_2 (Utilities|Array|ContainsItem SpecialClasses _returnvalue))
  (switch Utilities|FlowControl|Switch|SwitchonE_Blacklist-Whitelist Blacklist/Whitelist
    (:NewEnumerator0
      (if (not _returnvalue_2)
        (switch Utilities|FlowControl|Switch|SwitchonE_Add-Remove Add/Remove
          (:NewEnumerator0
            (Utilities|Array|AddUnique Array Item))
          (:NewEnumerator1
            (Utilities|Array|RemoveItem Array Item)))
        (return (Utilities|Array|IsEmpty Array))))
    (:NewEnumerator1
      (if _returnvalue_2
        (switch Utilities|FlowControl|Switch|SwitchonE_Add-Remove Add/Remove
          (:NewEnumerator0
            (Utilities|Array|AddUnique Array Item))
          (:NewEnumerator1
            (Utilities|Array|RemoveItem Array Item)))
        (return (Utilities|Array|IsEmpty Array))))))

(fn RotateRotatoronAxis
  (params (Rotator :type Rotator) (Rotation :type Float%20%28single-precision%29) (Axis :type E_XYZ%20Enum :default "NewEnumerator0"))
  (bind (_x _y _z) (Math|Rotator|GetAxes Rotator))
  (bind _returnvalue (Utilities|Select :Index Axis :NewEnumerator0 _x :NewEnumerator1 _y :NewEnumerator2 _z))
  (return (Math|Rotator|MakeRotationfromAxes (Math|Vector|RotateVectorAroundAxis _x Rotation _returnvalue) (Math|Vector|RotateVectorAroundAxis _y Rotation _returnvalue) (Math|Vector|RotateVectorAroundAxis _z Rotation _returnvalue))))