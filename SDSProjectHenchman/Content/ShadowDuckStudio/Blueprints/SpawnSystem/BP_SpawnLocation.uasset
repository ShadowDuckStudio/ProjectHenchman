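; BP_SpawnLocation is a spawn point that produces enemies for a given wave.
; BeginSpawning loads that wave's class-to-count map, starts a looping SpawnTick timer and shows a spawning icon briefly if the map has entries.
; Each tick spawns one enemy at the actor's transform, working through classes in turn, but only while the overlap-tracked SpawnDenialRadius is clear.
; AddtoSpawnList is an empty stub, with its AddClassToSpawnList calls left unconnected.
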(event OnComponentBeginOverlap(SpawnDenialRadius)
  (params (OverlappedComponent :type Primitive%20Component%20Object%20Reference) (OtherActor :type Actor%20Object%20Reference) (OtherComp :type Primitive%20Component%20Object%20Reference) (OtherBodyIndex :type Integer) (bFromSweep :type Boolean) (SweepResult :type Hit%20Result%20Structure%20%28by%20ref%29))
  (CallFunction|Add/RemoveArray (Variables|Default|GetCollidingActors) OtherActor "NewEnumerator0" (Variables|Default|GetIgnoredClasses) "NewEnumerator0"))

(event OnComponentEndOverlap(SpawnDenialRadius)
  (params (OverlappedComponent :type Primitive%20Component%20Object%20Reference) (OtherActor :type Actor%20Object%20Reference) (OtherComp :type Primitive%20Component%20Object%20Reference) (OtherBodyIndex :type Integer))
  (CallFunction|Add/RemoveArray (Variables|Default|GetCollidingActors) OtherActor "NewEnumerator1" (Variables|Default|GetIgnoredClasses) "NewEnumerator0"))

(event Custom|ClearSpawn
  (Utilities|Map|Clear (Variables|Default|GetSpawnList_1)))

(event EventBeginPlay)

(event Collision|EventActorBeginOverlap
  (params (OtherActor :type Actor%20Object%20Reference)))

(event EventTick
  (params (DeltaSeconds :type Float%20%28single-precision%29)))

(event EventAddtoSpawnList
  (params (Enemy :type F%20Wave%20Data%20Structure)))

(event EventBeginSpawning
  (params (WaveNo :type Integer))
  (Variables|Default|SetSpawnList_1 (Utilities|Struct|BreakF_EnemiesPerWave (Utilities|Array|Get(acopy) (Variables|Default|GetEnemiesPerWave) WaveNo)))
  (Utilities|Time|SetTimerbyFunctionName 0 "SpawnTick" (Variables|Default|GetSpawnTickTime) true)
  (if (not (Utilities|Map|IsEmpty (Variables|Default|GetSpawnList_1)))
    (Rendering|SetVisibility (Variables|Default|GetSpawningIcon) true false)
    (Utilities|FlowControl|Delay 5.0)
    (Rendering|SetVisibility (Variables|Default|GetSpawningIcon) false false)))

(fn ConstructionScript)

(fn SpawnTick
  (bind _spawnlist_1 (Variables|Default|GetSpawnList_1))
  (if (Utilities|Array|IsEmpty (Variables|Default|GetCollidingActors))
    (bind _keys (Utilities|Map|Keys _spawnlist_1))
    (bind _values (Utilities|Map|Values _spawnlist_1))
    (if (>= (Variables|Default|GetCurrentAmountNumber) (Utilities|Array|Get(acopy) _values (Variables|Default|GetClassNumber)))
      (Variables|Default|SetClassNumber (+ (Variables|Default|GetClassNumber) 1))
      (if (> (Variables|Default|GetClassNumber) (Utilities|Map|Length (Variables|Default|GetSpawnList_1)))
        (Utilities|Time|ClearTimerbyFunctionName 0 "SpawnTick")
        (Variables|Default|SetClassNumber 0)
        (else
          (Variables|Default|SetCurrentAmountNumber 0)))
      (else
        (Game|SpawnActorfromClass (Utilities|Array|Get(acopy) _keys (Variables|Default|GetClassNumber)) (Transformation|GetActorTransform) "AdjustIfPossibleButAlwaysSpawn" "MultiplyWithRoot" 0 0)
        (Variables|Default|SetCurrentAmountNumber (+ (Variables|Default|GetCurrentAmountNumber) 1))))))

(fn AddClasstoSpawnList
  (params (Class :type Actor%20Class%20Reference%20%28by%20ref%29) (Amount :type Integer))
  (bind _spawnlist_1 (Variables|Default|GetSpawnList_1))
  (bind (_value _returnvalue) (Utilities|Map|Find _spawnlist_1 Class))
  (Utilities|Map|Add (Variables|Default|GetSpawnList_1) Class (select _returnvalue (+ _value Amount) Amount)))