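; Spawn component that builds an enemy wave from a power budget and hands it to its owning BP_SpawnManager.
; A looping timer picks a random spawnable class, tallies it by class and subtracts its class-default cost from the remaining WavePower.
; An unaffordable pick triggers pruning of too-expensive classes.
; Once none remain, the timer stops and the tally is passed to the manager's AutoSpawn.
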(event EventBeginPlay)

(fn SetWaveSpawns
  (params (WavePower :type F%20Auto%20Spawn%20Variables%20Structure))
  (Variables|Default|SetWavePower WavePower)
  (Utilities|Time|SetTimerbyFunctionName 0 "AddSingleSpawn" (Variables|Default|GetAddSpawnTime) true))

(fn AddSingleSpawn
  (bind _wavepower (Variables|Default|GetWavePower))
  (bind (_wavepower_2 _spawnableclasses) (Utilities|Struct|BreakF_AutoSpawnVariables _wavepower))
  (bind _output_get (Variables|Default|SetRandomClass (.OutItem (Utilities|Array|Random _spawnableclasses))))
  (Variables|Default|SetClassFound? false)
  (if (<= (Utilities|GetClassDefaults _output_get) _wavepower_2)
    (CallFunction|IncrementSpawnAmount)
    (else
      (CallFunction|RemoveInvalidClasses)
      (if (Utilities|Array|IsEmpty (Utilities|Struct|BreakF_AutoSpawnVariables (Variables|Default|GetWavePower)))
        (Utilities|Time|ClearTimerbyFunctionName 0 "AddSingleSpawn")
        (CallFunction|SetOwnerSpawns)))))

(fn SetOwnerSpawns
  (bind _asbp_spawn_manager (Utilities|Casting|CastToBP_SpawnManager (Components|GetOwner)))
  (Variables|/Game/ShadowDuckStudio/Blueprints/SpawnSystem/BP_SpawnManager.BP_SpawnManager_C|SetAutoEnemySpawn _asbp_spawn_manager (Variables|Default|GetAutoEnemySpawn))
  (Default|AutoSpawn _asbp_spawn_manager))

(fn RemoveInvalidClasses
  (bind _wavepower (Variables|Default|GetWavePower))
  (bind (_wavepower_2 _spawnableclasses) (Utilities|Struct|BreakF_AutoSpawnVariables _wavepower))
  (for _array_element _spawnableclasses
    (if (not (<= (Utilities|GetClassDefaults _array_element) _wavepower_2))
      (Utilities|Array|RemoveItem _spawnableclasses _array_element)))
  (return))

(fn IncrementSpawnAmount
  (bind _wavepower (Variables|Default|GetWavePower))
  (bind _autoenemyspawn (Variables|Default|GetAutoEnemySpawn))
  (bind (_array_element _array_index) (Utilities|Array|ForEachLoopwithBreak _autoenemyspawn :!label _label)
    (:LoopBody
      (if (== (Variables|Default|GetRandomClass) (.EnemyClass (Utilities|Struct|BreakF_AutoSpawnEnemyInfo _array_element)))
        (Variables|Default|SetClassFound? true)
        (goto _label Break)))
    (:Completed
      (if (Variables|Default|GetClassFound?)
        (bind _structout (Utilities|Struct|SetmembersinF_AutoSpawnEnemyInfo _array_element (+ (.Amount (Utilities|Struct|BreakF_AutoSpawnEnemyInfo _array_element)) 1)))
        (Utilities|Array|SetArrayElem _autoenemyspawn _array_index _structout)
        (else
          (Utilities|Array|AddUnique _autoenemyspawn (Utilities|Struct|MakeF_AutoSpawnEnemyInfo (Variables|Default|GetRandomClass) 1))))
      (Utilities|Struct|SetmembersinF_AutoSpawnVariables _wavepower (- (Utilities|Struct|BreakF_AutoSpawnVariables _wavepower) (Utilities|GetClassDefaults (Variables|Default|GetRandomClass)))))))