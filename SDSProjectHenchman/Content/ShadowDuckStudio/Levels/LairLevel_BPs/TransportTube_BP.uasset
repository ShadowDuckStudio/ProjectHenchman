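; Two-way transport tube in the lair level that teleports the player character between two target volumes.
; Overlapping either target with the player capsule starts a one-second timer that teleports the character to the other target with zeroed rotation.
; A shared cooldown flag prevents bouncing straight back, and leaving a target clears it and cancels any pending teleport.
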(event OnComponentBeginOverlap(Target1)
  (params (OverlappedComponent :type Primitive%20Component%20Object%20Reference) (OtherActor :type Actor%20Object%20Reference) (OtherComp :type Primitive%20Component%20Object%20Reference) (OtherBodyIndex :type Integer) (bFromSweep :type Boolean) (SweepResult :type Hit%20Result%20Structure%20%28by%20ref%29))
  ;[1 1 1] Teleport To Target 2
  (if (and (not (Variables|Default|GetOnCooldown)) (== OtherComp (Variables|/Script/Engine.Character|GetCapsuleComponent (Variables|Default|GetPlayer%20Character))))
    (bind _returnvalue (Utilities|Time|SetTimerbyEvent (delegate Custom|Teleport2) 1.0))
    (Variables|Default|SetTeleportTimer _returnvalue)))

(event OnComponentBeginOverlap(Target2)
  (params (OverlappedComponent :type Primitive%20Component%20Object%20Reference) (OtherActor :type Actor%20Object%20Reference) (OtherComp :type Primitive%20Component%20Object%20Reference) (OtherBodyIndex :type Integer) (bFromSweep :type Boolean) (SweepResult :type Hit%20Result%20Structure%20%28by%20ref%29))
  ;[1 1 1] Teleport To Target 1
  (if (and (not (Variables|Default|GetOnCooldown)) (== OtherComp (Variables|/Script/Engine.Character|GetCapsuleComponent (Variables|Default|GetPlayer%20Character))))
    (bind _returnvalue (Utilities|Time|SetTimerbyEvent (delegate Custom|Teleport1) 1.0))
    (Variables|Default|SetTeleportTimer _returnvalue)))

(event OnComponentEndOverlap(Target1)
  (params (OverlappedComponent :type Primitive%20Component%20Object%20Reference) (OtherActor :type Actor%20Object%20Reference) (OtherComp :type Primitive%20Component%20Object%20Reference) (OtherBodyIndex :type Integer))
  ;[1 1 1] Teleport To Target 2
  ;;[1 1 1] Cooldown
  (if (not (Collision|IsOverlappingActor (Variables|Default|GetTarget1) (Variables|Default|GetPlayer%20Character) :!class /Script/Engine.PrimitiveComponent))
    (Utilities|Time|ClearandInvalidateTimerbyHandle (Variables|Default|GetTeleportTimer))
    (Variables|Default|SetOnCooldown false)))

(event OnComponentEndOverlap(Target2)
  (params (OverlappedComponent :type Primitive%20Component%20Object%20Reference) (OtherActor :type Actor%20Object%20Reference) (OtherComp :type Primitive%20Component%20Object%20Reference) (OtherBodyIndex :type Integer))
  ;[1 1 1] Teleport To Target 1
  ;;[1 1 1] Cooldown
  (if (not (Collision|IsOverlappingActor (Variables|Default|GetTarget2) (Variables|Default|GetPlayer%20Character) :!class /Script/Engine.PrimitiveComponent))
    (Utilities|Time|ClearandInvalidateTimerbyHandle (Variables|Default|GetTeleportTimer))
    (Variables|Default|SetOnCooldown false)))

(event Custom|Teleport2
  ;[1 1 1] Teleport To Target 2
  (Transformation|Teleport (Variables|Default|GetPlayer%20Character) (Transformation|GetWorldLocation (Variables|Default|GetTarget2)) "0, 0, 0")
  (Variables|Default|SetOnCooldown true))

(event Custom|Teleport1
  ;[1 1 1] Teleport To Target 1
  (Transformation|Teleport (Variables|Default|GetPlayer%20Character) (Transformation|GetWorldLocation (Variables|Default|GetTarget1)) "0, 0, 0")
  (Variables|Default|SetOnCooldown true))

(event EventBeginPlay
  ;[1 1 1] Set player Character
  (bind _asbp_hmcharacter (Utilities|Casting|CastToBP_HMCharacter (Game|GetPlayerCharacter 0)))
  (Variables|Default|SetPlayer%20Character _asbp_hmcharacter))

(fn ConstructionScript)