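; Lair level gate that slides down when a minion enters its trigger box and back up after one leaves.
; Begin overlap passes a DoOnce before the BP_MinionBase cast, so any overlapping actor can consume it.
; A minion's end overlap waits out a delay, raises the center entrance mesh and resets the DoOnce.
; Both moves use MoveComponentTo with offsets from the mesh's current relative location.
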(event OnComponentBeginOverlap(Box)
  (params (OverlappedComponent :type Primitive%20Component%20Object%20Reference) (OtherActor :type Actor%20Object%20Reference) (OtherComp :type Primitive%20Component%20Object%20Reference) (OtherBodyIndex :type Integer) (bFromSweep :type Boolean) (SweepResult :type Hit%20Result%20Structure%20%28by%20ref%29))
  (bind _centerentrancegate_staticmesh (Variables|Default|GetCenterEntranceGate_StaticMesh))
  (Utilities|FlowControl|DoOnce false
    (:Completed
      (Utilities|Casting|CastToBP_MinionBase OtherActor)
      (Components|MoveComponentTo _centerentrancegate_staticmesh (- (Variables|/Script/Engine.SceneComponent|GetRelativeLocation _centerentrancegate_staticmesh) "0.000000,0.000000,285.000000") "0, 0, 0" false false 1.0 false))))

(event OnComponentEndOverlap(Box)
  (params (OverlappedComponent :type Primitive%20Component%20Object%20Reference) (OtherActor :type Actor%20Object%20Reference) (OtherComp :type Primitive%20Component%20Object%20Reference) (OtherBodyIndex :type Integer))
  (bind _centerentrancegate_staticmesh (Variables|Default|GetCenterEntranceGate_StaticMesh))
  (Utilities|Casting|CastToBP_MinionBase OtherActor)
  (Utilities|FlowControl|Delay 8.0)
  (Components|MoveComponentTo _centerentrancegate_staticmesh (+ (Variables|/Script/Engine.SceneComponent|GetRelativeLocation _centerentrancegate_staticmesh) "0.000000,0.000000,285.000000") "0, 0, 0" false false 1.0 false)
  (Utilities|FlowControl|DoOnce false) ; enters at Reset
)

(event EventBeginPlay)

(event Collision|EventActorBeginOverlap
  (params (OtherActor :type Actor%20Object%20Reference)))

(event EventTick
  (params (DeltaSeconds :type Float%20%28single-precision%29)))

(fn ConstructionScript)