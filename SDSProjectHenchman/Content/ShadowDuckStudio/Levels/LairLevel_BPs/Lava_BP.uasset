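; Lair level lava hazard that teleports any minion touching it back to a spawn point and lowers when a minion enters its trigger.
; A DoOnce gates the drop; after a minion leaves, a delay precedes a slower rise back, then the gate resets.
; Each move plays three pipe-flow sounds that fade out once it finishes, over a looping-style ambience attached to the lava plane at BeginPlay.
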(event OnComponentBeginOverlap(LavaPlane_StaticMesh)
  (params (OverlappedComponent :type Primitive%20Component%20Object%20Reference) (OtherActor :type Actor%20Object%20Reference) (OtherComp :type Primitive%20Component%20Object%20Reference) (OtherBodyIndex :type Integer) (bFromSweep :type Boolean) (SweepResult :type Hit%20Result%20Structure%20%28by%20ref%29))
  (bind _asbp_minion_base (Utilities|Casting|CastToBP_MinionBase OtherActor))
  (Transformation|Teleport _asbp_minion_base (Transformation|GetWorldLocation (Variables|Default|GetSpawnPoint)) "0, 0, 0"))

(event OnComponentBeginOverlap(LavaTrigger)
  (params (OverlappedComponent :type Primitive%20Component%20Object%20Reference) (OtherActor :type Actor%20Object%20Reference) (OtherComp :type Primitive%20Component%20Object%20Reference) (OtherBodyIndex :type Integer) (bFromSweep :type Boolean) (SweepResult :type Hit%20Result%20Structure%20%28by%20ref%29))
  (bind _lavaplane_staticmesh (Variables|Default|GetLavaPlane_StaticMesh))
  ;[1 1 1] Lava Moves On Trigger
  (Utilities|FlowControl|DoOnce false
    (:Completed
      (Utilities|Casting|CastToBP_MinionBase OtherActor)
      (Utilities|PlayLavaFlowSound)
      (Components|MoveComponentTo _lavaplane_staticmesh (- (Variables|/Script/Engine.SceneComponent|GetRelativeLocation _lavaplane_staticmesh) "0.000000,0.000000,280.000000") "0, 0, 0" false false 1e+01 false)
      (Audio|Components|Audio|FadeOut (Variables|Default|GetLavaComingFromPipe_Cue) 2.0 0.0 "Linear" :!class /Script/Engine.AudioComponent))))

(event OnComponentEndOverlap(LavaTrigger)
  (params (OverlappedComponent :type Primitive%20Component%20Object%20Reference) (OtherActor :type Actor%20Object%20Reference) (OtherComp :type Primitive%20Component%20Object%20Reference) (OtherBodyIndex :type Integer))
  (bind _lavaplane_staticmesh (Variables|Default|GetLavaPlane_StaticMesh))
  ;[1 1 1] Lava Moves On Trigger
  (Utilities|Casting|CastToBP_MinionBase OtherActor)
  (Utilities|FlowControl|Delay 25.0)
  (Utilities|PlayLavaFlowSound)
  (Components|MoveComponentTo _lavaplane_staticmesh (+ (Variables|/Script/Engine.SceneComponent|GetRelativeLocation _lavaplane_staticmesh) "0.000000,0.000000,280.000000") "0, 0, 0" false false 2e+01 false)
  (Audio|Components|Audio|FadeOut (Variables|Default|GetLavaComingFromPipe_Cue) 2.0 0.0 "Linear" :!class /Script/Engine.AudioComponent)
  (Utilities|FlowControl|DoOnce false) ; enters at Reset
)

(event Custom|LavaAmbience
  ;[1 1 1] Lava Ambience
  (bind _returnvalue (Audio|SpawnSoundAttached "/Game/ShadowDuckStudio/SFX/LairSFX/LavaFlowingWithRocks_Reverb__Cue.LavaFlowingWithRocks_Reverb__Cue" (Variables|Default|GetLavaPlane_StaticMesh) "None" "0, 0, 0" "0, 0, 0" "KeepRelativeOffset" false 1.0 1.0 0.0 0 0))
  (Audio|Components|Audio|Play _returnvalue 0.0))

(event EventBeginPlay
  (CallFunction|LavaAmbience))

(fn ConstructionScript)