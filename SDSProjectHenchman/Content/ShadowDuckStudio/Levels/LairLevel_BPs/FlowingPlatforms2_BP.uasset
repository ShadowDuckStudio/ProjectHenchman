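; FlowingPlatforms2_BP is a Lair level moving platform that cycles endlessly along a one-way path through five position variables.
; From BeginPlay, chained latent MoveComponentTo calls carry the Platform component through each point at fixed durations, with a quicker final leg.
; It then hides the platform, moves it back to the first position with zero duration, shows it again and loops, disguising the reset.
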(event EventBeginPlay
  (bind _platform (Variables|Default|GetPlatform))
  (Components|MoveComponentTo _platform (Variables|Default|GetPostition%202) "0, 0, 0" false false 6.0 false :!label _label)
  (Components|MoveComponentTo _platform (Variables|Default|GetPostition%203) "0, 0, 0" false false 6.0 false)
  (Components|MoveComponentTo _platform (Variables|Default|GetPostition%204) "0, 0, 0" false false 6.0 false)
  (Components|MoveComponentTo _platform (Variables|Default|GetPostition%205) "0, 0, 0" false false 1.0 false)
  (Rendering|SetVisibility _platform false false)
  (Components|MoveComponentTo _platform (Variables|Default|GetPostition%201) "0, 0, 0" false false 0.0 false)
  (Rendering|SetVisibility _platform true false)
  (goto _label))

(fn ConstructionScript)