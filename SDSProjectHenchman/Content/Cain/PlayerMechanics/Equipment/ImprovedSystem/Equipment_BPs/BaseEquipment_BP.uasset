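; Base equipment actor that a BP_MinionBase character can pick up and wear on a mesh socket.
; Interacting stores this actor in the minion's EquipmentPickup variable, then destroys the actor.
; Attachment runs from an SVR event into a Multi event, named as a server-to-multicast pair, which snaps the equipment to the named socket on the owning minion's mesh.
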(event Custom|MultiAttach%20to%20Player
  (params (SocketName :type Name))
  ;[0.04417 1 0] Socket name input to change based on equipment
  (Transformation|AttachComponentToComponent (Variables|/Script/Engine.Character|GetMesh (.AsBP%20Minion%20Base (Utilities|Casting|CastToBP_MinionBase (Components|GetOwner)))) SocketName "SnapToTarget" "SnapToTarget" "SnapToTarget" true))

(event Custom|SVRAttach%20to%20Player
  (params (SocketName :type Name))
  (CallFunction|MultiAttachtoPlayer SocketName))

(event EventBeginPlay)

(event Collision|EventActorBeginOverlap
  (params (OtherActor :type Actor%20Object%20Reference)))

(event EventTick
  (params (DeltaSeconds :type Float%20%28single-precision%29)))

(event EventEquipmentInteract
  (params (ActorRef :type Actor%20Object%20Reference))
  ;[1 0 0] Change this to player base class when intergrating for mulitplayer
  (bind _asbp_minion_base (Utilities|Casting|CastToBP_MinionBase ActorRef))
  (Variables|/Game/Cain/PlayerMechanics/Playercharacter/Character/Base_Character/BP_MinionBase.BP_MinionBase_C|SetEquipment_Pickup _asbp_minion_base self)
  (Actor|DestroyActor))

(fn ConstructionScript)