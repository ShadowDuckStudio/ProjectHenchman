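; Hammer equipment Blueprint from the improved equipment system that can grow and shrink.
; IncreaseSize plays a timeline from the start, lerping the relative scale of the Head and BaseStatic components up to larger values.
; DecreaseSize reverses the same timeline to scale both parts back down.
; BeginPlay, overlap and Tick are disabled stubs, and the construction script only calls the parent.
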(event Custom|Increase%20Size
  (bind _size (Timeline|Timeline_0 PlayFromStart)
    (:Update
      (Transformation|SetRelativeTransform (Variables|Default|GetHead) (Math|Transform|MakeTransform "0, 0, 0" "0, 0, 0" (Math|Vector|Lerp(Vector) "1.000000,1.000000,1.000000" "2.000000,2.000000,2.000000" _size)) false false)
      (Transformation|SetRelativeTransform (Variables|Default|GetBaseStatic) (Math|Transform|MakeTransform "0, 0, 0" "0, 0, 0" (Math|Vector|Lerp(Vector) "0.020000,0.020000,0.020000" "0.050000,0.050000,0.050000" _size)) false false))))

(event Custom|Decrease%20Size
  (bind _size (Timeline|Timeline_0 Reverse)
    (:Update
      (Transformation|SetRelativeTransform (Variables|Default|GetHead) (Math|Transform|MakeTransform "0, 0, 0" "0, 0, 0" (Math|Vector|Lerp(Vector) "1.000000,1.000000,1.000000" "2.000000,2.000000,2.000000" _size)) false false)
      (Transformation|SetRelativeTransform (Variables|Default|GetBaseStatic) (Math|Transform|MakeTransform "0, 0, 0" "0, 0, 0" (Math|Vector|Lerp(Vector) "0.020000,0.020000,0.020000" "0.050000,0.050000,0.050000" _size)) false false))))

(event EventBeginPlay
  (|CallParentFunction) ; This node is disabled and will not be called.\nDrag off pins to build functionality.
)

(event Collision|EventActorBeginOverlap
  (params (OtherActor :type Actor%20Object%20Reference))
  (|CallParentFunction OtherActor) ; This node is disabled and will not be called.\nDrag off pins to build functionality.
)

(event EventTick
  (params (DeltaSeconds :type Float%20%28single-precision%29))
  (|CallParentFunction DeltaSeconds) ; This node is disabled and will not be called.\nDrag off pins to build functionality.
)

(fn ConstructionScript
  (|CallParentFunction))