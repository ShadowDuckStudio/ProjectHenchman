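; Multiplayer game mode that tracks connected player controllers and provides spawning of players as minion pawns.
; PostLogin and controller swaps on level changes add controllers to the AllPcs array, and logout removes those that cast to PC_Multiplayer.
; SpawnPlayer destroys any currently controlled pawn, spawns a BP_MinionBase at a randomly chosen PlayerStart and has the given controller possess it.
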(event EventPostLogin
  (params (NewPlayer :type Player%20Controller%20Object%20Reference))
  ;[0.04417 1 0] Events for when a player connects to the session
  ;;[1 0 0.9168] Adding player all players who connect to array
  (Utilities|Array|Add (Variables|Default|GetAll%20Pcs) NewPlayer))

(event EventOnSwapPlayerControllers
  (params (OldPC :type Player%20Controller%20Object%20Reference) (NewPC :type Player%20Controller%20Object%20Reference))
  ;[0.04417 1 0] Events for when a player connects to the session
  ;;[1 0 0.9168] If players load into another level such as lobby to mulitplayer map this updates the controllers
  (Utilities|Array|Add (Variables|Default|GetAll%20Pcs) NewPC))

(event EventOnLogout
  (params (ExitingController :type Controller%20Object%20Reference))
  ;[0.04417 1 0] Game mode event for when a player logs out of the session
  (bind _aspc_multiplayer (Utilities|Casting|CastToPC_Multiplayer ExitingController))
  (Utilities|Array|RemoveItem (Variables|Default|GetAll%20Pcs) _aspc_multiplayer))

(fn ConstructionScript)

(fn FindRandomPlayerStart
  (bind _outactors (Actor|GetAllActorsOfClass "/Script/Engine.PlayerStart"))
  (return (Transformation|GetActorTransform (Utilities|Array|Get(acopy) _outactors (Math|Random|RandomIntegerinRange 0 (- (Utilities|Array|Length _outactors) 1))))))

(fn SpawnPlayer
  (params (Player%20Controller :type Player%20Controller%20Object%20Reference))
  (bind _returnvalue (Pawn|GetControlledPawn Player%20Controller))
  (Utilities|IsValid _returnvalue
    (:Is%20Valid
      (Actor|DestroyActor _returnvalue))
    (:Is%20Not%20Valid
      _))
  (bind _returnvalue_2 (Game|SpawnActorfromClass "/Game/Cain/PlayerMechanics/Playercharacter/Character/Base_Character/BP_MinionBase.BP_MinionBase_C" (Spawn|FindRandomPlayerStart) "Undefined" "MultiplyWithRoot" 0 0))
  (Pawn|Possess Player%20Controller _returnvalue_2))